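; BP_TSSWeapon_Minigun is a minigun weapon that fires projectiles continuously from the moment it spins up until firing stops.
; Fire plays a start sound and starts a looping timer with a short spin-up delay, which StopFire clears.
; ShootMinigun checks ammo, then spawns a scaled-down projectile, muzzle effect and attenuated shot sound at the muzzle arrow.
; Tick rolls the barrel mesh while the timer handle is valid.
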(event `self.Fire`
  (bind _returnvalue (`KismetSystemLibrary.K2_SetTimerDelegate` (`|CreateDelegate` :!event `ShootMinigun`) 0.1 true false 0.5))
  (set `self.MinigunTimer` _returnvalue)
  (`GameplayStatics.PlaySoundAtLocation` "/Game/TSS/Sounds/minigun_start.minigun_start" (`self.K2_GetActorLocation`) (struct) 1.0 1.0 0.0 null null null null))

(event `self.StopFire`
  (`KismetSystemLibrary.K2_ClearAndInvalidateTimerHandle` (`self.MinigunTimer`)))

(event `ShootMinigun`
  (bind _arrowmuzzle (`self.ArrowMuzzle`))
  (bind _arrowmuzzle_2 (`self.ArrowMuzzle`))
  (bind _returnvalue (`SceneComponent.K2_GetComponentLocation` _arrowmuzzle))
  (bind _returnvalue_2 (`SceneComponent.K2_GetComponentLocation` _arrowmuzzle_2))
  (bind _bammoavalible (`self.CheckAmmo`))
  (if _bammoavalible
    (`|SpawnActorFromClass` "/Game/TSS/Blueprints/Weapons/BP_TSSProjectile.BP_TSSProjectile_C" (`KismetMathLibrary.MakeTransform` _returnvalue (`KismetMathLibrary.FindLookAtRotation` _returnvalue (+ _returnvalue (`SceneComponent.GetForwardVector` _arrowmuzzle))) (0.2 0.2 0.2)) "Undefined" "MultiplyWithRoot" null null)
    (`NiagaraFunctionLibrary.SpawnSystemAtLocation` "/Game/Lesson/VFX/NS_Muzzle.NS_Muzzle" _returnvalue_2 (`KismetMathLibrary.FindLookAtRotation` _returnvalue_2 (+ _returnvalue_2 (`SceneComponent.GetForwardVector` _arrowmuzzle_2))))
    (`GameplayStatics.PlaySoundAtLocation` "/Game/TSS/Sounds/minigun_shoot.minigun_shoot" (`SceneComponent.K2_GetComponentLocation` (`self.ArrowMuzzle`)) (struct) 1.0 1.0 0.0 "/Game/TSS/Sounds/SA_Shot.SA_Shot" null null null)))

(event `self.ReceiveTick`
  (params (DeltaSeconds :type "Float (single-precision)"))
  (if (`KismetSystemLibrary.K2_IsValidTimerHandle` (`self.MinigunTimer`))
    (`SceneComponent.K2_AddRelativeRotation` (`self.SM_Muzzle_MG`) (`KismetMathLibrary.MakeRotator` (* (`self.RotationSpeed`) (`GameplayStatics.GetWorldDeltaSeconds`))) false false)))

(fn `UserConstructionScript`
  (`parent.UserConstructionScript`))
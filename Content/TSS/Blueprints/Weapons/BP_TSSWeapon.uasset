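; BP_TSSWeapon is a weapon Blueprint with Fire and StopFire events, where Fire only prints a debug string and StopFire is empty.
; CheckAmmo casts the owner to BP_TSSCharacter and looks up its Ammo map, keyed by the weapon's class.
; It consumes one round and returns true if any remain, otherwise false; neither event in this file calls it.
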(event `Fire`
  (`KismetSystemLibrary.PrintString` "FIRE"))

(event `StopFire`)

(fn `CheckAmmo`
  (returns (bAmmoAvalible :type Boolean))
  (bind _asbp_tsscharacter (cast `/Game/TSS/Blueprints/BP_TSSCharacter` (`self.GetOwner`))
    (:`then`
      (bind _ammo (`/Game/TSS/Blueprints/BP_TSSCharacter.Ammo` _asbp_tsscharacter))
      (bind (_value _returnvalue) (`BlueprintMapLibrary.Map_Find` _ammo (`GameplayStatics.GetObjectClass` self)))
      (if _returnvalue
        (if (> _value 0)
          (`BlueprintMapLibrary.Map_Add` _ammo (`GameplayStatics.GetObjectClass` self) (- _value 1))
          (return true)
          (else
            (return false)))
        (else
          (return false))))
    (:`CastFailed`
      (return false))))

(fn `UserConstructionScript`)
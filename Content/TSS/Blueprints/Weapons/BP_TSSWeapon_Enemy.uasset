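; Enemy weapon Blueprint that fires a shot from its muzzle arrow.
; Its Fire event spawns a scaled-down actor at ArrowMuzzle, oriented along the arrow's forward vector through a look-at rotation, then plays an attenuated shot sound there.
; The spawned class is not specified in the graph, and the construction script only calls the parent.
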(event `self.Fire`
  (bind _arrowmuzzle (`self.ArrowMuzzle`))
  (bind _returnvalue (`SceneComponent.K2_GetComponentLocation` _arrowmuzzle))
  (`|SpawnActorFromClass` "/Game/TSS/Blueprints/Weapons/BP_TSSProjectile_Enemy.BP_TSSProjectile_Enemy_C" (`KismetMathLibrary.MakeTransform` _returnvalue (`KismetMathLibrary.FindLookAtRotation` _returnvalue (+ _returnvalue (`SceneComponent.GetForwardVector` _arrowmuzzle))) (0.2 0.2 0.2)) "Undefined" "MultiplyWithRoot" null null)
  (`GameplayStatics.PlaySoundAtLocation` "/Game/TSS/Sounds/SC_Shot.SC_Shot" (`SceneComponent.K2_GetComponentLocation` (`self.ArrowMuzzle`)) (struct) 1.0 1.0 0.0 "/Game/TSS/Sounds/SA_Shot.SA_Shot" null null null))

(fn `UserConstructionScript`
  (`parent.UserConstructionScript`))
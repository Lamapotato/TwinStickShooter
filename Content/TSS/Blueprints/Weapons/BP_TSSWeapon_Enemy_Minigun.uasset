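; Enemy minigun weapon Blueprint that fires a short burst of scaled-down enemy projectiles.
; Fire starts a looping timer and resets the shot counter for the burst.
; Shoot spawns a projectile along the muzzle arrow with a positional sound, clearing the timer once the counter runs out.
; Tick spins the muzzle mesh around its roll axis while the timer handle is valid.
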(event `self.Fire`
  (bind _returnvalue (`KismetSystemLibrary.K2_SetTimerDelegate` (`|CreateDelegate` :!event `Shoot`) 0.1 true))
  (set `self.ShootingTimer` _returnvalue)
  (set `self.NumberOfShots` 4))

(event `Shoot`
  (bind _arrowmuzzle (`self.ArrowMuzzle`))
  (bind _returnvalue (`SceneComponent.K2_GetComponentLocation` _arrowmuzzle))
  (if (> (`self.NumberOfShots`) 0)
    (`|SpawnActorFromClass` "/Game/TSS/Blueprints/Weapons/BP_TSSProjectile_Enemy.BP_TSSProjectile_Enemy_C" (`KismetMathLibrary.MakeTransform` _returnvalue (`KismetMathLibrary.FindLookAtRotation` _returnvalue (+ _returnvalue (`SceneComponent.GetForwardVector` _arrowmuzzle))) (0.2 0.2 0.2)) "Undefined" "MultiplyWithRoot" null null)
    (`GameplayStatics.PlaySoundAtLocation` "/Game/TSS/Sounds/SC_Shot.SC_Shot" (`SceneComponent.K2_GetComponentLocation` (`self.ArrowMuzzle`)) (struct) 1.0 1.0 0.0 "/Game/TSS/Sounds/SA_Shot.SA_Shot" null null null)
    (`/Engine/EditorBlueprintResources/StandardMacros.DecrementInt` (`self.NumberOfShots`))
    (else
      (`KismetSystemLibrary.K2_ClearAndInvalidateTimerHandle` (`self.ShootingTimer`)))))

(event `self.ReceiveTick`
  (params (DeltaSeconds :type "Float (single-precision)"))
  (if (`KismetSystemLibrary.K2_IsValidTimerHandle` (`self.ShootingTimer`))
    (`SceneComponent.K2_AddRelativeRotation` (`self.SM_Muzzle_MG`) (`KismetMathLibrary.MakeRotator` (* (`self.RotationSpeed`) (`GameplayStatics.GetWorldDeltaSeconds`))) false false)))

(fn `UserConstructionScript`
  (`parent.UserConstructionScript`))
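; BP_TSSWeapon_2 is a child weapon Blueprint that implements the Fire event for a projectile gun.
; When the ammo check passes, it spawns a scaled-down BP_TSSProjectile at the muzzle arrow, aimed along that arrow's forward vector.
; It also spawns a Niagara muzzle effect at the mesh's Muzzle socket and plays an attenuated pistol shot sound.
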(event `self.Fire`
  (bind _arrowmuzzle (`self.ArrowMuzzle`))
  (bind _returnvalue (`SceneComponent.K2_GetComponentLocation` _arrowmuzzle))
  (bind (_returnvalue_location _returnvalue_rotation) (`KismetMathLibrary.BreakTransform` (`SceneComponent.GetSocketTransform` (`self.WeaponMesh`) "Muzzle" "RTS_World")))
  (bind _bammoavalible (`self.CheckAmmo`))
  (if _bammoavalible
    (`|SpawnActorFromClass` "/Game/TSS/Blueprints/Weapons/BP_TSSProjectile.BP_TSSProjectile_C" (`KismetMathLibrary.MakeTransform` _returnvalue (`KismetMathLibrary.FindLookAtRotation` _returnvalue (+ _returnvalue (`SceneComponent.GetForwardVector` _arrowmuzzle))) (0.2 0.2 0.2)) "Undefined" "MultiplyWithRoot" null null)
    (`NiagaraFunctionLibrary.SpawnSystemAtLocation` "/Game/Lesson/VFX/NS_Muzzle.NS_Muzzle" _returnvalue_location _returnvalue_rotation)
    (`GameplayStatics.PlaySoundAtLocation` "/Game/TSS/Sounds/163456__lemudcrab__pistol-shot.163456__lemudcrab__pistol-shot" (`SceneComponent.K2_GetComponentLocation` (`self.ArrowMuzzle`)) (struct) 1.0 1.0 0.0 "/Game/TSS/Sounds/SA_Shot.SA_Shot" null null null)))

(fn `UserConstructionScript`
  (`parent.UserConstructionScript`))
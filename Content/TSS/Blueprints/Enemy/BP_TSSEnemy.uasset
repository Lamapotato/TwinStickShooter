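; TSS enemy Blueprint that patrols, investigates noises and chases the player, with a swappable attached weapon.
; AIMoveTo callbacks loop random patrols until HearNoise interrupts them, showing a camera-facing text indicator while the enemy investigates before resuming.
; PawnSensing sight triggers a self-repeating chase that plays a montage on reaching the player and an alert sound throttled by a timed DoOnce.
; ChangeWeapon replaces the current weapon actor at WeaponRoot.
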(event `self.ReceiveTick`
  (params (DeltaSeconds :type "Float (single-precision)"))
  (bind _textrender (`self.TextRender`))
  (`SceneComponent.K2_SetWorldRotation` _textrender (`KismetMathLibrary.FindLookAtRotation` (`SceneComponent.K2_GetComponentLocation` _textrender) (`SceneComponent.K2_GetComponentLocation` (`PlayerCameraManager.TransformComponent` (`GameplayStatics.GetPlayerCameraManager` 0)))) false false))

(event `self.ReceiveBeginPlay`
  (`self.Patrol`))

(event `Patrol`
  (`|AIMoveTo` self (`NavigationSystemV1.K2_GetRandomReachablePointInRadius` (`self.K2_GetActorLocation`) 2000.0 null null) null
    (:`OnSuccess`
      (`KismetSystemLibrary.Delay` 1.0))
    (:`OnFail`
      _))
  (if (`self.CanPatroll`)
    (`self.Patrol`)))

(event `Chase Player`
  (`|ExecutionSequence`
    (:`then_0`
      (`SceneComponent.SetVisibility` (`self.TextRender`) false false)
      (`|AIMoveTo` self (0.0 0.0 0.0) (`GameplayStatics.GetPlayerCharacter` 0)
        (:`OnSuccess`
          (`/Engine/EditorBlueprintResources/StandardMacros.DoOnce` false :!label _label
            (:`Completed`
              (`|PlayMontage` (`self.Mesh`)
                (:`OnCompleted`
                  (`|ExecutionSequence`
                    (:`then_0`
                      (goto _label :!via `Reset`))
                    (:`then_1`
                      (`self.Chase Player`))))))))
        (:`OnFail`
          (`KismetSystemLibrary.Delay` 0.2)
          (`self.Chase Player`))))
    (:`then_1`
      (if true
        (set `self.LastSoundTime` (`KismetSystemLibrary.GetGameTimeInSeconds`))
        (`/Engine/EditorBlueprintResources/StandardMacros.DoOnce` false :!label _label_2
          (:`Completed`
            (`GameplayStatics.PlaySoundAtLocation` "/Game/TSS/Models/Alert01.Alert01" (`self.K2_GetActorLocation`) (struct) 1.0 1.0 0.0 null null null null)
            (`KismetSystemLibrary.Delay` 60.0)
            (goto _label_2 :!via `Reset`)))))))

(event `/Game/TSS/Blueprints/Enemy/BPI_Hear.HearNoise`
  (params (Location :type "Vector Structure"))
  (set `self.CanPatroll` false)
  (`SceneComponent.SetVisibility` (`self.TextRender`) true false)
  (`|AIMoveTo` self Location null
    (:`OnSuccess`
      (set `self.CanPatroll` true)
      (`KismetSystemLibrary.Delay` 5.0)
      (if (`self.CanPatroll`)
        (`SceneComponent.SetVisibility` (`self.TextRender`) false false)
        (`self.Patrol`)))))

(event `self.PawnSensing.OnSeePawn`
  (params (Pawn :type "Pawn Object Reference"))
  (`self.Chase Player`))

(fn `ChangeWeapon`
  (params (WeaponClass :type "/Game/TSS/Blueprints/BP_TSSWeapon Class Reference"))
  (`/Engine/EditorBlueprintResources/StandardMacros.IsValid` (`self.Weapon`)
    (:`Is Valid`
      (`self.K2_DestroyActor` (`self.Weapon`)))
    (:`Is Not Valid`
      _))
  (bind _returnvalue (`|SpawnActorFromClass` WeaponClass (`KismetMathLibrary.MakeTransform` (`SceneComponent.K2_GetComponentLocation` (`self.WeaponRoot`))) "AlwaysSpawn" "MultiplyWithRoot" null null))
  (bind _output_get (set `self.Weapon` _returnvalue))
  (`self.K2_AttachToComponent` _output_get (`self.WeaponRoot`) "None" "KeepWorld" "KeepWorld" "KeepWorld" true)
  (`self.K2_SetActorRelativeRotation` :`self` _output_get))

(fn `UserConstructionScript`)
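; BP_TSSEnemySpawner is an enemy spawner that works through a queue of enemy classes on a looping timer.
; Each tick of the timer spawns the first queued class at the Billboard's location, adjusting for collisions, then removes it from the queue.
; When IsInfinite is set, each spawned enemy's destruction appends its class back to the queue, so the spawner replenishes as enemies are destroyed.
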(event `self.ReceiveBeginPlay`
  (`KismetSystemLibrary.K2_SetTimerDelegate` (`|CreateDelegate` :!event `SpawnEnemy`) (`self.SpawnInterval`) true))

(event `SpawnEnemy`
  (bind _enemiestospawn (`self.EnemiesToSpawn`))
  (if (`KismetArrayLibrary.Array_IsValidIndex` _enemiestospawn)
    (bind _returnvalue (`|SpawnActorFromClass` (`|GetArrayItem` _enemiestospawn) (`KismetMathLibrary.MakeTransform` (`SceneComponent.K2_GetComponentLocation` (`self.Billboard`))) "AdjustIfPossibleButAlwaysSpawn" "MultiplyWithRoot" null null))
    (`KismetArrayLibrary.Array_Remove` (`self.EnemiesToSpawn`))
    (if (`self.IsInfinite`)
      (add `self.OnDestroyed` _returnvalue (`|CreateDelegate` :!event `EnemyDestroyed`)))))

(event `EnemyDestroyed` :!signature `self.OnDestroyed`
  (params (DestroyedActor :type "Actor Object Reference"))
  (bind _asbp_tssenemy (castclass `/Game/TSS/Blueprints/BP_TSSEnemy` (`GameplayStatics.GetObjectClass` DestroyedActor)))
  (`KismetArrayLibrary.Array_Add` (`self.EnemiesToSpawn`) _asbp_tssenemy))

(fn `UserConstructionScript`)
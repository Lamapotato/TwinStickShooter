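; BP_TSS_ENEMY_VLAD1 is an enemy that walks to switched-off lamps and turns them back on.
; A Delay on Tick rescans all BP_TSSLamp actors about every half second and moves to the first unlit one, not the nearest, via AIMoveTo.
; On arrival it sets IsOn and raises the light's intensity.
; FindNextOfLamp still returns an array element when none are unlit; player-facing rotation logic is disconnected.
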(event `self.ReceiveTick`
  (params (DeltaSeconds :type "Float (single-precision)"))
  (`KismetSystemLibrary.Delay` 0.5)
  (bind _outactors (`GameplayStatics.GetAllActorsOfClass` "/Game/TSS/Blueprints/BP_TSSLamp.BP_TSSLamp_C"))
  (set `self.AllLamps` _outactors)
  (bind _foundlamp (`self.FindNextOfLamp`))
  (`/Engine/EditorBlueprintResources/StandardMacros.IsValid` _foundlamp
    (:`Is Valid`
      (bind _output_get (set `self.TargetLamp` _foundlamp))
      (`|AIMoveTo` self (0.0 0.0 0.0) _output_get 5.0 (stale _output_get_2)
        (:`OnSuccess`
          (bind _output_get_2 (set `/Game/TSS/Blueprints/BP_TSSLamp.IsOn` true _output_get))
          (`LightComponent.SetIntensity` (`/Game/TSS/Blueprints/BP_TSSLamp.PointLight` _output_get) 5000.0))))))

(event `/Game/TSS/Blueprints/BPI_Interactable.Interact`)

(event `MoveToLamp`)

(event `self.ReceiveBeginPlay`)

(fn `FindNextOfLamp`
  (returns (FoundLamp :type "/Game/TSS/Blueprints/BP_TSSLamp Object Reference"))
  (for _array_element (`self.AllLamps`)
    (if (not (`/Game/TSS/Blueprints/BP_TSSLamp.IsOn` _array_element))
      (return _array_element)))
  (return _array_element))

(fn `UserConstructionScript`)
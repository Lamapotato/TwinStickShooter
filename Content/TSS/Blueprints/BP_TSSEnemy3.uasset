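; BP_TSSEnemy3 is an enemy character that patrols a looping list of Target actors and chases pawns it sees.
; Patrol uses AIMoveTo with a pause between points, while PawnSensing switches to chasing and plays an alert sound throttled by a DoOnce.
; A retriggerable delay ends the chase shortly after sightings stop, then halts movement and resumes patrol.
; ChangeWeapon replaces the current weapon with a spawned one attached to WeaponRoot.
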(event `OnMove3`
  (if (not (`self.IsChasing`))
    (`/Engine/EditorBlueprintResources/StandardMacros.IncrementInt` (`self.int`) :!label _label
      (:`  `
        (if (> (`self.int`) (`KismetArrayLibrary.Array_LastIndex` (`self.Target`)))
          (set `self.int` 0))
        (`|AIMoveTo` self (0.0 0.0 0.0) (`|GetArrayItem` (`self.Target`) (`self.int`))
          (:`OnSuccess`
            _)
          (:`OnFail`
            _))
        (`KismetSystemLibrary.Delay` 3.0)
        (`self.OnMove3`)))))

(event `self.ReceiveBeginPlay`
  (goto _label))

(event `self.PawnSensing.OnSeePawn`
  (params (Pawn :type "Pawn Object Reference"))
  (set `self.IsChasing` true)
  (`|ExecutionSequence`
    (:`then_0`
      (`|AIMoveTo` self (0.0 0.0 0.0) Pawn))
    (:`then_1`
      (`KismetSystemLibrary.RetriggerableDelay` 1.0)
      (set `self.IsChasing` false)
      (`|ExecutionSequence`
        (:`then_1`
          (`MovementComponent.StopMovementImmediately` (`self.CharacterMovement`))
          (`self.OnMove3`))))
    (:`then_2`
      (if true
        (set `self.LastSoundTime` (`KismetSystemLibrary.GetGameTimeInSeconds`))
        (`/Engine/EditorBlueprintResources/StandardMacros.DoOnce` false :!label _label_2
          (:`Completed`
            (`GameplayStatics.PlaySoundAtLocation` "/Game/TSS/Models/S_EnemyAlert_Cue.S_EnemyAlert_Cue" (`self.K2_GetActorLocation`) (struct) 1.0 1.0 0.0 null null null null)
            (`KismetSystemLibrary.Delay` 60.0)
            (goto _label_2 :!via `Reset`)))))))

(fn `ChangeWeapon`
  (params (WeaponClass :type "/Game/TSS/Blueprints/BP_TSSWeapon Class Reference"))
  (`/Engine/EditorBlueprintResources/StandardMacros.IsValid` (`self.Weapon`)
    (:`Is Valid`
      (`self.K2_DestroyActor` (`self.Weapon`)))
    (:`Is Not Valid`
      _))
  (bind _returnvalue (`|SpawnActorFromClass` WeaponClass (`KismetMathLibrary.MakeTransform` (`SceneComponent.K2_GetComponentLocation` (`self.WeaponRoot`))) "AlwaysSpawn" "MultiplyWithRoot" null null))
  (bind _output_get (set `self.Weapon` _returnvalue))
  (`self.K2_AttachToComponent` _output_get (`self.WeaponRoot`) "None" "KeepWorld" "KeepWorld" "KeepWorld" true)
  (`self.K2_SetActorRelativeRotation` :`self` _output_get))

(fn `UserConstructionScript`)
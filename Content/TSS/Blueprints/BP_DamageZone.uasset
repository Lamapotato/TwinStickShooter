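; BP_DamageZone is a box-shaped zone that periodically damages a BP_TSSCharacter standing inside it.
; On begin overlap it stores the character, applies BaseDamage immediately and starts a looping timer at DamagePeriod for repeated damage.
; It tracks one character at a time, clearing the timer and reference when that stored character leaves the box.
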(event `self.Box.OnComponentBeginOverlap`
  (params (OverlappedComponent :type "PrimitiveComponent Object Reference") (OtherActor :type "Actor Object Reference") (OtherComp :type "PrimitiveComponent Object Reference") (OtherBodyIndex :type Integer) (bFromSweep :type Boolean) (SweepResult :type "HitResult Structure (by ref)"))
  (bind _asbp_tsscharacter (cast `/Game/TSS/Blueprints/BP_TSSCharacter` OtherActor))
  (bind _output_get (set `self.As BP TSSCharacter` _asbp_tsscharacter))
  (`GameplayStatics.ApplyDamage` _output_get (`self.Base Damage`))
  (bind _returnvalue (`KismetSystemLibrary.K2_SetTimerDelegate` (`|CreateDelegate` :!event `DamageTick`) (`self.DamagePeriod`) true))
  (set `self.DamageTimer` _returnvalue))

(event `DamageTick`
  (`GameplayStatics.ApplyDamage` (`self.As BP TSSCharacter`) (`self.Base Damage`)))

(event `self.Box.OnComponentEndOverlap`
  (params (OverlappedComponent :type "PrimitiveComponent Object Reference") (OtherActor :type "Actor Object Reference") (OtherComp :type "PrimitiveComponent Object Reference") (OtherBodyIndex :type Integer))
  (if (== (`self.As BP TSSCharacter`) OtherActor)
    (`KismetSystemLibrary.K2_ClearAndInvalidateTimerHandle` (`self.DamageTimer`))
    (set `self.As BP TSSCharacter` null)))

(fn `UserConstructionScript`)
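; TSS character Blueprint that can swap the weapon it carries at runtime.
; ChangeWeapon destroys any current weapon, spawns the given class at the WeaponRoot location and stores it as Weapon.
; The new weapon attaches to WeaponRoot keeping world transform, then has its relative rotation zeroed to align with that root.
; BeginPlay and the construction script are empty, and nothing in these graphs calls ChangeWeapon.
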(event `self.ReceiveBeginPlay`)

(fn `ChangeWeapon`
  (params (WeaponClass :type "/Game/TSS/Blueprints/BP_TSSWeapon Class Reference"))
  (`/Engine/EditorBlueprintResources/StandardMacros.IsValid` (`self.Weapon`)
    (:`Is Valid`
      (`self.K2_DestroyActor` (`self.Weapon`)))
    (:`Is Not Valid`
      _))
  (bind _returnvalue (`|SpawnActorFromClass` WeaponClass (`KismetMathLibrary.MakeTransform` (`SceneComponent.K2_GetComponentLocation` (`self.WeaponRoot`))) "AlwaysSpawn" "MultiplyWithRoot" null null))
  (bind _output_get (set `self.Weapon` _returnvalue))
  (`self.K2_AttachToComponent` _output_get (`self.WeaponRoot`) "None" "KeepWorld" "KeepWorld" "KeepWorld" true)
  (`self.K2_SetActorRelativeRotation` :`self` _output_get))

(fn `UserConstructionScript`)
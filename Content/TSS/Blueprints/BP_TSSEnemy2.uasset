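; Enemy AI character for TSS that patrols a looping list of target actors and attacks the player on sight.
; Patrol chains AIMoveTo calls with a pause at each point.
; AI Perception sensing a BP_TSSCharacter switches it to chasing with focus and a self-repeating, delayed ShootStep firing projectiles from an arrow component; losing the player resumes patrol.
; A weapon is attached at BeginPlay, and ChangeWeapon supports swapping weapon actors.
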(event `OnMove`
  (`/Engine/EditorBlueprintResources/StandardMacros.IncrementInt` (`self.int`) :!label _label
    (:`  `
      (if (> (`self.int`) (`KismetArrayLibrary.Array_LastIndex` (`self.Target`)))
        (set `self.int` 0))
      (`|AIMoveTo` self (0.0 0.0 0.0) (`|GetArrayItem` (`self.Target`) (`self.int`)) 50.0
        (:`OnSuccess`
          _)
        (:`OnFail`
          _))
      (`KismetSystemLibrary.Delay` 3.0)
      (if (not (`self.IsChasing`))
        (`self.OnMove`)))))

(event `self.ReceiveBeginPlay`
  (bind _returnvalue (`|SpawnActorFromClass` "/Game/TSS/Blueprints/BP_TSSWeapon_2.BP_TSSWeapon_2_C" (`KismetMathLibrary.MakeTransform` (0.0 0.0 0.0)) "Undefined" "MultiplyWithRoot" null null))
  (set `self.MyWeapon` _returnvalue)
  (`self.K2_AttachToComponent` (`self.MyWeapon`) (`self.WeaponRoot`) "None" "SnapToTarget" "SnapToTarget" "KeepRelative" true)
  (goto _label))

(event `self.AIPerception.OnTargetPerceptionUpdated`
  (params (Actor :type "Actor Object Reference") (Stimulus :type "AIStimulus Structure"))
  (bind _asbp_tsscharacter (cast `/Game/TSS/Blueprints/BP_TSSCharacter` Actor))
  (set `self.TargetPlayer` _asbp_tsscharacter)
  (if (`.bSuccessfullySensed` (break `AIStimulus` Stimulus))
    (`self.ShootStep`)
    (`AIController.K2_SetFocus` (`AIBlueprintHelperLibrary.GetAIController` null) (`self.TargetPlayer`))
    (`MovementComponent.StopMovementImmediately` (`self.CharacterMovement`))
    (set `self.IsChasing` true)
    (`|AIMoveTo` self (0.0 0.0 0.0) (`self.TargetPlayer`) 50.0)
    (else
      (set `self.IsChasing` false)
      (`KismetSystemLibrary.Delay` 3.0)
      (`self.OnMove`))))

(event `ShootStep`
  (`KismetSystemLibrary.PrintString` "ShootStep")
  (if (`self.IsChasing`)
    (`|SpawnActorFromClass` "/Game/TSS/Blueprints/BP_TSSProjectile.BP_TSSProjectile_C" (`SceneComponent.K2_GetComponentToWorld` (`self.Arrow1`)) "AlwaysSpawn" "MultiplyWithRoot" null null)
    (`KismetSystemLibrary.Delay` 1.0)
    (`self.ShootStep`)))

(fn `ChangeWeapon`
  (params (WeaponClass :type "/Game/TSS/Blueprints/BP_TSSWeapon Class Reference"))
  (`/Engine/EditorBlueprintResources/StandardMacros.IsValid` (`self.Weapon`)
    (:`Is Valid`
      (`self.K2_DestroyActor` (`self.Weapon`)))
    (:`Is Not Valid`
      _))
  (bind _returnvalue (`|SpawnActorFromClass` WeaponClass (`KismetMathLibrary.MakeTransform` (`SceneComponent.K2_GetComponentLocation` (`self.WeaponRoot`))) "AlwaysSpawn" "MultiplyWithRoot" null null))
  (bind _output_get (set `self.Weapon` _returnvalue))
  (`self.K2_AttachToComponent` _output_get (`self.WeaponRoot`) "None" "KeepWorld" "KeepWorld" "KeepWorld" true)
  (`self.K2_SetActorRelativeRotation` :`self` _output_get))

(fn `UserConstructionScript`)
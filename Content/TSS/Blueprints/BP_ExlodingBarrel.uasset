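; Exploding barrel actor that detonates when it takes any damage, hurting nearby pawns.
; AnyDamage passes through a DoOnce into the explosion logic, which the Test event also triggers directly.
; The explosion spawns a particle effect, applies flat damage to pawns found by a sphere overlap around the Container within Radius, plays a sound, then destroys the barrel.
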(event `Test`
  (`GameplayStatics.SpawnEmitterAtLocation` "/Game/ExampleContent/Blueprint_Communication/Effects/P_Explosion_Bomb.P_Explosion_Bomb" (`self.K2_GetActorLocation`) :!label _label)
  (bind _outactors (`KismetSystemLibrary.SphereOverlapActors` (`SceneComponent.K2_GetComponentLocation` (`self.container`)) (`self.Radius`) (`|MakeArray` "ObjectTypeQuery3" :!type "EObjectTypeQuery Enum")))
  (for _array_element _outactors
    (`GameplayStatics.ApplyDamage` _array_element 5.0 null self))
  (`GameplayStatics.PlaySoundAtLocation` "/Game/TSS/Sounds/big-bang.big-bang" (`SceneComponent.K2_GetComponentLocation` (`self.container`)) (struct) 1.0 1.0 0.0 null null null null)
  (`self.K2_DestroyActor`))

(event `self.ReceiveAnyDamage`
  (params (Damage :type "Float (single-precision)") (DamageType :type "DamageType Object Reference") (InstigatedBy :type "Controller Object Reference") (DamageCauser :type "Actor Object Reference"))
  (`/Engine/EditorBlueprintResources/StandardMacros.DoOnce` false
    (:`Completed`
      (goto _label))))

(fn `UserConstructionScript`)
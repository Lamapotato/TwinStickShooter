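; Enemy actor for the TSS game that faces the player, shoots at them and, when MovingEnemy is set, repeatedly chases them.
; It spawns a weapon on WeaponRoot and fires on a looping, start-staggered timer only when a camera-channel trace hits the player character.
; Damage lowers Health, with the overhead text updated before subtraction.
; At zero it plays a weighted-random death sound and destroys itself and its weapon.
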(event `self.ReceiveBeginPlay`
  (bind _returnvalue (`GameplayStatics.GetPlayerPawn` 0))
  (`self.ChangeWeapon` "/Game/TSS/Blueprints/Weapons/BP_TSSWeapon_Enemy.BP_TSSWeapon_Enemy_C")
  (`KismetSystemLibrary.K2_SetTimerDelegate` (delegate `CallShootEvent`) 1.0 true false 0.0 1.0)
  (if (`self.MovingEnemy`)
    (`/Engine/EditorBlueprintResources/StandardMacros.IsValid` _returnvalue :!label _label
      (:`Is Valid`
        (`|AIMoveTo` self (0.0 0.0 0.0) _returnvalue
          (:`OnSuccess`
            _)
          (:`OnFail`
            _))
        (`KismetSystemLibrary.Delay` 1.0)
        (goto _label)))))

(event `CallShootEvent`
  (bind _outhit (`KismetSystemLibrary.LineTraceSingle` :`Start` (`SceneComponent.K2_GetComponentLocation` (`self.Arrow1`)) :`End` (`self.K2_GetActorLocation` (`GameplayStatics.GetPlayerPawn` 0)) :`TraceChannel` "TraceTypeQuery2" :`DrawTime` 2.0))
  (cast `/Game/TSS/Blueprints/BP_TSSCharacter` (`.HitActor` (`GameplayStatics.BreakHitResult` _outhit)))
  (`/Game/TSS/Blueprints/Weapons/BP_TSSWeapon.Fire` (`self.Weapon`)))

(event `self.ReceiveTick`
  (params (DeltaSeconds :type "Float (single-precision)"))
  (bind _returnvalue (`GameplayStatics.GetPlayerPawn` 0))
  (bind (_returnvalue_roll _returnvalue_pitch _returnvalue_yaw) (`KismetMathLibrary.BreakRotator` (`KismetMathLibrary.FindLookAtRotation` (`self.K2_GetActorLocation`) (`self.K2_GetActorLocation` _returnvalue))))
  (`/Engine/EditorBlueprintResources/StandardMacros.IsValid` _returnvalue
    (:`Is Valid`
      (`SceneComponent.K2_SetWorldRotation` (`self.SM_TargetBaseMesh`) (`KismetMathLibrary.MakeRotator` 0.0 0.0 _returnvalue_yaw) false false))))

(event `self.ReceiveAnyDamage`
  (params (Damage :type "Float (single-precision)") (DamageType :type "DamageType Object Reference") (InstigatedBy :type "Controller Object Reference") (DamageCauser :type "Actor Object Reference"))
  (`self.UpdateHealth`)
  (bind _output_get (set `self.Health` (- (`self.Health`) Damage)))
  (if (<= _output_get 0.0)
    (if (`KismetMathLibrary.RandomBoolWithWeight` 0.35)
      (`GameplayStatics.PlaySoundAtLocation` (`self.VilgelmSound`) (0.0 0.0 0.0) (struct) 1.0 1.0 0.0 null null null null)
      (else
        (`GameplayStatics.PlaySoundAtLocation` (`KismetArrayLibrary.Array_Random` (`self.SoundDeath`)) (0.0 0.0 0.0) (struct) 1.0 1.0 0.0 null null null null)))
    (`self.K2_DestroyActor`)))

(event `self.ReceiveDestroyed`
  (`/Engine/EditorBlueprintResources/StandardMacros.IsValid` (`self.Weapon`)
    (:`Is Valid`
      (`self.K2_DestroyActor` (`self.Weapon`)))))

(fn `ChangeWeapon`
  (params (WeaponClass :type "/Game/TSS/Blueprints/Weapons/BP_TSSWeapon Class Reference"))
  (`/Engine/EditorBlueprintResources/StandardMacros.IsValid` (`self.Weapon`)
    (:`Is Valid`
      (`self.K2_DestroyActor` (`self.Weapon`)))
    (:`Is Not Valid`
      _))
  (bind _returnvalue (`|SpawnActorFromClass` WeaponClass (`KismetMathLibrary.MakeTransform` (`SceneComponent.K2_GetComponentLocation` (`self.WeaponRoot`))) "AlwaysSpawn" "MultiplyWithRoot" null null))
  (bind _output_get (set `self.Weapon` _returnvalue))
  (`self.K2_AttachToComponent` _output_get (`self.WeaponRoot`) "None" "KeepWorld" "KeepWorld" "KeepWorld" true)
  (`self.K2_SetActorRelativeRotation` :`self` _output_get))

(fn `UpdateHealth`
  (`TextRenderComponent.K2_SetText` (`self.HealthTextRender`) (`KismetTextLibrary.Conv_IntToText` (`KismetMathLibrary.FTrunc` (`self.Health`)))))

(fn `UserConstructionScript`
  (`self.UpdateHealth`))
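; BP_DamageVolume is a box trigger that damages a BP_TSSCharacter and pushes it away on contact.
; When the character's capsule begins overlapping the box, it plays a lasgun impact sound at the volume and applies damage.
; A Timeline then feeds forced movement input along the direction from the volume to the character as a knockback.
; The PushCharacter function is an empty stub, with the push logic living in the EventGraph.
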(event `self.Box.OnComponentBeginOverlap`
  (params (OverlappedComponent :type "PrimitiveComponent Object Reference") (OtherActor :type "Actor Object Reference") (OtherComp :type "PrimitiveComponent Object Reference") (OtherBodyIndex :type Integer) (bFromSweep :type Boolean) (SweepResult :type "HitResult Structure (by ref)"))
  (bind _asbp_tsscharacter (cast `/Game/TSS/Blueprints/BP_TSSCharacter` OtherActor))
  (set `self.TSSCharacter` _asbp_tsscharacter)
  (if (== OtherComp (`Character.CapsuleComponent` _asbp_tsscharacter))
    (`GameplayStatics.PlaySoundAtLocation` "/Game/TSS/Sounds/234082__211redman112__lasgun-impact.234082__211redman112__lasgun-impact" (`self.K2_GetActorLocation`) (struct) 1.0 1.0 0.0 null null null null)
    (`GameplayStatics.ApplyDamage` (`self.TSSCharacter`) 1.0)
    (`Timeline|Timeline` :!via `PlayFromStart`
      (:`Update`
        (`Pawn.AddMovementInput` (`self.TSSCharacter`) (`KismetMathLibrary.Normal` (- (`self.K2_GetActorLocation` (`self.TSSCharacter`)) (`self.K2_GetActorLocation`))) 1.0 true)))))

(fn `PushCharacter`
  (params (Actor :type "Object Object Reference") (ActorComponent :type "Object Object Reference"))
  (locals (TSSCharacter :type "/Game/TSS/Blueprints/BP_TSSCharacter Object Reference")))

(fn `UserConstructionScript`)
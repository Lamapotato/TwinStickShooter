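; BP_Vlad_Patrool is an armed AI pawn that patrols a fixed rectangular route while firing on a timer.
; BeginPlay calls Weapon, starts a looping Shoot timer with randomized initial delay, then chains AI MoveTo nodes through four hard-coded corners, pausing at each.
; The route repeats only while moves succeed, as failures are unhandled.
; Tick yaws the weapon root toward the player pawn, independently of movement, and Shoot fires without range or visibility checks.
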(event `self.ReceiveBeginPlay`
  (`self.Weapon` null)
  (`KismetSystemLibrary.K2_SetTimerDelegate` (delegate `self.Shoot`) 3.0 true false 0.0 3.0)
  (`|AIMoveTo` self (-1999.0 288.0 849.0) null 0.0 :!label _label
    (:`then`
      (`KismetSystemLibrary.Delay` 4.0)
      (`|AIMoveTo` self (-1981.0 -1266.0 849.0) null 0.0
        (:`then`
          (`KismetSystemLibrary.Delay` 4.0)
          (`|AIMoveTo` self (-262.0 -1266.0 849.0) null 0.0
            (:`then`
              (`KismetSystemLibrary.Delay` 4.0)
              (`|AIMoveTo` self (-262.0 288.0 849.0) null 0.0
                (:`then`
                  (`KismetSystemLibrary.Delay` 4.0)
                  (goto _label))))))))))

(event `self.Shoot`
  (`/Game/TSS/Blueprints/BP_TSSWeapon.Fire` (`self.Weapom`)))

(event `self.ReceiveTick`
  (params (DeltaSeconds :type "Float (single-precision)"))
  (bind _returnvalue (`GameplayStatics.GetPlayerPawn` 0))
  (bind (_returnvalue_roll _returnvalue_pitch _returnvalue_yaw) (`KismetMathLibrary.BreakRotator` (`KismetMathLibrary.FindLookAtRotation` (`self.K2_GetActorLocation`) (`self.K2_GetActorLocation` _returnvalue))))
  (`/Engine/EditorBlueprintResources/StandardMacros.IsValid` _returnvalue
    (:`Is Valid`
      (`SceneComponent.K2_SetWorldRotation` (`self.Weaponroot`) (`KismetMathLibrary.MakeRotator` 0.0 0.0 _returnvalue_yaw) false false))))

(fn `UserConstructionScript`
  (`parent.UserConstructionScript`))
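; Two-stage shooter boss that fires enemy projectiles from two arrow components on a fast looping timer.
; While the shield sphere exists, a ping-ponging Timeline driven by a FlipFlop sweeps the arrows in mirrored arcs, spreading the shots.
; DeactivateShield destroys the sphere, centers both arrows and starts the second stage.
; In that stage, Tick smoothly turns the whole boss toward the player with RInterpTo.
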(event `self.ReceiveBeginPlay`
  (`KismetSystemLibrary.K2_SetTimerDelegate` (`|CreateDelegate` :!event `CustomEvent`) 0.05 true)
  (`/Engine/EditorBlueprintResources/StandardMacros.IsValid` (`self.Sphere`)
    (:`Is Valid`
      (`/Engine/EditorBlueprintResources/StandardMacros.FlipFlop` :!label _label
        (:`A`
          (bind (_direction _newtrack_0) (`Timeline|Timeline` :!via `PlayFromStart` :!label _label_2)
            (:`Update`
              (`/Engine/EditorBlueprintResources/StandardMacros.IsValid` (`self.Sphere`)
                (:`Is Valid`
                  (bind _returnvalue (`KismetMathLibrary.Lerp` -60.0 60.0 _newtrack_0))
                  (`SceneComponent.K2_SetRelativeRotation` (`self.Arrow1`) (`KismetMathLibrary.MakeRotator` 0.0 0.0 _returnvalue) false false)
                  (`SceneComponent.K2_SetRelativeRotation` (`self.Arrow`) (`KismetMathLibrary.MakeRotator` 0.0 0.0 (* _returnvalue -1.0)) false false))))
            (:`Finished`
              (goto _label))))
        (:`B`
          (goto _label_2 :!via `ReverseFromEnd`))))))

(event `CustomEvent`
  (bind _arrow1 (`self.Arrow1`))
  (bind _arrow (`self.Arrow`))
  (`|SpawnActorFromClass` "/Game/TSS/Blueprints/Weapons/BP_TSSProjectile_Enemy_BOSS.BP_TSSProjectile_Enemy_BOSS_C" (`KismetMathLibrary.MakeTransform` (`SceneComponent.K2_GetComponentLocation` _arrow) (`SceneComponent.K2_GetComponentRotation` _arrow) (0.2 0.2 0.2)) "Undefined" "MultiplyWithRoot" null null)
  (`|SpawnActorFromClass` "/Game/TSS/Blueprints/Weapons/BP_TSSProjectile_Enemy_BOSS.BP_TSSProjectile_Enemy_BOSS_C" (`KismetMathLibrary.MakeTransform` (`SceneComponent.K2_GetComponentLocation` _arrow1) (`SceneComponent.K2_GetComponentRotation` _arrow1) (0.2 0.2 0.2)) "Undefined" "MultiplyWithRoot" null null))

(event `DeactivateShield`
  (`ActorComponent.K2_DestroyComponent` (`self.Sphere`))
  (set `self.b2ndStage` true)
  (`SceneComponent.K2_SetRelativeRotation` (`self.Arrow1`) (`KismetMathLibrary.MakeRotator` 0.0) false false)
  (`SceneComponent.K2_SetRelativeRotation` (`self.Arrow`) (`KismetMathLibrary.MakeRotator` 0.0) false false))

(event `self.ReceiveTick`
  (params (DeltaSeconds :type "Float (single-precision)"))
  (if (`self.b2ndStage`)
    (`self.K2_SetActorRotation` (`KismetMathLibrary.RInterpTo` (`self.K2_GetActorRotation`) (`KismetMathLibrary.FindLookAtRotation` (`self.K2_GetActorLocation`) (`self.K2_GetActorLocation` (`GameplayStatics.GetPlayerPawn` 0))) (`GameplayStatics.GetWorldDeltaSeconds`) (`self.Interp Speed`)))))

(fn `UserConstructionScript`)
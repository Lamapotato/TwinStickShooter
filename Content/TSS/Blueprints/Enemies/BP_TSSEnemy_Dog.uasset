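; Dog enemy for TSS that spots the player, starts moving and bites at close range.
; A looping timer set on BeginPlay appears to drive a line-trace sight check, which on success starts movement, clears the timer and barks.
; The shoot event becomes a melee bite: bark, montage, delay, then sphere-overlap damage at the bite point.
; The mesh yaws toward the player, and PlayHitSound is empty.
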(event `self.ReceiveBeginPlay`
  (`parent.ReceiveBeginPlay`)
  (bind _returnvalue (`KismetSystemLibrary.K2_SetTimerDelegate` (`|CreateDelegate` :!event `CanSeePlayer`) 3.0 true))
  (set `self.CanSeeTimer` _returnvalue))

(event `self.CallShootEvent`
  (if (< (`KismetMathLibrary.Vector_Distance` (`self.K2_GetActorLocation`) (`self.K2_GetActorLocation` (`GameplayStatics.GetPlayerPawn` 0))) 200.0)
    (`GameplayStatics.PlaySoundAtLocation` "/Game/TSS/Sounds/SC_Bark.SC_Bark" (`self.K2_GetActorLocation`) (struct) 1.0 1.0 0.0 null null null null)
    (bind _returnvalue (`self.PlayAnimMontage` "/Game/TSS/Characters/Dog/Animations/Attack/Anim_Shepherd_dog_Attack_F_Montage.Anim_Shepherd_dog_Attack_F_Montage"))
    (`KismetSystemLibrary.Delay` (- _returnvalue (`self.AnimDurationOffset`)))
    (bind _outactors (`KismetSystemLibrary.SphereOverlapActors` (`SceneComponent.K2_GetComponentLocation` (`self.BiteLocation`)) (`self.BiteRadius`) (`|MakeArray` "ObjectTypeQuery3" :!type "EObjectTypeQuery Enum") "/Game/TSS/Blueprints/BP_TSSCharacter.BP_TSSCharacter_C"))
    (for _array_element _outactors
      (`GameplayStatics.ApplyDamage` _array_element 1.0 null self))))

(event `CanSeePlayer`
  (bind _outhit (`KismetSystemLibrary.LineTraceSingle` :`Start` (`SceneComponent.K2_GetComponentLocation` (`self.Arrow1`)) :`End` (`self.K2_GetActorLocation` (`GameplayStatics.GetPlayerPawn` 0)) :`TraceChannel` "TraceTypeQuery2" :`DrawTime` 2.0))
  (cast `/Game/TSS/Blueprints/BP_TSSCharacter` (`.HitActor` (`GameplayStatics.BreakHitResult` _outhit)))
  (`self.StartMoving`)
  (`KismetSystemLibrary.K2_ClearAndInvalidateTimerHandle` (`self.CanSeeTimer`))
  (`GameplayStatics.SpawnSoundAtLocation` "/Game/TSS/Sounds/418108__crazymonke9__dog-tripple-bark.418108__crazymonke9__dog-tripple-bark" (`self.K2_GetActorLocation`) (struct) 1.0 1.0 0.0 null null))

(event `self.ReceiveTick`
  (params (DeltaSeconds :type "Float (single-precision)"))
  (bind _returnvalue (`GameplayStatics.GetPlayerPawn` 0))
  (bind _mesh (`self.Mesh`))
  (bind (_returnvalue_roll _returnvalue_pitch) (`KismetMathLibrary.BreakRotator` (`SceneComponent.K2_GetComponentRotation` _mesh)))
  (bind (_returnvalue_roll_2 _returnvalue_pitch_2 _returnvalue_yaw) (`KismetMathLibrary.BreakRotator` (`KismetMathLibrary.FindLookAtRotation` (`self.K2_GetActorLocation`) (`self.K2_GetActorLocation` _returnvalue))))
  (`/Engine/EditorBlueprintResources/StandardMacros.IsValid` _returnvalue
    (:`Is Valid`
      (`SceneComponent.K2_SetWorldRotation` _mesh (`KismetMathLibrary.MakeRotator` _returnvalue_roll _returnvalue_pitch (+ _returnvalue_yaw -90.0)) false false))))

(fn `PlayHitSound`)

(fn `UserConstructionScript`
  (`parent.UserConstructionScript`))
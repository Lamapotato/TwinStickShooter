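; TSS enemy character that shoots at the player and optionally chases them through a repeating AI MoveTo.
; A looping timer traces to the player and fires the spawned, attached weapon only when the trace hits the player character.
; Tick yaws the base mesh toward the player.
; Damage plays random hit montages; death stops shooting, hides the health widget and destroys the enemy after a montage-timed delay, taking its weapon with it.
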(event `self.ReceiveBeginPlay`
  (`|ExecutionSequence`
    (:`then_0`
      (`self.ChangeWeapon` (`self.Weapon Class`))
      (bind _returnvalue (`KismetSystemLibrary.K2_SetTimerDelegate` (delegate `CallShootEvent`) (`self.TimeBetweenShots`) true false 0.0 1.0))
      (set `self.ShootEventTimer` _returnvalue)
      (if (`self.MovingEnemy`)
        (`self.StartMoving`)))
    (:`then_1`
      (bind _aswbp_enemy_health (cast `/Game/TSS/Blueprints/UI/WBP_EnemyHealth` (`WidgetComponent.GetUserWidgetObject` (`self.HealthWidget`))))
      (set `/Game/TSS/Blueprints/UI/WBP_EnemyHealth.Enemy` self _aswbp_enemy_health))))

(event `CallShootEvent`
  (bind _outhit (`KismetSystemLibrary.LineTraceSingle` :`Start` (`SceneComponent.K2_GetComponentLocation` (`self.Arrow1`)) :`End` (`self.K2_GetActorLocation` (`GameplayStatics.GetPlayerPawn` 0)) :`TraceChannel` "TraceTypeQuery2" :`DrawTime` 2.0))
  (cast `/Game/TSS/Blueprints/BP_TSSCharacter` (`.HitActor` (`GameplayStatics.BreakHitResult` _outhit)))
  (`/Game/TSS/Blueprints/Weapons/BP_TSSWeapon.Fire` (`self.Weapon`)))

(event `self.ReceiveTick`
  (params (DeltaSeconds :type "Float (single-precision)"))
  (bind _returnvalue (`GameplayStatics.GetPlayerPawn` 0))
  (bind _sm_targetbasemesh (`self.SM_TargetBaseMesh`))
  (bind (_returnvalue_roll _returnvalue_pitch) (`KismetMathLibrary.BreakRotator` (`SceneComponent.K2_GetComponentRotation` _sm_targetbasemesh)))
  (bind (_returnvalue_roll_2 _returnvalue_pitch_2 _returnvalue_yaw) (`KismetMathLibrary.BreakRotator` (`KismetMathLibrary.FindLookAtRotation` (`self.K2_GetActorLocation`) (`self.K2_GetActorLocation` _returnvalue))))
  (`/Engine/EditorBlueprintResources/StandardMacros.IsValid` _returnvalue
    (:`Is Valid`
      (`SceneComponent.K2_SetWorldRotation` _sm_targetbasemesh (`KismetMathLibrary.MakeRotator` _returnvalue_roll _returnvalue_pitch _returnvalue_yaw) false false))))

(event `self.ReceiveAnyDamage`
  (params (Damage :type "Float (single-precision)") (DamageType :type "DamageType Object Reference") (InstigatedBy :type "Controller Object Reference") (DamageCauser :type "Actor Object Reference"))
  (bind _output_get (set `self.Health` (- (`self.Health`) Damage)))
  (`self.PlayRandomAnimMontageFromArray` (`self.AnimMontagesHits`))
  (if (<= _output_get 0.0)
    (bind _animduration (`self.PlayRandomAnimMontageFromArray` (`self.AnimMontagesDeaths`)))
    (`CharacterMovementComponent.DisableMovement` (`self.CharacterMovement`))
    (`NavMovementInterface.StopActiveMovement` (`self.CharacterMovement`))
    (`SceneComponent.SetVisibility` (`self.HealthWidget`) false false)
    (`self.SetActorTickEnabled` false)
    (`KismetSystemLibrary.K2_ClearAndInvalidateTimerHandle` (`self.ShootEventTimer`))
    (set `self.bDead` true)
    (`KismetSystemLibrary.Delay` (- _animduration (`self.AnimDurationOffset`)))
    (`self.K2_DestroyActor`)))

(event `self.ReceiveDestroyed`
  (`/Engine/EditorBlueprintResources/StandardMacros.IsValid` (`self.Weapon`)
    (:`Is Valid`
      (`self.K2_DestroyActor` (`self.Weapon`)))))

(event `StartMoving`
  (bind _returnvalue (`GameplayStatics.GetPlayerPawn` 0))
  (`/Engine/EditorBlueprintResources/StandardMacros.IsValid` _returnvalue :!label _label
    (:`Is Valid`
      (`|AIMoveTo` self (0.0 0.0 0.0) _returnvalue
        (:`OnSuccess`
          _)
        (:`OnFail`
          _))
      (`KismetSystemLibrary.Delay` 1.0)
      (if (not (`self.bDead`))
        (goto _label)))))

(fn `ChangeWeapon`
  (params (WeaponClass :type "/Game/TSS/Blueprints/Weapons/BP_TSSWeapon Class Reference"))
  (if (`KismetSystemLibrary.IsValidClass` WeaponClass)
    (`/Engine/EditorBlueprintResources/StandardMacros.IsValid` (`self.Weapon`)
      (:`Is Valid`
        (`self.K2_DestroyActor` (`self.Weapon`)))
      (:`Is Not Valid`
        _))
    (bind _returnvalue (`|SpawnActorFromClass` WeaponClass (`KismetMathLibrary.MakeTransform` (`SceneComponent.K2_GetComponentLocation` (`self.WeaponRoot`))) "AlwaysSpawn" "MultiplyWithRoot" null null))
    (bind _output_get (set `self.Weapon` _returnvalue))
    (`self.K2_AttachToComponent` _output_get (`self.WeaponRoot`) "None" "KeepWorld" "KeepWorld" "KeepWorld" true)
    (`self.K2_SetActorRelativeRotation` :`self` _output_get)))

(fn `PlayRandomAnimMontageFromArray`
  (params (AnimMontagesArray :type "Array of AnimMontage Object Reference"))
  (returns (AnimDuration :type "Float (double-precision)"))
  (if (`KismetArrayLibrary.Array_IsNotEmpty` AnimMontagesArray)
    (bind _returnvalue (`self.PlayAnimMontage` (`KismetArrayLibrary.Array_Random` AnimMontagesArray)))
    (return _returnvalue)))

(fn `UserConstructionScript`
  (set `self.MaxHealth` (`self.Health`)))
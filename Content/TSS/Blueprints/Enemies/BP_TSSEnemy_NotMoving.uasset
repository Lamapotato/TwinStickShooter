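; BP_TSSEnemy_NotMoving is an enemy variant that can stay dormant until explicitly started.
; On BeginPlay it sets actor tick from a TickEnabled flag and runs the parent BeginPlay only when that flag is true.
; The StartEnemy event activates it later by enabling tick and calling the deferred parent BeginPlay, leaving enemy behavior to the parent class.
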(event `StartEnemy`
  (`self.SetActorTickEnabled` true)
  (`parent.ReceiveBeginPlay`))

(event `self.ReceiveBeginPlay`
  (`self.SetActorTickEnabled` (`self.TickEnabled`))
  (if (`self.TickEnabled`)
    (`parent.ReceiveBeginPlay`)))

(fn `UserConstructionScript`
  (`parent.UserConstructionScript`))
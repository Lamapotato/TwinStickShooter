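; BP_TSSWeapon_1 is a hitscan weapon Blueprint that damages whatever actor its shot hits.
; Its Fire event runs a short line trace on the Camera channel, straight forward from the ArrowMuzzle component, with debug drawing on.
; The hit actor goes straight into ApplyDamage for a fixed amount, without checking the trace result.
; The construction script only calls its parent, and the other events are unused stubs.
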(event `self.Fire`
  (bind _arrowmuzzle (`self.ArrowMuzzle`))
  (bind _returnvalue (`SceneComponent.K2_GetComponentLocation` _arrowmuzzle))
  (bind _outhit (`KismetSystemLibrary.LineTraceSingle` :`Start` _returnvalue :`End` (+ _returnvalue (* (`SceneComponent.GetForwardVector` _arrowmuzzle) 500.0)) :`TraceChannel` "TraceTypeQuery2" :`DrawDebugType` "ForDuration"))
  (`GameplayStatics.ApplyDamage` (`.HitActor` (`GameplayStatics.BreakHitResult` _outhit)) 10.0))

(fn `UserConstructionScript`
  (`parent.UserConstructionScript`))
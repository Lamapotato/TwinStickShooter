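; BP_TSSDoor_Locked is a door that only passes interaction on when the player holds every keycard it requires.
; On Interact, it checks each entry in Neededkeycards against the Keycards array on the player's BP_TSSCharacter.
; Each missing card prints an on-screen message naming its type from the keycard's class defaults.
; If none is flagged missing, it calls the parent Interact to run the inherited behavior.
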(event `/Game/TSS/Blueprints/BPI_Interactable.Interact`
  (set `self.NoNeededKeycard` false)
  (bind _asbp_tsscharacter (cast `/Game/TSS/Blueprints/BP_TSSCharacter` (`GameplayStatics.GetPlayerPawn` 0)))
  (for _array_element (`self.Neededkeycards`)
    (bind _asbp_floating_item_keycard (castclass `/Game/TSS/Blueprints/Items/BP_FloatingItem_Keycard` _array_element))
    (if (== (`KismetArrayLibrary.Array_Find` (`/Game/TSS/Blueprints/BP_TSSCharacter.Keycards` _asbp_tsscharacter) _array_element) -1)
      (set `self.NoNeededKeycard` true)
      (`KismetSystemLibrary.PrintString` (`KismetTextLibrary.Conv_TextToString` (`|FormatText` "You still need \"{type}\" keycard" (defaults `Object` _asbp_floating_item_keycard))))))
  (if (not (`self.NoNeededKeycard`))
    (`parent.Interact`)))

(fn `UserConstructionScript`
  (`parent.UserConstructionScript`))
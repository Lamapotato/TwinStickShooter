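; Grenade projectile Blueprint that explodes on hit, dealing area damage around the impact point.
; The Hit event runs a sphere overlap limited to WorldDynamic objects, applies flat damage without falloff to each actor found, then destroys the projectile.
; A temporary debug sphere shows the blast radius, and there is no other active event logic.
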(event `self.ReceiveHit`
  (params (MyComp :type "PrimitiveComponent Object Reference") (Other :type "Actor Object Reference") (OtherComp :type "PrimitiveComponent Object Reference") (bSelfMoved :type Boolean) (HitLocation :type "Vector Structure") (HitNormal :type "Vector Structure") (NormalImpulse :type "Vector Structure") (Hit :type "HitResult Structure (by ref)"))
  (`KismetSystemLibrary.DrawDebugSphere` HitLocation 200.0 12 (struct :`R` 1.0 :`A` 1.0) 2.0 1.0)
  (bind _outactors (`KismetSystemLibrary.SphereOverlapActors` HitLocation 200.0 (`|MakeArray` "ObjectTypeQuery2" :!type "EObjectTypeQuery Enum")))
  (for _array_element _outactors
    (`GameplayStatics.ApplyDamage` _array_element 20.0))
  (`self.K2_DestroyActor`))

(fn `UserConstructionScript`
  (`parent.UserConstructionScript`))
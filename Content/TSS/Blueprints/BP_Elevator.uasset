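; BP_Elevator is an elevator that carries a platform mesh along a spline when a BP_TSSCharacter enters its trigger box.
; After a one-second delay, a Timeline drives the mesh by spline distance, playing forward or in reverse according to GoingDown.
; On finish it flips GoingDown and resets the DoOnce that blocks retriggering.
; The construction script places the mesh at the spline's end when GoingDown is false.
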(event `self.box.OnComponentBeginOverlap`
  (params (OverlappedComponent :type "PrimitiveComponent Object Reference") (OtherActor :type "Actor Object Reference") (OtherComp :type "PrimitiveComponent Object Reference") (OtherBodyIndex :type Integer) (bFromSweep :type Boolean) (SweepResult :type "HitResult Structure (by ref)"))
  (bind _spline (`self.Spline`))
  (cast `/Game/TSS/Blueprints/BP_TSSCharacter` OtherActor)
  (`/Engine/EditorBlueprintResources/StandardMacros.DoOnce` false :!label _label
    (:`Completed`
      (`KismetSystemLibrary.Delay` 1.0)
      (if (`self.bGoingDown`)
        (`KismetSystemLibrary.PrintString` "Hello")
        (bind (_direction _newtrack_0) (`Timeline|Timeline` :!via `PlayFromStart` :!label _label_2)
          (:`Update`
            (`SceneComponent.K2_SetWorldLocation` (`self.StaticMesh`) (`SplineComponent.GetLocationAtDistanceAlongSpline` _spline (* _newtrack_0 (`SplineComponent.GetSplineLength` _spline)) "World") false false))
          (:`Finished`
            (set `self.bGoingDown` (not (`self.bGoingDown`)))
            (goto _label :!via `Reset`)))
        (else
          (goto _label_2 :!via `ReverseFromEnd`))))))

(fn `UserConstructionScript`
  (bind _spline (`self.Spline`))
  (if (not (`self.bGoingDown`))
    (`SceneComponent.K2_SetWorldLocation` (`self.StaticMesh`) (`SplineComponent.GetLocationAtDistanceAlongSpline` _spline (`SplineComponent.GetSplineLength` _spline) "World") false false)))
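; BP_RoomGenerator is a room builder that turns instanced floor and wall pieces into individual actors and scatters health kits.
; SpawnRoom uses SpawnActorsFromInstances to spawn a StaticMeshActor for each instance in two instanced mesh components.
; ScatterHealthPacks line-traces from random offsets around the actor and spawns healthkit pickups at hits, with debug drawing on.
; Grid layout code with perimeter walls and corners is disconnected, leaving the construction script empty.
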(event `SpawnRoom`
  (`self.SpawnActorsFromInstances` (`self.InstancedStaticMesh`))
  (`self.SpawnActorsFromInstances` (`self.InstancedStaticMesh1`)))

(event `ScatterHealthPacks`
  (bind _returnvalue (+ (* (`KismetMathLibrary.RandomUnitVector`) (`self.ScatterDistance`)) (`self.K2_GetActorLocation`)))
  (for _ (range (+ (`self.NumberOfHealthkits`) 1))
    (bind (_outhit _returnvalue_2) (`KismetSystemLibrary.LineTraceSingle` :`Start` _returnvalue :`End` (- _returnvalue (0.0 0.0 500.0)) :`TraceChannel` "TraceTypeQuery1" :`DrawDebugType` "ForDuration"))
    (if _returnvalue_2
      (`|SpawnActorFromClass` "/Game/TSS/Blueprints/Items/BP_FloatingItem_Healthkit.BP_FloatingItem_Healthkit_C" (`KismetMathLibrary.MakeTransform` (`.Location` (`GameplayStatics.BreakHitResult` _outhit))) "Undefined" "MultiplyWithRoot" null null))))

(fn `SpawnActorsFromInstances`
  (params (InputPin :type "InstancedStaticMeshComponent Object Reference"))
  (for _index (range (+ (`InstancedStaticMeshComponent.GetInstanceCount` InputPin) 1))
    (bind _returnvalue (`|SpawnActorFromClass` "/Script/Engine.StaticMeshActor" (`InstancedStaticMeshComponent.GetInstanceTransform` InputPin _index true) "AlwaysSpawn" "MultiplyWithRoot" null null))
    (`StaticMeshComponent.SetStaticMesh` (`StaticMeshActor.StaticMeshComponent` _returnvalue) (`StaticMeshComponent.StaticMesh` InputPin)))
  (return))

(fn `UserConstructionScript`
  (locals (z :type "Float (single-precision)" :default 0.0) (Offset :type "Vector Structure")))
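; BP_PuzzlePiece is a piece in a slot-based sliding puzzle that moves into an empty adjacent slot when selected.
; SelectPiece scans the current slot's Neighbors and takes the first one without a valid piece.
; It clears the old slot, links itself and the new slot to each other, then has that slot update the puzzle location.
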(event `SelectPiece`
  (for _array_element (`/Game/TSS/Blueprints/Puzzle/BP_PuzzleSlot.Neighbors` (`self.PuzzleSlot`))
    (set `self.NewSlot` _array_element)
    (`/Engine/EditorBlueprintResources/StandardMacros.IsValid` (`/Game/TSS/Blueprints/Puzzle/BP_PuzzleSlot.PuzzlePiece` (`self.NewSlot`))
      (:`Is Not Valid`
        (set `/Game/TSS/Blueprints/Puzzle/BP_PuzzleSlot.PuzzlePiece` null (`self.PuzzleSlot`))
        (set `/Game/TSS/Blueprints/Puzzle/BP_PuzzleSlot.PuzzlePiece` self (`self.NewSlot`))
        (set `self.PuzzleSlot` (`self.NewSlot`))
        (`/Game/TSS/Blueprints/Puzzle/BP_PuzzleSlot.UpdatePuzzleLocation` (`self.NewSlot`))
        (break)))))

(fn `UserConstructionScript`)
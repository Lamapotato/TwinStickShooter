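; BP_PuzzleSlot is a puzzle slot actor that holds a reference to a puzzle piece and positions it.
; UpdatePuzzleLocation moves a valid piece to sit 50 units above the slot, without sweep.
; The construction script runs that update and writes the slot back into the piece's PuzzleSlot, linking both at construction.
; That back-reference write has no validity check.
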(event `UpdatePuzzleLocation`
  (`/Engine/EditorBlueprintResources/StandardMacros.IsValid` (`self.PuzzlePiece`)
    (:`Is Valid`
      (`self.K2_SetActorLocation` (`self.PuzzlePiece`) (+ (`self.K2_GetActorLocation`) (0.0 0.0 50.0)) false false))))

(fn `UserConstructionScript`
  (`self.UpdatePuzzleLocation`)
  (set `/Game/TSS/Blueprints/Puzzle/BP_PuzzlePiece.PuzzleSlot` self (`self.PuzzlePiece`)))
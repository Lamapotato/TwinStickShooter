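; BP_TSSEnemy_Patrol_DZ is an enemy that patrols along a list of target points.
; On BeginPlay it moves via AI Move To toward the current point, then increments the index and wraps to the first after the last.
; A failed move also advances to the next point, so the patrol loops for as long as the index stays valid.
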(event `self.ReceiveBeginPlay`
  (bind _targetpoints (`self.TargetPoints`))
  (bind _patroltargetindrx (`self.PatrolTargetIndrx`))
  (if (`KismetArrayLibrary.Array_IsValidIndex` _targetpoints _patroltargetindrx) :!label _label
    (`|AIMoveTo` self (0.0 0.0 0.0) (`|GetArrayItem` _targetpoints _patroltargetindrx)
      (:`OnSuccess`
        _)
      (:`OnFail`
        _))
    (bind _result (`/Engine/EditorBlueprintResources/StandardMacros.IncrementInt` (`self.PatrolTargetIndrx`))
      (:`  `
        (if (< _result (`KismetArrayLibrary.Array_Length` (`self.TargetPoints`)))
          (goto _label)
          (else
            (set `self.PatrolTargetIndrx` 0)
            (goto _label)))))))

(fn `UserConstructionScript`
  (`parent.UserConstructionScript`))
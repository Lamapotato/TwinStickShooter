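; BP_FloatingItem_Ammo is an ammo pickup, a child floating item that grants ammunition to the player character.
; On PickupItem it casts player pawn 0 to BP_TSSCharacter and adds Amount to the current count for AmmoClass in that character's Ammo map, then destroys itself.
; The pickup sound plays from the Destroyed event at the actor's location, so it fires on any destruction of the item.
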(event `self.PickupItem`
  (bind _asbp_tsscharacter (cast `/Game/TSS/Blueprints/BP_TSSCharacter` (`GameplayStatics.GetPlayerPawn` 0)))
  (bind _ammo (`/Game/TSS/Blueprints/BP_TSSCharacter.Ammo` _asbp_tsscharacter))
  (`BlueprintMapLibrary.Map_Add` _ammo (`self.AmmoClass`) (+ (`BlueprintMapLibrary.Map_Find` _ammo (`self.AmmoClass`)) (`self.Amount`)))
  (`self.K2_DestroyActor`))

(event `self.ReceiveDestroyed`
  (`GameplayStatics.SpawnSoundAtLocation` "/Game/TSS/Sounds/SC_PickupAmmo.SC_PickupAmmo" (`self.K2_GetActorLocation`) (struct) 1.0 1.0 0.0 null null))

(fn `UserConstructionScript`
  (`parent.UserConstructionScript`))
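; BP_FloatingItem_Healthkit is a health pickup that heals the player's TSS character.
; Its PickupItem event casts the first player pawn to BP_TSSCharacter, applies negative damage scaled from its Health value as healing, then destroys itself.
; The Destroyed event plays a power-up sound at the item's location, so the cue fires on any destruction.
; Construction defers to the parent class.
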(event `self.PickupItem`
  (bind _asbp_tsscharacter (cast `/Game/TSS/Blueprints/BP_TSSCharacter` (`GameplayStatics.GetPlayerPawn` 0)))
  (`GameplayStatics.ApplyDamage` _asbp_tsscharacter (* (`self.Health`) -1.0))
  (`self.K2_DestroyActor`))

(event `self.ReceiveDestroyed`
  (`GameplayStatics.SpawnSoundAtLocation` "/Game/TSS/Sounds/531176__ryusa__synth-chiptune-8-bit-ui-interface-item-use-health-power-up.531176__ryusa__synth-chiptune-8-bit-ui-interface-item-use-health-power-up" (`self.K2_GetActorLocation`) (struct) 1.0 1.0 0.0 null null))

(fn `UserConstructionScript`
  (`parent.UserConstructionScript`))
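; BP_Vlad is an enemy bot that chases and shoots at the player, and is destroyed with its weapon when damage drains its Health.
; BeginPlay spawns a BP_TSSWeapon_2 on Weaponroot, starts a looping timer that fires it, and re-issues AIMoveTo toward the player through a zero-delay loop.
; Tick turns only the mesh's yaw to face the player.
; A line-of-sight trace is present but unconnected, so firing ignores visibility.
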(event `self.ReceiveAnyDamage`
  (params (Damage :type "Float (single-precision)") (DamageType :type "DamageType Object Reference") (InstigatedBy :type "Controller Object Reference") (DamageCauser :type "Actor Object Reference"))
  ;[0.04711 0.15 0.03519 0.5] Хп бота
  (bind _output_get (set `self.Health` (- (`self.Health`) Damage)))
  (if (<= _output_get 0.0)
    (`self.K2_DestroyActor`)
    (`self.K2_DestroyActor` (`self.Weapom`))))

(event `self.ReceiveTick`
  (params (DeltaSeconds :type "Float (single-precision)"))
  (bind _returnvalue (`GameplayStatics.GetPlayerPawn` 0))
  (bind (_returnvalue_roll _returnvalue_pitch _returnvalue_yaw) (`KismetMathLibrary.BreakRotator` (`KismetMathLibrary.FindLookAtRotation` (`self.K2_GetActorLocation`) (`self.K2_GetActorLocation` _returnvalue))))
  ;[0.15 0.1245 0 0.5] Поворот за игроком
  (`/Engine/EditorBlueprintResources/StandardMacros.IsValid` _returnvalue
    (:`Is Valid`
      (`SceneComponent.K2_SetWorldRotation` (`self.StaticMesh`) (`KismetMathLibrary.MakeRotator` 0.0 0.0 _returnvalue_yaw) false false))))

(event `self.ReceiveBeginPlay`
  (bind _returnvalue (`GameplayStatics.GetPlayerPawn` 0))
  ;[0.03406 0.1363 0.15 0.5] Хождение за игроком
  (`self.Weapon` null)
  (`KismetSystemLibrary.K2_SetTimerDelegate` (delegate `Shoot`) 3.0 true false 0.0 3.0)
  (`/Engine/EditorBlueprintResources/StandardMacros.IsValid` _returnvalue :!label _label
    (:`Is Valid`
      (`|AIMoveTo` self (0.0 0.0 0.0) _returnvalue
        (:`then`
          (`KismetSystemLibrary.Delay` 0.0)
          (goto _label))))))

(event `Shoot`
  (`/Game/TSS/Blueprints/BP_TSSWeapon.Fire` (`self.Weapom`)))

(fn `UserConstructionScript`)

(fn `Weapon`
  (params (Class :type "Actor Object Reference"))
  (`/Engine/EditorBlueprintResources/StandardMacros.IsValid` (`self.Weapom`)
    (:`Is Valid`
      (`self.K2_DestroyActor` (`self.Weapom`)))
    (:`Is Not Valid`
      _))
  (bind _returnvalue (`|SpawnActorFromClass` "/Game/TSS/Blueprints/BP_TSSWeapon_2.BP_TSSWeapon_2_C" (`KismetMathLibrary.MakeTransform` (`SceneComponent.K2_GetComponentLocation` (`self.Weaponroot`))) "AlwaysSpawn" "MultiplyWithRoot" null null))
  (bind _output_get (set `self.Weapom` _returnvalue))
  (`self.K2_AttachToComponent` _output_get (`self.Weaponroot`) "None" "KeepWorld" "KeepWorld" "KeepWorld" true)
  (`self.K2_SetActorRelativeRotation` :`self` _output_get))
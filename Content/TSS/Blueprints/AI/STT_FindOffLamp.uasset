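; StateTree task that sends an AI actor to a switched-off TSS lamp to interact with it.
; On entering the state it scans all BP_TSSLamp actors and issues an AI MoveTo for each one that is off, without breaking the loop.
; A successful move calls Interact on the last stored lamp and finishes the task as succeeded.
; Move failure and finding no off lamp never finish the task.
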(event `self.ReceiveLatentEnterState`
  (params (Transition :type "StateTreeTransitionResult Structure (by ref)"))
  (bind _outactors (`GameplayStatics.GetAllActorsOfClass` "/Game/TSS/Blueprints/BP_TSSLamp.BP_TSSLamp_C"))
  (for _array_element _outactors
    (bind _asbp_tsslamp (cast `/Game/TSS/Blueprints/BP_TSSLamp` _array_element))
    (if (not (`/Game/TSS/Blueprints/BP_TSSLamp.IsOn` _asbp_tsslamp))
      (bind _output_get (set `self.As BP TSSLamp` _asbp_tsslamp))
      (`|AIMoveTo` (`self.Actor`) (0.0 0.0 0.0) _output_get
        (:`OnSuccess`
          (`/Game/TSS/Blueprints/BP_TSSLamp.Interact` (`self.As BP TSSLamp`))
          (`self.FinishTask` true))))))

(fn `NewFunction`)
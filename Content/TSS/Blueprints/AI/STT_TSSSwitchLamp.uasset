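; StateTree task that sends an AI pawn to switch on a disabled lamp.
; On entering the state it scans all BP_TSSLamp actors, breaks at the first one not enabled and moves the pawn to it with AIMoveTo.
; Arrival triggers the lamp's Interact; both success and failed moves finish the task as succeeded.
; When no lamp is disabled, FinishTask is never called.
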(event `self.ReceiveLatentEnterState`
  (params (Transition :type "StateTreeTransitionResult Structure (by ref)"))
  (bind _outactors (`GameplayStatics.GetAllActorsOfClass` "/Game/TSS/Blueprints/BP_TSSLamp.BP_TSSLamp_C"))
  (for _array_element _outactors
    (if (not (`/Game/TSS/Blueprints/BP_TSSLamp.IslampEnabled` _array_element))
      (`|ExecutionSequence`
        (:`then_0`
          (break))
        (:`then_1`
          (set `self.Lamp` _array_element)
          (`|AIMoveTo` (`self.Actor`) (0.0 0.0 0.0) (`self.Lamp`)
            (:`OnSuccess`
              (`/Game/TSS/Blueprints/BPI_Interactable.Interact` (`self.Lamp`))
              (`self.FinishTask` true))
            (:`OnFail`
              (`self.FinishTask` true))))))))
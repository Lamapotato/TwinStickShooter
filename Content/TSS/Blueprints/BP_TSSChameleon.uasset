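; BP_TSSChameleon is an interactable Blueprint that toggles a color between green and red.
; Each Interact event flips a FlipFlop that writes the Color vector in the MPC_TSSParams Material Parameter Collection, so every material reading that parameter changes together.
; An alternative per-instance approach, using a dynamic material instance on the Cube, remains in disconnected nodes and never runs.
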(event `/Game/TSS/Blueprints/BPI_Interactable.Interact`
  (`/Engine/EditorBlueprintResources/StandardMacros.FlipFlop`
    (:`A`
      (`KismetMaterialLibrary.SetVectorParameterValue` "/Game/TSS/Blueprints/MPC_TSSParams.MPC_TSSParams" "Color" (`self.Green`)))
    (:`B`
      (`KismetMaterialLibrary.SetVectorParameterValue` "/Game/TSS/Blueprints/MPC_TSSParams.MPC_TSSParams" "Color" (`self.Red`)))))

(fn `UserConstructionScript`)
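; Player character for a cursor-aimed shooter (stick-aimed on Android), handling movement, weapons, health, interaction, pause and lose screens.
; Enhanced Input actions and Mobile events share handlers; weapon switching spawns the owned weapon on a hand socket.
; Punching briefly raises BlockPlane; ProjectileParried triggers a global time-dilation hit stop that Tick ends by frame count.
; Damage pulses a material parameter and ragdolls at zero health; a sphere finds the nearest interactable.
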(event OnComponentBeginOverlap(Sphere)
  (params (OverlappedComponent :type Primitive%20Component%20Object%20Reference) (OtherActor :type Actor%20Object%20Reference) (OtherComp :type Primitive%20Component%20Object%20Reference) (OtherBodyIndex :type Integer) (bFromSweep :type Boolean) (SweepResult :type Hit%20Result%20Structure%20%28by%20ref%29))
  (Utilities|Casting|CastToBPI_Interactable OtherActor)
  (Math|Integer|IncrementInt (Variables|Default|GetInteractableCount)
    (:%20%20
      (Development|SetHiddeninGame (Variables|Default|GetTextRender) (not (> (Variables|Default|GetInteractableCount) 0)) false))))

(event OnComponentEndOverlap(Sphere)
  (params (OverlappedComponent :type Primitive%20Component%20Object%20Reference) (OtherActor :type Actor%20Object%20Reference) (OtherComp :type Primitive%20Component%20Object%20Reference) (OtherBodyIndex :type Integer))
  (Utilities|Casting|CastToBPI_Interactable OtherActor)
  (Math|Integer|DecrementInt (Variables|Default|GetInteractableCount)
    (:%20%20
      (Development|SetHiddeninGame (Variables|Default|GetTextRender) (not (> (Variables|Default|GetInteractableCount) 0)) false))))

(event Custom|RemovePauseMenu
  (Widget|RemovefromParent (Variables|Default|GetPauseMenu))
  (EventDispatchers|UnbindallEventsfromCallRemoveMenu (Variables|Default|GetPauseMenu))
  (Variables|Default|SetPauseMenu 0)
  (Game|SetGamePaused false))

(event Custom|MobileJump
  (Character|Jump))

(event Custom|ProjectileParried
  (Development|SetHiddeninGame (Variables|Default|GetBlockPlane) true false)
  (Collision|SetCollisionEnabled (Variables|Default|GetBlockPlane) "NoCollision")
  (Variables|Default|SetHitFrames 0)
  (Utilities|Time|SetGlobalTimeDilation 0.0))

(event Custom|ExitHitStop
  (Utilities|Time|SetGlobalTimeDilation 1.0))

(event Custom|MobileWeapon1
  (if (!= (Utilities|Array|FindItem (Variables|Default|GetAvalibleWeapons) "/Game/TSS/Blueprints/Weapons/BP_TSSWeapon_2.BP_TSSWeapon_2_C") -1)
    (CallFunction|ChangeWeapon "/Game/TSS/Blueprints/Weapons/BP_TSSWeapon_2.BP_TSSWeapon_2_C")))

(event Custom|MobileWeapon2
  (if (!= (Utilities|Array|FindItem (Variables|Default|GetAvalibleWeapons) "/Game/TSS/Blueprints/Weapons/BP_TSSWeapon_Minigun.BP_TSSWeapon_Minigun_C") -1)
    (CallFunction|ChangeWeapon "/Game/TSS/Blueprints/Weapons/BP_TSSWeapon_Minigun.BP_TSSWeapon_Minigun_C")))

(event Custom|MobileWeapon3
  (if (!= (Utilities|Array|FindItem (Variables|Default|GetAvalibleWeapons) "/Game/ИванПаскарь/BP_Ракетница.BP_Ракетница_C") -1)
    (CallFunction|ChangeWeapon "/Game/ИванПаскарь/BP_Ракетница.BP_Ракетница_C")))

(event Custom|MobileFireStart
  (Utilities|IsValid (Variables|Default|GetWeapon)
    (:Is%20Valid
      (Default|Fire (Variables|Default|GetWeapon)))))

(event Custom|MobileFireStop
  (Utilities|IsValid (Variables|Default|GetWeapon)
    (:Is%20Valid
      (Default|StopFire (Variables|Default|GetWeapon)))))

(event Custom|MobilePunch
  (Development|SetHiddeninGame (Variables|Default|GetBlockPlane) false false)
  (Collision|SetCollisionEnabled (Variables|Default|GetBlockPlane) "QueryAndPhysics")
  (Animation|PlayAnimMontage "/Game/TSS/Animations/AM_cross_punch_Montage.AM_cross_punch_Montage" 3.0 "None")
  (Audio|PlaySoundatLocation "/Game/TSS/Sounds/SC_Punch.SC_Punch" (Transformation|GetActorLocation) "0, 0, 0" 1.0 1.0 0.0 0 0 0 0)
  (Utilities|FlowControl|Delay 0.5)
  (Development|SetHiddeninGame (Variables|Default|GetBlockPlane) true false)
  (Collision|SetCollisionEnabled (Variables|Default|GetBlockPlane) "NoCollision"))

(event Custom|MobilePause
  (Utilities|IsValid (Variables|Default|GetPauseMenu)
    (:Is%20Valid
      (CallFunction|RemovePauseMenu))
    (:Is%20Not%20Valid
      (bind _returnvalue (UserInterface|CreateWidget "/Game/TSS/Blueprints/UI/WBP_PauseMenu.WBP_PauseMenu_C"))
      (bind _output_get (Variables|Default|SetPauseMenu _returnvalue))
      (UserInterface|Viewport|AddtoViewport _output_get 0)
      (EventDispatchers|BindEventtoCallRemoveMenu _output_get (EventDispatchers|CreateEvent :!event Custom|RemovePauseMenu))
      (Game|SetGamePaused true))))

(event Custom|MobileInteract
  (bind _closestactor (CallFunction|OpenClosestDoor))
  (bind _asbpi_interactable (Utilities|Casting|CastToBPI_Interactable _closestactor))
  (Default|Interact _asbpi_interactable))

(event Input|EnhancedActionEvents|EnhancedInputActionIA_TSSMove
  (params (ActionValue :type Vector%202D%20Structure) (ElapsedSeconds :type Float%20%28double-precision%29) (TriggeredSeconds :type Float%20%28double-precision%29) (InputAction :type Input%20Action%20Object%20Reference :default "/Game/TSS/Blueprints/Input/IA_TSSMove.IA_TSSMove"))
  (bind (_x _y) (Math|Vector2D|BreakVector2D ActionValue))
  (bind _mesh (Variables|Character|GetMesh))
  (:Triggered
    (Class|PawnMovementComponent|AddInputVector (Variables|Character|GetCharacterMovement) (Math|Vector|MakeVector _x _y 0.0) false))
  (:Started
    (Components|Animation|SetAnimation _mesh "/Game/Characters/Mannequins/Anims/Rifle/Walk/MF_Rifle_Walk_Fwd.MF_Rifle_Walk_Fwd"))
  (:Completed
    (Components|Animation|SetAnimation _mesh "/Game/Characters/Mannequins/Anims/Rifle/MF_Rifle_Idle_ADS.MF_Rifle_Idle_ADS")))

(event Input|EnhancedActionEvents|EnhancedInputActionIA_TSSInteract
  (params (ActionValue :type Boolean) (ElapsedSeconds :type Float%20%28double-precision%29) (TriggeredSeconds :type Float%20%28double-precision%29) (InputAction :type Input%20Action%20Object%20Reference :default "/Game/TSS/Blueprints/Input/IA_TSSInteract.IA_TSSInteract"))
  (bind _closestactor (CallFunction|OpenClosestDoor))
  (bind _asbpi_interactable (Utilities|Casting|CastToBPI_Interactable _closestactor))
  (Default|Interact _asbpi_interactable))

(event Input|EnhancedActionEvents|EnhancedInputActionIA_TSSPunch
  (params (ActionValue :type Boolean) (ElapsedSeconds :type Float%20%28double-precision%29) (TriggeredSeconds :type Float%20%28double-precision%29) (InputAction :type Input%20Action%20Object%20Reference :default "/Game/TSS/Blueprints/Input/IA_TSSPunch.IA_TSSPunch"))
  (Development|SetHiddeninGame (Variables|Default|GetBlockPlane) false false)
  (Collision|SetCollisionEnabled (Variables|Default|GetBlockPlane) "QueryAndPhysics")
  (Animation|PlayAnimMontage "/Game/TSS/Animations/AM_cross_punch_Montage.AM_cross_punch_Montage" 3.0 "None")
  (Audio|PlaySoundatLocation "/Game/TSS/Sounds/SC_Punch.SC_Punch" (Transformation|GetActorLocation) "0, 0, 0" 1.0 1.0 0.0 0 0 0 0)
  (Utilities|FlowControl|Delay 0.5)
  (Development|SetHiddeninGame (Variables|Default|GetBlockPlane) true false)
  (Collision|SetCollisionEnabled (Variables|Default|GetBlockPlane) "NoCollision"))

(event Input|EnhancedActionEvents|EnhancedInputActionIA_TSSJump
  (params (ActionValue :type Boolean) (ElapsedSeconds :type Float%20%28double-precision%29) (TriggeredSeconds :type Float%20%28double-precision%29) (InputAction :type Input%20Action%20Object%20Reference :default "/Game/TSS/Blueprints/Input/IA_TSSJump.IA_TSSJump"))
  (Character|Jump))

(event Input|EnhancedActionEvents|EnhancedInputActionIA_TSSSelectWeapon1
  (params (ActionValue :type Boolean) (ElapsedSeconds :type Float%20%28double-precision%29) (TriggeredSeconds :type Float%20%28double-precision%29) (InputAction :type Input%20Action%20Object%20Reference :default "/Game/TSS/Blueprints/Input/IA_TSSSelectWeapon1.IA_TSSSelectWeapon1"))
  (if (!= (Utilities|Array|FindItem (Variables|Default|GetAvalibleWeapons) "/Game/TSS/Blueprints/Weapons/BP_TSSWeapon_2.BP_TSSWeapon_2_C") -1)
    (CallFunction|ChangeWeapon "/Game/TSS/Blueprints/Weapons/BP_TSSWeapon_2.BP_TSSWeapon_2_C")))

(event Input|EnhancedActionEvents|EnhancedInputActionIA_TSSPause
  (params (ActionValue :type Boolean) (ElapsedSeconds :type Float%20%28double-precision%29) (TriggeredSeconds :type Float%20%28double-precision%29) (InputAction :type Input%20Action%20Object%20Reference :default "/Game/TSS/Blueprints/Input/IA_TSSPause.IA_TSSPause"))
  (Utilities|IsValid (Variables|Default|GetPauseMenu)
    (:Is%20Valid
      (CallFunction|RemovePauseMenu))
    (:Is%20Not%20Valid
      (bind _returnvalue (UserInterface|CreateWidget "/Game/TSS/Blueprints/UI/WBP_PauseMenu.WBP_PauseMenu_C"))
      (bind _output_get (Variables|Default|SetPauseMenu _returnvalue))
      (UserInterface|Viewport|AddtoViewport _output_get 0)
      (EventDispatchers|BindEventtoCallRemoveMenu _output_get (EventDispatchers|CreateEvent :!event Custom|RemovePauseMenu))
      (Game|SetGamePaused true))))

(event Input|EnhancedActionEvents|EnhancedInputActionIA_TSSSelectWeapon2
  (params (ActionValue :type Boolean) (ElapsedSeconds :type Float%20%28double-precision%29) (TriggeredSeconds :type Float%20%28double-precision%29) (InputAction :type Input%20Action%20Object%20Reference :default "/Game/TSS/Blueprints/Input/IA_TSSSelectWeapon2.IA_TSSSelectWeapon2"))
  (if (!= (Utilities|Array|FindItem (Variables|Default|GetAvalibleWeapons) "/Game/TSS/Blueprints/Weapons/BP_TSSWeapon_Minigun.BP_TSSWeapon_Minigun_C") -1)
    (CallFunction|ChangeWeapon "/Game/TSS/Blueprints/Weapons/BP_TSSWeapon_Minigun.BP_TSSWeapon_Minigun_C")))

(event Input|EnhancedActionEvents|EnhancedInputActionIA_TSSFire
  (params (ActionValue :type Boolean) (ElapsedSeconds :type Float%20%28double-precision%29) (TriggeredSeconds :type Float%20%28double-precision%29) (InputAction :type Input%20Action%20Object%20Reference :default "/Game/TSS/Blueprints/Input/IA_TSSFire.IA_TSSFire"))
  (:Started
    (Utilities|IsValid (Variables|Default|GetWeapon)
      (:Is%20Valid
        (Default|Fire (Variables|Default|GetWeapon)))))
  (:Canceled
    (Utilities|IsValid (Variables|Default|GetWeapon)
      (:Is%20Valid
        (Default|StopFire (Variables|Default|GetWeapon))))))

(event Input|EnhancedActionEvents|EnhancedInputActionIA_TSSSelectWeapon3
  (params (ActionValue :type Boolean) (ElapsedSeconds :type Float%20%28double-precision%29) (TriggeredSeconds :type Float%20%28double-precision%29) (InputAction :type Input%20Action%20Object%20Reference :default "/Game/TSS/Blueprints/Input/IA_TSSSelectWeapon3.IA_TSSSelectWeapon3"))
  (if (!= (Utilities|Array|FindItem (Variables|Default|GetAvalibleWeapons) "/Game/ИванПаскарь/BP_Ракетница.BP_Ракетница_C") -1)
    (CallFunction|ChangeWeapon "/Game/ИванПаскарь/BP_Ракетница.BP_Ракетница_C")))

(event Input|EnhancedActionEvents|EnhancedInputActionIA_TSSAim
  (params (ActionValue :type Vector%202D%20Structure) (ElapsedSeconds :type Float%20%28double-precision%29) (TriggeredSeconds :type Float%20%28double-precision%29) (InputAction :type Input%20Action%20Object%20Reference :default "/Game/TSS/Blueprints/Input/IA_TSSAim.IA_TSSAim"))
  (bind _returnvalue (Transformation|GetActorLocation))
  (bind (_x _y) (Math|Vector2D|BreakVector2D ActionValue))
  (switch string (Game|GetPlatformName)
    (:Android
      (Transformation|SetRelativeRotation (Variables|Character|GetMesh) (Math|Rotator|MakeRotator 0.0 0.0 (.yaw (Math|Rotator|FindLookatRotation _returnvalue (+ _returnvalue (Math|Vector|MakeVector _x _y 0.0))))) false false))))

(event EventBeginPlay
  (bind _returnvalue (Game|GetPlayerController 0))
  (bind _returnvalue_2 (PlayerController|LocalPlayerSubsystems|GetEnhancedInputLocalPlayerSubsystem _returnvalue))
  (Development|SetHiddeninGame (Variables|Default|GetBlockPlane) true false)
  (Collision|SetCollisionEnabled (Variables|Default|GetBlockPlane) "NoCollision")
  (Class|EnhancedInputSubsystemInterface|ClearAllMappings _returnvalue_2)
  (Input|AddMappingContext _returnvalue_2 "/Game/TSS/Blueprints/Input/IMC_TSSMovent.IMC_TSSMovent" 0 "(bIgnoreAllPressedKeysUntilRelease=True,bForceImmediately=False,bNotifyUserSettings=False)")
  (Variables|/Script/Engine.PlayerController|SetbShowMouseCursor (Game|GetPlayerController 0) true)
  (bind _returnvalue_3 (UserInterface|CreateWidget "/Game/TSS/Blueprints/UI/WBP_PlayerInfo.WBP_PlayerInfo_C" 0 0))
  (bind _output_get (Variables|Default|SetPlayerHealthWidget _returnvalue_3))
  (UserInterface|Viewport|AddtoViewport _output_get 0)
  (Variables|/Game/TSS/Blueprints/UI/WBP_PlayerInfo.WBP_PlayerInfo_C|SetCharacter (Variables|Default|GetPlayerHealthWidget) self))

(event EventTick
  (params (DeltaSeconds :type Float%20%28single-precision%29))
  (bind _returnvalue (Game|GetPlayerController 0))
  (bind (_hitresult _returnvalue_2) (Game|Player|GetHitResultUnderCursorbyChannel _returnvalue "TraceTypeQuery1" true))
  (Utilities|FlowControl|Sequence
    (:then_0
      (Utilities|Casting|CastToPlayerController (Pawn|GetController))
      (switch string (Game|GetPlatformName)
        (:Default
          (if _returnvalue_2
            (Transformation|SetRelativeRotation (Variables|Character|GetMesh) (Math|Rotator|MakeRotator 0.0 0.0 (+ (.yaw (Math|Rotator|FindLookatRotation (Transformation|GetActorLocation) (.Location (Collision|BreakHitResult _hitresult)))) -9e+01)) false false)))))
    (:then_1
      (if (Math|Float|NearlyEqual(Float) (Class|GameplayStatics|GetGlobalTimeDilation) 0.0001 1e-06)
        (bind _result (Math|Integer|IncrementInt (Variables|Default|GetHitFrames))
          (:%20%20
            (if (> _result 15)
              (CallFunction|ExitHitStop))))))
    (:then_2
      (if (Variables|Default|GetShowPath)
        (for _array_element (Variables|Default|GetOut%20Path%20Positions)
          (Rendering|Debug|DrawDebugSphere _array_element 1e+01 12 "(R=1.000000,G=1.000000,B=1.000000,A=1.000000)" 0.0))))))

(event Game|Damage|EventAnyDamage
  (params (Damage :type Float%20%28single-precision%29) (DamageType :type Damage%20Type%20Object%20Reference) (InstigatedBy :type Controller%20Object%20Reference) (DamageCauser :type Actor%20Object%20Reference))
  (bind _mesh (Variables|Character|GetMesh))
  (Utilities|FlowControl|Sequence
    (:then_0
      (bind _output_get (Variables|Default|SetHealth (Math|Float|Min(Float) (- (Variables|Default|GetHealth) Damage) (Variables|Default|GetMaxHealth))))
      (if (<= _output_get 0.0)
        (Utilities|FlowControl|DoOnce false
          (:Completed
            (Input|DisableInput (Game|GetPlayerController 0))
            (Physics|SetSimulatePhysics _mesh true)
            (Collision|SetCollisionProfileName _mesh "Ragdoll" true :!class /Script/Engine.PrimitiveComponent)
            (bind _returnvalue (UserInterface|CreateWidget "/Game/TSS/Blueprints/UI/WBP_Lose.WBP_Lose_C"))
            (UserInterface|Viewport|AddtoViewport _returnvalue 0)
            (Audio|PlaySound2D "/Game/TSS/Sounds/metal_gear_solid_game_over_screen_clean_background-1.metal_gear_solid_game_over_screen_clean_background-1" 1.0 1.0 0.0 0 0)))))
    (:then_1
      (if (> Damage 0.0)
        (Utilities|IsValid self
          (:Is%20Valid
            (bind _newtrack_0 (Timeline|Timeline PlayFromStart)
              (:Update
                (Rendering|Material|SetScalarParameterValue "/Game/TSS/Blueprints/MPC_TSSParams.MPC_TSSParams" "Damaged" _newtrack_0 :!class /Script/Engine.KismetMaterialLibrary)))))))))

(event EventDestroyed
  (if (not (Variables|Default|GetbIsWinning))
    (Input|DisableInput (Game|GetPlayerController 0))
    (bind _returnvalue (UserInterface|CreateWidget "/Game/TSS/Blueprints/UI/WBP_Lose.WBP_Lose_C"))
    (UserInterface|Viewport|AddtoViewport _returnvalue 0)))

(event Input|KeyboardEvents|DebugKey3
  (params (Key :type Key%20Structure :default "None") (ActionValue :type Input%20Action%20Value%20Structure)))

(event Input|KeyboardEvents|Add
  (params (Key :type Key%20Structure :default "None"))
  (:Pressed
    (Audio|SetSoundMixClassOverride "/Engine/EngineSounds/Duck_Normal_Attack_MixMod.Duck_Normal_Attack_MixMod" "/Game/TSS/Sounds/SC_Music.SC_Music" (Variables|Default|GetVolume) 1.0 1.0 true)
    (Audio|PushSoundMixModifier "/Engine/EngineSounds/Duck_Normal_Attack_MixMod.Duck_Normal_Attack_MixMod")
    (Math|Float|IncrementFloat (Variables|Default|GetVolume))))

(event Input|KeyboardEvents|Subtract
  (params (Key :type Key%20Structure :default "None")))

(fn ConstructionScript)

(fn ChangeWeapon
  (params (WeaponClass :type BP%20TSS%20Weapon%20Class%20Reference))
  (bind _mesh (Variables|Character|GetMesh))
  (Utilities|IsValid (Variables|Default|GetWeapon)
    (:Is%20Valid
      (Actor|DestroyActor (Variables|Default|GetWeapon)))
    (:Is%20Not%20Valid
      _))
  (bind _returnvalue (Game|SpawnActorfromClass WeaponClass (Math|Transform|MakeTransform (Transformation|GetWorldLocation _mesh) (Transformation|GetSocketRotation _mesh "hand_r_weapon") "1.000000,1.000000,1.000000") "AlwaysSpawn" "MultiplyWithRoot" self 0))
  (bind _output_get (Variables|Default|SetWeapon _returnvalue))
  (Transformation|AttachComponentToComponent _output_get (Variables|Character|GetMesh) "hand_r_weapon" "SnapToTarget" "SnapToTarget" "SnapToTarget" true)
  (Transformation|SetActorRelativeRotation _output_get))

(fn OpenClosestDoor
  (for _array_element (Collision|GetOverlappingActors (Variables|Default|GetSphere) "/Script/Engine.Actor" :!class /Script/Engine.PrimitiveComponent)
    (Utilities|Casting|CastToBPI_Interactable _array_element)
    (if (< (Transformation|GetDistanceTo self _array_element) (LocalVariables|GetClosestDistance))
      (LocalVariables|SetClosestDistance (Transformation|GetDistanceTo self _array_element))
      (LocalVariables|SetClosestInteractible _array_element)))
  (bind _asbpi_interactable (Utilities|Casting|CastToBPI_Interactable (LocalVariables|GetClosestInteractible))
    (:then
      (return _asbpi_interactable))
    (:CastFailed
      (return 0))))

(fn UpdatePitch
  (params (Pitch%20Multiplier :type Float%20%28single-precision%29))
  (Audio|Parameter|SetFloatParameter (Variables|Default|Get485076__inspectorj__heartbeat-regular-single-01-01-loop) "Pit" Pitch%20Multiplier :!class /Script/Engine.AudioComponent))
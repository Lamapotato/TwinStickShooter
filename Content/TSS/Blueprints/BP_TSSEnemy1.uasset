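; Enemy pawn Blueprint that patrols endlessly between actors in its Target array and can swap its held weapon.
; From BeginPlay, OnMove increments and wraps the index before each AI MoveTo, so the first destination is the second entry.
; Success and failure both pause briefly, then advance to the next target.
; ChangeWeapon, not called here, destroys any current weapon and attaches a newly spawned one to WeaponRoot.
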(event `OnMove`
  (`/Engine/EditorBlueprintResources/StandardMacros.IncrementInt` (`self.int`) :!label _label
    (:`  `
      (if (> (`self.int`) (`KismetArrayLibrary.Array_LastIndex` (`self.Target`)))
        (set `self.int` 0))
      (`|AIMoveTo` self (0.0 0.0 0.0) (`|GetArrayItem` (`self.Target`) (`self.int`))
        (:`OnSuccess`
          _)
        (:`OnFail`
          _))
      (`KismetSystemLibrary.Delay` 3.0)
      (`self.OnMove`))))

(event `self.ReceiveBeginPlay`
  (goto _label))

(fn `ChangeWeapon`
  (params (WeaponClass :type "/Game/TSS/Blueprints/BP_TSSWeapon Class Reference"))
  (`/Engine/EditorBlueprintResources/StandardMacros.IsValid` (`self.Weapon`)
    (:`Is Valid`
      (`self.K2_DestroyActor` (`self.Weapon`)))
    (:`Is Not Valid`
      _))
  (bind _returnvalue (`|SpawnActorFromClass` WeaponClass (`KismetMathLibrary.MakeTransform` (`SceneComponent.K2_GetComponentLocation` (`self.WeaponRoot`))) "AlwaysSpawn" "MultiplyWithRoot" null null))
  (bind _output_get (set `self.Weapon` _returnvalue))
  (`self.K2_AttachToComponent` _output_get (`self.WeaponRoot`) "None" "KeepWorld" "KeepWorld" "KeepWorld" true)
  (`self.K2_SetActorRelativeRotation` :`self` _output_get))

(fn `UserConstructionScript`)
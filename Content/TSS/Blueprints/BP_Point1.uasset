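; Waypoint actor that teleports itself among four fixed corners of a rectangle when BP_TSSCharacter overlaps its Box.
; A Sequence enters four chained DoOnce gates, each moving the actor and resetting the next, with the last re-arming the first.
; Each reset precedes that gate's Sequence pin, so one overlap can cascade through all four moves.
; A cast to BP_Vlad_Patrool is left unconnected.
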(event `self.Box.OnComponentBeginOverlap`
  (params (OverlappedComponent :type "PrimitiveComponent Object Reference") (OtherActor :type "Actor Object Reference") (OtherComp :type "PrimitiveComponent Object Reference") (OtherBodyIndex :type Integer) (bFromSweep :type Boolean) (SweepResult :type "HitResult Structure (by ref)"))
  (cast `/Game/TSS/Blueprints/BP_TSSCharacter` OtherActor)
  (`|ExecutionSequence`
    (:`then_0`
      (`/Engine/EditorBlueprintResources/StandardMacros.DoOnce` false :!label _label
        (:`Completed`
          (`self.K2_SetActorLocation` (-1999.0 288.0 849.0) false true)
          (goto _label_2 :!via `Reset`))))
    (:`then_1`
      (`/Engine/EditorBlueprintResources/StandardMacros.DoOnce` false :!label _label_2
        (:`Completed`
          (`self.K2_SetActorLocation` (-1981.0 -1266.0 849.0) false true)
          (goto _label_3 :!via `Reset`))))
    (:`then_2`
      (`/Engine/EditorBlueprintResources/StandardMacros.DoOnce` true :!label _label_3
        (:`Completed`
          (`self.K2_SetActorLocation` (-262.0 -1266.0 849.0) false true)
          (goto _label_4 :!via `Reset`))))
    (:`then_3`
      (`/Engine/EditorBlueprintResources/StandardMacros.DoOnce` true :!label _label_4
        (:`Completed`
          (`self.K2_SetActorLocation` (-262.0 288.0 849.0) false true)
          (goto _label :!via `Reset`))))))

(fn `UserConstructionScript`)
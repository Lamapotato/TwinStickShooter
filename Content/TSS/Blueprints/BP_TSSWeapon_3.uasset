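; BP_TSSWeapon_3 is a spread-shot weapon Blueprint that launches a burst of five projectiles each time it fires.
; The Fire event spawns scaled-down BP_TSSProjectile actors at the ArrowMuzzle location, ignoring collisions at spawn.
; Each projectile takes the muzzle's forward look-at rotation combined with a random pitch and yaw offset, producing a wide scattered cone.
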(event `self.Fire`
  (bind _arrowmuzzle (`self.ArrowMuzzle`))
  (bind _returnvalue (`SceneComponent.K2_GetComponentLocation` _arrowmuzzle))
  (for _ (range 1 6)
    (`|SpawnActorFromClass` "/Game/TSS/Blueprints/BP_TSSProjectile.BP_TSSProjectile_C" (`KismetMathLibrary.MakeTransform` _returnvalue (`KismetMathLibrary.ComposeRotators` (`KismetMathLibrary.FindLookAtRotation` _returnvalue (+ _returnvalue (`SceneComponent.GetForwardVector` _arrowmuzzle))) (`KismetMathLibrary.MakeRotator` 0.0 (`KismetMathLibrary.RandomFloatInRange` -30.0 30.0) (`KismetMathLibrary.RandomFloatInRange` -30.0 30.0))) (0.2 0.2 0.2)) "AlwaysSpawn" "MultiplyWithRoot" null null)))

(fn `UserConstructionScript`
  (`parent.UserConstructionScript`))
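; BP_TSS_ENEMY_VLAD2 is an enemy pawn that chases the player.
; On BeginPlay it issues an AI MoveTo toward the player pawn and, after each successful move and a short delay, issues it again; a failed move ends the loop.
; Every tick it sets its static mesh's world rotation to face the player, using only the look-at yaw.
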(event `self.ReceiveBeginPlay`
  (bind _returnvalue (`GameplayStatics.GetPlayerPawn` 0))
  (`/Engine/EditorBlueprintResources/StandardMacros.IsValid` _returnvalue :!label _label
    (:`Is Valid`
      (`|AIMoveTo` self (0.0 0.0 0.0) _returnvalue
        (:`OnSuccess`
          (`KismetSystemLibrary.Delay` 1.0)
          (goto _label))))))

(event `self.ReceiveTick`
  (params (DeltaSeconds :type "Float (single-precision)"))
  (bind _returnvalue (`GameplayStatics.GetPlayerPawn` 0))
  (bind (_returnvalue_roll _returnvalue_pitch _returnvalue_yaw) (`KismetMathLibrary.BreakRotator` (`KismetMathLibrary.FindLookAtRotation` (`self.K2_GetActorLocation`) (`self.K2_GetActorLocation` _returnvalue))))
  (`/Engine/EditorBlueprintResources/StandardMacros.IsValid` _returnvalue
    (:`Is Valid`
      (`SceneComponent.K2_SetWorldRotation` (`self.StaticMesh`) (`KismetMathLibrary.MakeRotator` 0.0 0.0 _returnvalue_yaw) false false))))

(fn `UserConstructionScript`)
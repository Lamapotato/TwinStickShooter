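; Enemy actor for the TSS game that yaws to face the player and, if MovingEnemy is set, repeatedly pursues them with AIMoveTo.
; Damage lowers Health and destroys it at zero; the health text refreshes before subtraction, so it lags one hit.
; A randomly staggered looping timer calls CallShootEvent, but that event and ChangeWeapon are empty.
; Their line-trace firing and weapon-spawning nodes are disconnected, so it never arms or shoots.
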(event `self.ReceiveBeginPlay`
  (bind _returnvalue (`GameplayStatics.GetPlayerPawn` 0))
  (`self.ChangeWeapon` "/Game/TSS/Blueprints/Weapons/BP_TSSWeapon_Enemy.BP_TSSWeapon_Enemy_C")
  (`KismetSystemLibrary.K2_SetTimerDelegate` (delegate `CallShootEvent`) 1.0 true false 0.0 1.0)
  (if (`self.MovingEnemy`)
    (`/Engine/EditorBlueprintResources/StandardMacros.IsValid` _returnvalue :!label _label
      (:`Is Valid`
        (`|AIMoveTo` self (0.0 0.0 0.0) _returnvalue
          (:`OnSuccess`
            _)
          (:`OnFail`
            _))
        (`KismetSystemLibrary.Delay` 1.0)
        (goto _label)))))

(event `CallShootEvent`)

(event `self.ReceiveTick`
  (params (DeltaSeconds :type "Float (single-precision)"))
  (bind _returnvalue (`GameplayStatics.GetPlayerPawn` 0))
  (bind (_returnvalue_roll _returnvalue_pitch _returnvalue_yaw) (`KismetMathLibrary.BreakRotator` (`KismetMathLibrary.FindLookAtRotation` (`self.K2_GetActorLocation`) (`self.K2_GetActorLocation` _returnvalue))))
  (`/Engine/EditorBlueprintResources/StandardMacros.IsValid` _returnvalue
    (:`Is Valid`
      (`SceneComponent.K2_SetWorldRotation` (`self.CapsuleComponent`) (`KismetMathLibrary.MakeRotator` 0.0 0.0 _returnvalue_yaw) false false))))

(event `self.ReceiveAnyDamage`
  (params (Damage :type "Float (single-precision)") (DamageType :type "DamageType Object Reference") (InstigatedBy :type "Controller Object Reference") (DamageCauser :type "Actor Object Reference"))
  (`self.UpdateHealth`)
  (bind _output_get (set `self.Health` (- (`self.Health`) Damage)))
  (if (<= _output_get 0.0)
    (`self.K2_DestroyActor`)))

(event `self.ReceiveDestroyed`
  (`/Engine/EditorBlueprintResources/StandardMacros.IsValid` (`self.Weapon`)
    (:`Is Valid`
      (`self.K2_DestroyActor` (`self.Weapon`)))))

(fn `ChangeWeapon`
  (params (WeaponClass :type "/Game/TSS/Blueprints/Weapons/BP_TSSWeapon Class Reference")))

(fn `UpdateHealth`
  (`TextRenderComponent.K2_SetText` (`self.HealthTextRender`) (`KismetTextLibrary.Conv_IntToText` (`KismetMathLibrary.FTrunc` (`self.Health`)))))

(fn `UserConstructionScript`
  (`self.UpdateHealth`))
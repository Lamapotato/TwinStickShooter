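; BP_Human_PavelTokarev is a lesson human Blueprint that shows its Name and can report its state through on-screen prints.
; The Construction Script writes Name into a TextRender component.
; PrintInfo prints Name only when Hungry, then prints the last Thoughts entry or a Russian "thinking about nothing" fallback.
; Both functions leave their parent calls unconnected, and the event graph holds only disabled default events.
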(fn `PrintInfo`
  (bind _thoughts (`self.Thoughts`))
  (if (`self.bHungry`)
    (`KismetSystemLibrary.PrintString` (`self.Name`)))
  (if (`KismetArrayLibrary.Array_IsNotEmpty` _thoughts)
    (`KismetSystemLibrary.PrintString` (`|GetArrayItem` _thoughts (`KismetArrayLibrary.Array_LastIndex` _thoughts)))
    (else
      (`KismetSystemLibrary.PrintString` "Ни о чем не думает"))))

(fn `UserConstructionScript`
  (`TextRenderComponent.K2_SetText` (`self.TextRender`) (`KismetTextLibrary.Conv_StringToText` (`self.Name`))))
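; BP_Human_Pavel_M is a lesson actor: a jointed human that plays a toilet-humor squat on BeginPlay, dropping a poop component (Какашечка).
; One timeline drives it: the Движение track rotates shoulder, pelvis and knee while lowering and shifting the whole actor.
; The Падение track lerps the poop downward from its cached relative position.
; The construction script shows a fixed entry from the Thoughts array on a TextRender.
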(event `self.ReceiveBeginPlay`
  (`parent.ReceiveBeginPlay`)
  (bind _output_get (set `self.Попа` (`SceneComponent.RelativeLocation` (`self.Какашечка`))))
  (bind _output_get_2 (set `self.Тело` (`self.K2_GetActorLocation`)))
  (bind (_direction `_движение` `_падение`) (`Timeline|Шкала времени`)
    (:`Update`
      (`|ExecutionSequence`
        (:`then_0`
          (`SceneComponent.K2_SetRelativeRotation` (`self.Плечо`) (`KismetMathLibrary.RLerp` (struct) (struct :`Roll` -90.0) `_движение`) false false)
          (`SceneComponent.K2_SetRelativeRotation` (`self.ТАЗ`) (`KismetMathLibrary.RLerp` (struct) (struct :`Roll` -90.0) `_движение`) false false)
          (`SceneComponent.K2_SetRelativeRotation` (`self.колено`) (`KismetMathLibrary.RLerp` (struct) (struct :`Roll` -90.0) `_движение`) false false))
        (:`then_1`
          (`SceneComponent.K2_SetRelativeLocation` (`self.Какашечка`) (`KismetMathLibrary.VLerp` (`self.Попа`) (+ _output_get (`KismetMathLibrary.MakeVector` 0.0 0.0 -100.0)) `_падение`) false false))
        (:`then_2`
          (`self.K2_SetActorLocation` (`KismetMathLibrary.VLerp` (`self.Тело`) (+ _output_get_2 (`KismetMathLibrary.MakeVector` 0.0 30.0 -60.0)) `_движение`)))))))

(fn `UserConstructionScript`
  (`TextRenderComponent.K2_SetText` (`self.TextRender`) (`KismetTextLibrary.Conv_StringToText` (`|GetArrayItem` (`self.Thoughts`) 3))))
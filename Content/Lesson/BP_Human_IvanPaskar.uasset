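; A lesson human Blueprint that labels itself with its name and can report basic personal info.
; The construction script writes Name to a TextRender component, without running the parent's construction script.
; Its PrintInfo override prints Name, Age and the first entry of Thoughts, also skipping the parent version.
; The event graph holds only unused default events.
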(fn `PrintInfo`
  (`KismetSystemLibrary.PrintString` (`self.Name`))
  (`KismetSystemLibrary.PrintString` (`KismetStringLibrary.Conv_IntToString` (`self.Age`)))
  (`KismetSystemLibrary.PrintString` (`|GetArrayItem` (`self.Thoughts`))))

(fn `UserConstructionScript`
  (`TextRenderComponent.K2_SetText` (`self.TextRender`) (`KismetTextLibrary.Conv_StringToText` (`self.Name`))))
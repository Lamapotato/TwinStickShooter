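; Boss enemy bot that hunts the player with twin machine guns and otherwise heads for a BP_flag1 actor.
; A trigger overlap toggles chase mode, swaps a head material and slides the gun housings via a timeline.
; While chasing, Tick faces and follows the player; move success or failure runs a line trace that gates muzzle spin and DoOnce-throttled bullets.
; At zero health it is replaced by BP_dead_boss with an explosion sound.
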(event `self.ReceiveAnyDamage`
  (params (Damage :type "Float (single-precision)") (DamageType :type "DamageType Object Reference") (InstigatedBy :type "Controller Object Reference") (DamageCauser :type "Actor Object Reference"))
  (set `self.health` (- (`self.health`) Damage))
  (if (<= (`self.health`) 0.0)
    (`self.K2_DestroyActor`)
    (`GameplayStatics.PlaySoundAtLocation` "/Game/Lesson/TTS_PAVEL_M/Audio/big-bang.big-bang" (`self.K2_GetActorLocation`) (struct) 1.0 1.0 0.0 null null null null)
    (`|SpawnActorFromClass` "/Game/Lesson/TTS_PAVEL_M/Blueprints/BP_bot/BP_dead_boss.BP_dead_boss_C" (`KismetMathLibrary.MakeTransform` (+ (`self.K2_GetActorLocation`) (0.0 0.0 100.0)) (`self.поворот`)) "AlwaysSpawn" "MultiplyWithRoot" null null)))

(event `self.ReceiveTick`
  (params (DeltaSeconds :type "Float (single-precision)"))
  (bind _returnvalue (`GameplayStatics.GetPlayerPawn` 0))
  (bind _returnvalue_2 (`GameplayStatics.GetPlayerPawn` 0))
  (bind _arrow1 (`self.Arrow1`))
  (bind _arrow2 (`self.Arrow2`))
  (bind _returnvalue_3 (`SceneComponent.K2_GetComponentLocation` _arrow2))
  (bind _returnvalue_4 (`SceneComponent.K2_GetComponentLocation` _arrow1))
  (bind _returnvalue_5 (`KismetMathLibrary.FindLookAtRotation` (`self.K2_GetActorLocation`) (`self.K2_GetActorLocation` _returnvalue)))
  (`/Engine/EditorBlueprintResources/StandardMacros.IsValid` _returnvalue
    (:`Is Valid`
      (set `self.поворот` _returnvalue_5)
      (if (`self.Move_on`)
        (`self.K2_SetActorRotation` _returnvalue_5)
        (`/Engine/EditorBlueprintResources/StandardMacros.IsValid` _returnvalue_2
          (:`Is Valid`
            (`|AIMoveTo` self (0.0 0.0 0.0) _returnvalue_2
              (:`OnSuccess`
                _)
              (:`OnFail`
                _))
            (`KismetSystemLibrary.Delay` 0.001)
            (bind _outhit (`KismetSystemLibrary.LineTraceSingle` :`Start` (`SceneComponent.K2_GetComponentLocation` (`self.Arrow1`)) :`End` (`self.K2_GetActorLocation` (`GameplayStatics.GetPlayerPawn` 0)) :`TraceChannel` "TraceTypeQuery1" :`DrawTime` 0.5))
            (cast `/Game/Lesson/TTS_PAVEL_M/Blueprints/BP_character/BP_MedocCharacter` (`.HitActor` (`GameplayStatics.BreakHitResult` _outhit)))
            (`SceneComponent.K2_AddLocalRotation` (`self.SM_Muzzle_MG`) (struct :`Roll` 13.0) false false)
            (`SceneComponent.K2_AddLocalRotation` (`self.SM_Muzzle_MG1`) (struct :`Roll` 13.0) false false)
            (`|ExecutionSequence`
              (:`then_0`
                (`/Engine/EditorBlueprintResources/StandardMacros.DoOnce` false :!label _label
                  (:`Completed`
                    (`|SpawnActorFromClass` "/Game/Lesson/TTS_PAVEL_M/Blueprints/BP_bot/BP_Boss_bullet.BP_Boss_bullet_C" (`KismetMathLibrary.MakeTransform` _returnvalue_3 (`KismetMathLibrary.FindLookAtRotation` _returnvalue_3 (+ _returnvalue_3 (`SceneComponent.GetForwardVector` _arrow2)))) "Undefined" "MultiplyWithRoot" null null)
                    (`KismetSystemLibrary.Delay` 0.1)
                    (goto _label :!via `Reset`))))
              (:`then_1`
                (`/Engine/EditorBlueprintResources/StandardMacros.DoOnce` false :!label _label_2
                  (:`Completed`
                    (`|SpawnActorFromClass` "/Game/Lesson/TTS_PAVEL_M/Blueprints/BP_bot/BP_Boss_bullet.BP_Boss_bullet_C" (`KismetMathLibrary.MakeTransform` _returnvalue_4 (`KismetMathLibrary.FindLookAtRotation` _returnvalue_4 (+ _returnvalue_4 (`SceneComponent.GetForwardVector` _arrow1)))) "Undefined" "MultiplyWithRoot" null null)
                    (`GameplayStatics.PlaySoundAtLocation` "/Game/Lesson/TTS_PAVEL_M/Audio/MG_sound.MG_sound" _returnvalue_4 (struct) 1.0 1.0 0.0 null null null null)
                    (`KismetSystemLibrary.Delay` 0.1)
                    (goto _label_2 :!via `Reset`)))))))
        (else
          (bind _returnvalue_6 (`GameplayStatics.GetActorOfClass` "/Game/Lesson/TTS_PAVEL_M/Blueprints/BP_actors/BP_flag1.BP_flag1_C"))
          (bind _asaicontroller (cast `AIController` (`self.GetController`)))
          (`AIBlueprintHelperLibrary.SimpleMoveToActor` _asaicontroller _returnvalue_6))))))

(event `self.Trigger_collision.OnComponentBeginOverlap`
  (params (OverlappedComponent :type "PrimitiveComponent Object Reference") (OtherActor :type "Actor Object Reference") (OtherComp :type "PrimitiveComponent Object Reference") (OtherBodyIndex :type Integer) (bFromSweep :type Boolean) (SweepResult :type "HitResult Structure (by ref)"))
  (cast `/Game/Lesson/TTS_PAVEL_M/Blueprints/BP_character/BP_MedocCharacter` OtherActor)
  (set `self.Move_on` true)
  (`PrimitiveComponent.SetMaterial` (`self.SM_Boss_head`) 3 "/Engine/VREditor/LaserPointer/LaserPointerMaterial.LaserPointerMaterial")
  (bind (_direction `_новая_дорожка_0`) (`Timeline|Шкала времени` :!label _label_3)
    (:`Update`
      (`SceneComponent.K2_SetRelativeLocation` (`self.SM_Corpuse_mg1`) (`KismetMathLibrary.VLerp` (-6.0 -40.0 -4.0) (-6.0 -10.0 -4.0) `_новая_дорожка_0`) false false)
      (`SceneComponent.K2_SetRelativeLocation` (`self.SM_Corpuse_mg`) (`KismetMathLibrary.VLerp` (-6.0 40.0 -4.0) (-6.0 10.0 -4.0) `_новая_дорожка_0`) false false))))

(event `self.Trigger_collision.OnComponentEndOverlap`
  (params (OverlappedComponent :type "PrimitiveComponent Object Reference") (OtherActor :type "Actor Object Reference") (OtherComp :type "PrimitiveComponent Object Reference") (OtherBodyIndex :type Integer))
  (cast `/Game/Lesson/TTS_PAVEL_M/Blueprints/BP_character/BP_MedocCharacter` OtherActor)
  (set `self.Move_on` false)
  (`PrimitiveComponent.SetMaterial` (`self.SM_Boss_head`) 3 "/Engine/VREditor/LaserPointer/LaserPointerMaterial_Inst.LaserPointerMaterial_Inst")
  (goto _label_3 :!via `Reverse`))

(fn `UserConstructionScript`)
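; BP_boom_bot is a kamikaze enemy bot that chases the player and explodes on contact or at zero health.
; Sphere1 overlap by BP_MedocCharacter enables Tick-driven facing and repeated AIMoveTo; a timeline animates its flame mesh.
; Sphere overlap or death triggers a one-time timeline that spins and grows a blast mesh.
; Each blast update damages BP_MedocCharacter regardless of distance, until a short delay destroys the bot and plays Bigbang.
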(event `self.ReceiveBeginPlay`
  (bind _sm_flame_gunflamer (`self.SM_Flame_gunflamer`))
  (bind (_direction `_новая_дорожка_0`) (`Timeline|Шкала времени`)
    (:`Update`
      (`SceneComponent.K2_AddLocalRotation` _sm_flame_gunflamer (struct :`Roll` 70.0) false false)
      (`SceneComponent.SetWorldScale3D` _sm_flame_gunflamer (`KismetMathLibrary.VLerp` (0.375 1.03125 0.78125) (0.7 1.0 0.7) `_новая_дорожка_0`)))))

(event `self.ReceiveAnyDamage`
  (params (Damage :type "Float (single-precision)") (DamageType :type "DamageType Object Reference") (InstigatedBy :type "Controller Object Reference") (DamageCauser :type "Actor Object Reference"))
  (bind _sm_boom_sphere (`self.SM_Boom_sphere`))
  (set `self.health` (- (`self.health`) Damage))
  (if (<= (`self.health`) 0.0)
    (`/Engine/EditorBlueprintResources/StandardMacros.DoOnce` false :!label _label
      (:`Completed`
        (bind (_direction `_новая_дорожка_0`) (`Timeline|Шкала времени_0`)
          (:`Update`
            (`SceneComponent.K2_AddLocalRotation` _sm_boom_sphere (struct :`Yaw` 70.0) false false)
            (`SceneComponent.SetWorldScale3D` _sm_boom_sphere (`KismetMathLibrary.VLerp` (0.1 0.1 0.1) (4.0 4.0 4.0) `_новая_дорожка_0`))
            (bind _returnvalue (`GameplayStatics.GetActorOfClass` "/Game/Lesson/TTS_PAVEL_M/Blueprints/BP_character/BP_MedocCharacter.BP_MedocCharacter_C"))
            (`GameplayStatics.ApplyDamage` _returnvalue 1.0)
            (`KismetSystemLibrary.Delay` 0.25)
            (`self.K2_DestroyActor`)
            (`GameplayStatics.PlaySoundAtLocation` "/Game/Lesson/TTS_PAVEL_M/Audio/big-bang.big-bang" (`self.K2_GetActorLocation`) (struct) 1.0 1.0 0.0 null null null null)))))))

(event `self.Sphere.OnComponentBeginOverlap`
  (params (OverlappedComponent :type "PrimitiveComponent Object Reference") (OtherActor :type "Actor Object Reference") (OtherComp :type "PrimitiveComponent Object Reference") (OtherBodyIndex :type Integer) (bFromSweep :type Boolean) (SweepResult :type "HitResult Structure (by ref)"))
  (cast `/Game/Lesson/TTS_PAVEL_M/Blueprints/BP_character/BP_MedocCharacter` OtherActor)
  (goto _label))

(event `self.Sphere1.OnComponentBeginOverlap`
  (params (OverlappedComponent :type "PrimitiveComponent Object Reference") (OtherActor :type "Actor Object Reference") (OtherComp :type "PrimitiveComponent Object Reference") (OtherBodyIndex :type Integer) (bFromSweep :type Boolean) (SweepResult :type "HitResult Structure (by ref)"))
  (cast `/Game/Lesson/TTS_PAVEL_M/Blueprints/BP_character/BP_MedocCharacter` OtherActor)
  (set `self.Move_on` true))

(event `self.ReceiveTick`
  (params (DeltaSeconds :type "Float (single-precision)"))
  (bind _returnvalue (`GameplayStatics.GetPlayerPawn` 0))
  (bind _returnvalue_2 (`GameplayStatics.GetPlayerPawn` 0))
  (`/Engine/EditorBlueprintResources/StandardMacros.IsValid` _returnvalue
    (:`Is Valid`
      (if (`self.Move_on`)
        (`self.K2_SetActorRotation` (`KismetMathLibrary.FindLookAtRotation` (`self.K2_GetActorLocation`) (`self.K2_GetActorLocation` _returnvalue)))
        (`/Engine/EditorBlueprintResources/StandardMacros.IsValid` _returnvalue_2 :!label _label_2
          (:`Is Valid`
            (`|AIMoveTo` self (0.0 0.0 0.0) _returnvalue_2
              (:`OnSuccess`
                _)
              (:`OnFail`
                _))
            (`KismetSystemLibrary.Delay` 0.001)
            (goto _label_2)))))))

(fn `UserConstructionScript`)
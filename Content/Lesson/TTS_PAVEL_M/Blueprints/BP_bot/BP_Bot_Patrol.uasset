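; Patrol bot enemy that walks between a flag and a lever actor, switching on a timed delay, and attacks the player inside its trigger.
; Trigger overlaps set InputVector, which switches Tick from patrolling to facing and chasing the player via AI SimpleMove.
; While chasing, a line trace hitting BP_MedocCharacter fires bullets with sound, rate-limited by DoOnce and Delay.
; Damage reduces Health; death destroys it and spawns separate head and body wreck actors with an explosion sound.
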(event `self.ReceiveAnyDamage`
  (params (Damage :type "Float (single-precision)") (DamageType :type "DamageType Object Reference") (InstigatedBy :type "Controller Object Reference") (DamageCauser :type "Actor Object Reference"))
  (bind _returnvalue (`self.K2_GetActorLocation`))
  (set `self.Health` (- (`self.Health`) Damage))
  (if (<= (`self.Health`) 0.0)
    (`self.K2_DestroyActor`)
    (`GameplayStatics.PlaySoundAtLocation` "/Game/Lesson/TTS_PAVEL_M/Audio/big-bang.big-bang" (`self.K2_GetActorLocation`) (struct) 1.0 1.0 0.0 null null null null)
    (`|SpawnActorFromClass` "/Game/Lesson/TTS_PAVEL_M/Blueprints/BP_bot/BP_dead_bot_head.BP_dead_bot_head_C" (`KismetMathLibrary.MakeTransform` (+ _returnvalue (0.0 0.0 100.0)) (`self.поворот`)) "AlwaysSpawn" "MultiplyWithRoot" null null)
    (`|SpawnActorFromClass` "/Game/Lesson/TTS_PAVEL_M/Blueprints/BP_bot/BP_dead_bot_corpuse.BP_dead_bot_corpuse_C" (`KismetMathLibrary.MakeTransform` (+ _returnvalue (0.0 0.0 20.0)) (`self.поворот`)) "AlwaysSpawn" "MultiplyWithRoot" null null)))

(event `self.ReceiveTick`
  (params (DeltaSeconds :type "Float (single-precision)"))
  (bind _returnvalue (`GameplayStatics.GetPlayerPawn` 0))
  (bind _arrow1 (`self.Arrow1`))
  (bind _returnvalue_2 (`SceneComponent.K2_GetComponentLocation` _arrow1))
  (`/Engine/EditorBlueprintResources/StandardMacros.IsValid` _returnvalue
    (:`Is Valid`
      (if (`self.bInputVector`)
        (bind _output_get (set `self.поворот` (`KismetMathLibrary.MakeRotator` 0.0 0.0 (.yaw (`KismetMathLibrary.FindLookAtRotation` (`self.K2_GetActorLocation`) (`self.K2_GetActorLocation` _returnvalue))))))
        (`self.K2_SetActorRotation` _output_get)
        (bind _asaicontroller (cast `AIController` (`self.GetController`)))
        (`AIBlueprintHelperLibrary.SimpleMoveToActor` _asaicontroller (`GameplayStatics.GetPlayerPawn` 0))
        (bind _outhit (`KismetSystemLibrary.LineTraceSingle` :`Start` (`SceneComponent.K2_GetComponentLocation` (`self.Arrow1`)) :`End` (`self.K2_GetActorLocation` (`GameplayStatics.GetPlayerPawn` 0)) :`TraceChannel` "TraceTypeQuery1" :`DrawTime` 0.5))
        (cast `/Game/Lesson/TTS_PAVEL_M/Blueprints/BP_character/BP_MedocCharacter` (`.HitActor` (`GameplayStatics.BreakHitResult` _outhit)))
        (`/Engine/EditorBlueprintResources/StandardMacros.DoOnce` false :!label _label
          (:`Completed`
            (`|SpawnActorFromClass` "/Game/Lesson/TTS_PAVEL_M/Blueprints/BP_character/BP_bullet.BP_bullet_C" (`KismetMathLibrary.MakeTransform` _returnvalue_2 (`KismetMathLibrary.FindLookAtRotation` _returnvalue_2 (+ _returnvalue_2 (`SceneComponent.GetForwardVector` _arrow1)))) "Undefined" "MultiplyWithRoot" null null)
            (`GameplayStatics.PlaySoundAtLocation` "/Game/Lesson/TTS_PAVEL_M/Audio/Пушка.Пушка" _returnvalue_2 (struct) 1.0 1.0 0.0 null null null null)
            (`KismetSystemLibrary.Delay` 0.7)
            (goto _label :!via `Reset`)))
        (else
          ; ПАТРУЛЬ
          (if (`self.Patrol`)
            (bind _returnvalue_3 (`GameplayStatics.GetActorOfClass` "/Game/Lesson/TTS_PAVEL_M/Blueprints/BP_actors/BP_flag.BP_flag_C"))
            (bind _asaicontroller_2 (cast `AIController` (`self.GetController`)))
            (`AIBlueprintHelperLibrary.SimpleMoveToActor` _asaicontroller_2 _returnvalue_3)
            (`KismetSystemLibrary.Delay` 5.0)
            (set `self.Patrol` false)
            (else
              (bind _returnvalue_4 (`GameplayStatics.GetActorOfClass` "/Game/Lesson/TTS_PAVEL_M/Blueprints/BP_actors/Buttons_and_gates/BP_рычаг.BP_рычаг_C"))
              (bind _asaicontroller_3 (cast `AIController` (`self.GetController`)))
              (`AIBlueprintHelperLibrary.SimpleMoveToActor` _asaicontroller_3 _returnvalue_4)
              (`KismetSystemLibrary.Delay` 5.0)
              (set `self.Patrol` true))))))))

(event `self.Trigger_collision.OnComponentBeginOverlap`
  (params (OverlappedComponent :type "PrimitiveComponent Object Reference") (OtherActor :type "Actor Object Reference") (OtherComp :type "PrimitiveComponent Object Reference") (OtherBodyIndex :type Integer) (bFromSweep :type Boolean) (SweepResult :type "HitResult Structure (by ref)"))
  (cast `/Game/Lesson/TTS_PAVEL_M/Blueprints/BP_character/BP_MedocCharacter` OtherActor)
  (set `self.bInputVector` true))

(event `self.Trigger_collision.OnComponentEndOverlap`
  (params (OverlappedComponent :type "PrimitiveComponent Object Reference") (OtherActor :type "Actor Object Reference") (OtherComp :type "PrimitiveComponent Object Reference") (OtherBodyIndex :type Integer))
  (cast `/Game/Lesson/TTS_PAVEL_M/Blueprints/BP_character/BP_MedocCharacter` OtherActor)
  (set `self.bInputVector` false))

(fn `UserConstructionScript`)
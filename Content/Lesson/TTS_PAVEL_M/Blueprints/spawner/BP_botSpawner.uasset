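; Bot spawner actor that spawns a queued list of bot classes, then retracts and destroys itself.
; StartSpawn, optionally triggered on BeginPlay, adds rotating movement, starts a looping two-second timer and uses a timeline to lower the mesh from above.
; SpawnBot spawns the first queued class at the actor's location and removes it from the array.
; Once the queue is empty, a second timeline raises the mesh and a delay precedes destruction.
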(event `self.ReceiveTick`
  (params (DeltaSeconds :type "Float (single-precision)")))

(event `self.ReceiveBeginPlay`
  (if (`self.Enable on start`)
    (`self.Start spawn`)))

(event `Start spawn`
  (`AddComponent|NODE_AddRotatingMovementComponent-0`)
  (`KismetSystemLibrary.K2_SetTimerDelegate` (`|CreateDelegate` :!event `SpawnBot`) 2.0 true)
  (bind (_direction `_новая_дорожка_0`) (`Timeline|Шкала времени`)
    (:`Update`
      (`SceneComponent.K2_SetRelativeLocation` (`self.SM_MERGED_StaticMeshActor_38`) (`KismetMathLibrary.VLerp` (0.0 0.0 800.0) (0.0 0.0 0.0) `_новая_дорожка_0`) false false))))

(event `SpawnBot`
  (bind _botstospawn (`self.BotsToSpawn`))
  (if (`KismetArrayLibrary.Array_IsValidIndex` _botstospawn)
    (`|SpawnActorFromClass` (`|GetArrayItem` _botstospawn) (`KismetMathLibrary.MakeTransform` (`self.K2_GetActorLocation`)) "Undefined" "MultiplyWithRoot" null null)
    (`KismetArrayLibrary.Array_Remove` (`self.BotsToSpawn`))
    (else
      (bind (_direction `_новая_дорожка_0`) (`Timeline|Шкала времени_0`)
        (:`Update`
          (`SceneComponent.K2_SetRelativeLocation` (`self.SM_MERGED_StaticMeshActor_38`) (`KismetMathLibrary.VLerp` (0.0 0.0 0.0) (0.0 0.0 800.0) `_новая_дорожка_0`) false false)
          (`KismetSystemLibrary.Delay` 2.0)
          (`self.K2_DestroyActor`))))))

(fn `UserConstructionScript`)
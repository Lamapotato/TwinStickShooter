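; Laser weapon Blueprint that fires a short-range hitscan shot when its Linetrace_shoot event is called.
; Each shot plays a laser sound and line-traces forward from an Arrow component on the Visibility channel, applying fixed damage to the hit actor.
; A temporary static mesh component flashes as the shot visual, and a DoOnce gate resets after its brief delay, limiting fire rate.
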(event `Linetrace_shoot`
  (bind _arrow (`self.Arrow`))
  (bind _returnvalue (`SceneComponent.K2_GetComponentLocation` _arrow))
  (`/Engine/EditorBlueprintResources/StandardMacros.DoOnce` false :!label _label
    (:`Completed`
      (`GameplayStatics.PlaySoundAtLocation` "/Game/Lesson/TTS_PAVEL_M/Audio/лазер.лазер" _returnvalue (struct) 0.3 1.0 0.0 null null null null)
      (bind _outhit (`KismetSystemLibrary.LineTraceSingle` :`Start` _returnvalue :`End` (+ _returnvalue (* (`SceneComponent.GetForwardVector` _arrow) 800.0)) :`TraceChannel` "TraceTypeQuery1" :`DrawTime` 0.5))
      (`|ExecutionSequence`
        (:`then_0`
          (bind _returnvalue_2 (`AddComponent|NODE_AddStaticMeshComponent-2` :`RelativeTransform` (`SceneComponent.GetRelativeTransform` _arrow)))
          (`KismetSystemLibrary.Delay` 0.2)
          (`ActorComponent.K2_DestroyComponent` _returnvalue_2)
          (goto _label :!via `Reset`))
        (:`then_1`
          (`GameplayStatics.ApplyDamage` (`.HitActor` (`GameplayStatics.BreakHitResult` _outhit)) 5.0))))))

(fn `UserConstructionScript`)
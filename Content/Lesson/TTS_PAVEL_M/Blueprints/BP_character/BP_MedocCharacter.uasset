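; BP_MedocCharacter is the player character, moved by Enhanced Input, turned toward the mouse cursor, with health shown on its back.
; Front, left and right weapons and a laser sight toggle by spawning or destroying attached actors; timelines slide weapon mounts, and one input fires all weapons.
; Overlap queries call interfaces on the nearest interactable or triggerable actor.
; It also handles damage, limited repair charges, lift lowering and deleting all bots.
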(event `self.ReceiveTick`
  (params (DeltaSeconds :type "Float (single-precision)"))
  ; Поворот персонажа по "YAW" курсором
  (`self.Character_Mouse_Rotation`)
  ; Вывод здоровья на спине
  (`TextRenderComponent.K2_SetText` (`self.TextRender`) (`KismetTextLibrary.Conv_DoubleToText` (`self.Health`) "HalfToEven"))
  ;[0 0.3229 0.205 0.1913] Замена цвета актора при приоритетном растоянии
  (`self.Trigged_object`))

(event `self.ReceiveBeginPlay`
  (bind _returnvalue (pcsubsystem `EnhancedInputLocalPlayerSubsystem` (`GameplayStatics.GetPlayerController` 0)))
  ; IMC_MedocMovement
  (`EnhancedInputSubsystemInterface.ClearAllMappings` _returnvalue)
  (`EnhancedInputSubsystemInterface.AddMappingContext` _returnvalue "/Game/Lesson/TTS_PAVEL_M/Blueprints/BP_character/IMC_MedocMovement.IMC_MedocMovement" 0 (struct))
  ; Задаем куросор
  (set `PlayerController.bShowMouseCursor` true (`GameplayStatics.GetPlayerController` 0)))

(event `EnhancedInput|/Game/Lesson/TTS_PAVEL_M/Blueprints/BP_character/IA_MedocMove`
  (params (ActionValue :type "Vector2D Structure") (ElapsedSeconds :type "Float (double-precision)") (TriggeredSeconds :type "Float (double-precision)") (InputAction :type "InputAction Object Reference" :default "/Game/Lesson/TTS_PAVEL_M/Blueprints/BP_character/IA_MedocMove.IA_MedocMove"))
  (bind (_x _y) (`KismetMathLibrary.BreakVector2D` ActionValue))
  ; Движение "WASD"
  (:`Triggered`
    (`PawnMovementComponent.AddInputVector` (`self.CharacterMovement`) (`KismetMathLibrary.MakeVector` _x _y) false)))

(event `self.ReceiveAnyDamage`
  (params (Damage :type "Float (single-precision)") (DamageType :type "DamageType Object Reference") (InstigatedBy :type "Controller Object Reference") (DamageCauser :type "Actor Object Reference"))
  ; Урое по здоровью
  (set `self.Health` (- (`self.Health`) Damage)))

(event `EnhancedInput|/Game/Lesson/TTS_PAVEL_M/Blueprints/BP_character/IA_MedocJump`
  (params (ActionValue :type Boolean) (ElapsedSeconds :type "Float (double-precision)") (TriggeredSeconds :type "Float (double-precision)") (InputAction :type "InputAction Object Reference" :default "/Game/Lesson/TTS_PAVEL_M/Blueprints/BP_character/IA_MedocJump.IA_MedocJump"))
  ; Прыжок "Пробел"
  (:`Triggered`
    (`self.Jump`)))

(event `EnhancedInput|/Game/Lesson/TTS_PAVEL_M/Blueprints/BP_character/IA_Repair`
  (params (ActionValue :type Boolean) (ElapsedSeconds :type "Float (double-precision)") (TriggeredSeconds :type "Float (double-precision)") (InputAction :type "InputAction Object Reference" :default "/Game/Lesson/TTS_PAVEL_M/Blueprints/BP_character/IA_Repair.IA_Repair"))
  (bind (_returnvalue_x _returnvalue_y _returnvalue_z) (`KismetMathLibrary.BreakVector` (`SceneComponent.K2_GetComponentLocation` (`self.Repair_root`))))
  ; Ремонт на "Q"
  (:`Triggered`
    (if (<= (`self.Health`) 75.0)
      (`/Engine/EditorBlueprintResources/StandardMacros.DoOnce` false :!label _label
        (:`Completed`
          (if (>= (`self.repair`) 1)
            (set `self.Health` (+ (`self.Health`) 25.0))
            (set `self.repair` (- (`self.repair`) 1))
            (bind _returnvalue (`|SpawnActorFromClass` "/Game/Lesson/TTS_PAVEL_M/Blueprints/BP_character/BP_Repair.BP_Repair_C" (`KismetMathLibrary.MakeTransform` (`KismetMathLibrary.MakeVector` _returnvalue_x (+ _returnvalue_y 25.0) _returnvalue_z)) "AlwaysSpawn" "MultiplyWithRoot" null null))
            (bind _output_get (set `self.Repair_tool` _returnvalue))
            (`self.K2_AttachToComponent` _output_get (`self.Repair_root`) "None" "KeepWorld" "SnapToTarget" "KeepWorld" true)
            (`GameplayStatics.PlaySoundAtLocation` "/Game/Lesson/TTS_PAVEL_M/Audio/ремонт.ремонт" (`self.K2_GetActorLocation`) (struct) 1.0 1.0 0.0 null null null null)
            (`KismetSystemLibrary.Delay` 1.5)
            (`self.K2_DestroyActor` (`self.Repair_tool`))
            (goto _label :!via `Reset`)))))))

(event `EnhancedInput|/Game/Lesson/TTS_PAVEL_M/Blueprints/BP_character/IA_Select_Weapon_HeavyG`
  (params (ActionValue :type Boolean) (ElapsedSeconds :type "Float (double-precision)") (TriggeredSeconds :type "Float (double-precision)") (InputAction :type "InputAction Object Reference" :default "/Game/Lesson/TTS_PAVEL_M/Blueprints/BP_character/IA_Select_Weapon_HeavyG.IA_Select_Weapon_HeavyG"))
  (bind _heavy_root (`self.Heavy_root`))
  ; Добавляем и убираем фронтальное оружие на "1"
  (:`Triggered`
    (if (`self.bWeaponEquippedFRONT`)
      (`KismetSystemLibrary.RetriggerableDelay` 0.5)
      (`GameplayStatics.PlaySoundAtLocation` "/Game/Lesson/TTS_PAVEL_M/Audio/Лопость.Лопость" (`self.K2_GetActorLocation`) (struct) 1.0 1.0 0.0 null null null null)
      (bind _returnvalue (`|SpawnActorFromClass` "/Game/Lesson/TTS_PAVEL_M/Blueprints/BP_character/BP_Weapon_HeavyG.BP_Weapon_HeavyG_C" (`KismetMathLibrary.MakeTransform` (`SceneComponent.K2_GetComponentLocation` _heavy_root) (`SceneComponent.K2_GetComponentRotation` _heavy_root)) "AlwaysSpawn" "MultiplyWithRoot" null null))
      (bind _output_get (set `self.Front_weapon` _returnvalue))
      (`self.K2_AttachToComponent` _output_get (`self.Heavy_root`) "None" "KeepWorld" "KeepWorld" "KeepWorld" true)
      (bind _output_get_2 (set `self.CorpuseFront` (`SceneComponent.RelativeLocation` (`self.Heavy_root`))))
      (bind (_direction `_выдвижение`) (`Timeline|Шкала времени_3` :!via `PlayFromStart`)
        (:`Update`
          (`SceneComponent.K2_SetRelativeRotation` (`self.SM_Panel_front`) (`KismetMathLibrary.RLerp` (struct) (struct :`Pitch` -140.0) `_выдвижение`) false false)
          (`SceneComponent.K2_SetRelativeLocation` (`self.Heavy_root`) (`KismetMathLibrary.VLerp` (`self.CorpuseFront`) (+ _output_get_2 (`KismetMathLibrary.MakeVector` 20.0)) `_выдвижение`) false false)
          (set `self.bWeaponEquippedFRONT` false)))
      (else
        (`KismetSystemLibrary.RetriggerableDelay` 0.5)
        (`GameplayStatics.PlaySoundAtLocation` "/Game/Lesson/TTS_PAVEL_M/Audio/Лопость.Лопость" (`self.K2_GetActorLocation`) (struct) 1.0 1.0 0.0 null null null null)
        (bind _output_get_3 (set `self.CorpuseFront` (`SceneComponent.RelativeLocation` (`self.Heavy_root`))))
        (bind (_direction_2 `_выдвижение_2`) (`Timeline|Шкала времени_4` :!via `PlayFromStart`)
          (:`Update`
            (`SceneComponent.K2_SetRelativeRotation` (`self.SM_Panel_front`) (`KismetMathLibrary.RLerp` (struct :`Pitch` -140.0) (struct) `_выдвижение_2`) false false)
            (`SceneComponent.K2_SetRelativeLocation` (`self.Heavy_root`) (`KismetMathLibrary.VLerp` (`self.CorpuseFront`) (+ _output_get_3 (`KismetMathLibrary.MakeVector` -20.0)) `_выдвижение_2`) false false)
            (set `self.bWeaponEquippedFRONT` true)
            (`KismetSystemLibrary.Delay` 0.5)
            (`self.K2_DestroyActor` (`self.Front_weapon`))))))))

(event `Down_lift`
  ;[0 0.3229 0.205 0.1913] Тригер на лифт
  (bind _returnvalue (`GameplayStatics.GetActorOfClass` "/Game/Lesson/TTS_PAVEL_M/Blueprints/BP_actors/Buttons_and_gates/BP_lift.BP_lift_C"))
  (`/Game/Lesson/TTS_PAVEL_M/Blueprints/BP_actors/Buttons_and_gates/BP_lift.lift_down` _returnvalue))

(event `EnhancedInput|/Game/Lesson/TTS_PAVEL_M/Blueprints/BP_character/IA_Select_Weapon_Laser`
  (params (ActionValue :type Boolean) (ElapsedSeconds :type "Float (double-precision)") (TriggeredSeconds :type "Float (double-precision)") (InputAction :type "InputAction Object Reference" :default "/Game/Lesson/TTS_PAVEL_M/Blueprints/BP_character/IA_Select_Weapon_Laser.IA_Select_Weapon_Laser"))
  (bind _left_root (`self.Left_root`))
  ; Добавляем и убираем левое оружие на "2"
  (:`Triggered`
    (if (`self.bWeaponEquippedLEFT`)
      (`KismetSystemLibrary.RetriggerableDelay` 0.5)
      (`GameplayStatics.PlaySoundAtLocation` "/Game/Lesson/TTS_PAVEL_M/Audio/Лопость.Лопость" (`self.K2_GetActorLocation`) (struct) 1.0 1.0 0.0 null null null null)
      (bind _returnvalue (`|SpawnActorFromClass` "/Game/Lesson/TTS_PAVEL_M/Blueprints/BP_character/BP_Weapon_Laser.BP_Weapon_Laser_C" (`KismetMathLibrary.MakeTransform` (`SceneComponent.K2_GetComponentLocation` _left_root) (`SceneComponent.K2_GetComponentRotation` _left_root)) "AlwaysSpawn" "MultiplyWithRoot" null null))
      (bind _output_get (set `self.Left_weapon` _returnvalue))
      (`self.K2_AttachToComponent` _output_get (`self.Left_root`) "None" "KeepWorld" "KeepWorld" "KeepWorld" true)
      (bind _output_get_2 (set `self.CorpuseLeft` (`SceneComponent.RelativeLocation` (`self.Left_root`))))
      (bind (_direction `_выдвижение`) (`Timeline|Шкала времени` :!via `PlayFromStart`)
        (:`Update`
          (`SceneComponent.K2_SetRelativeLocation` (`self.Left_root`) (`KismetMathLibrary.VLerp` (`self.CorpuseLeft`) (+ _output_get_2 (`KismetMathLibrary.MakeVector` 0.0 -28.0)) `_выдвижение`) false false)
          (set `self.bWeaponEquippedLEFT` false)))
      (else
        (`KismetSystemLibrary.RetriggerableDelay` 0.5)
        (`GameplayStatics.PlaySoundAtLocation` "/Game/Lesson/TTS_PAVEL_M/Audio/Лопость.Лопость" (`self.K2_GetActorLocation`) (struct) 1.0 1.0 0.0 null null null null)
        (bind _output_get_3 (set `self.CorpuseLeft` (`SceneComponent.RelativeLocation` (`self.Left_root`))))
        (bind (_direction_2 `_выдвижение_2`) (`Timeline|Шкала времени_0` :!via `PlayFromStart`)
          (:`Update`
            (`SceneComponent.K2_SetRelativeLocation` (`self.Left_root`) (`KismetMathLibrary.VLerp` (`self.CorpuseLeft`) (+ _output_get_3 (`KismetMathLibrary.MakeVector` 0.0 28.0)) `_выдвижение_2`) false false)
            (set `self.bWeaponEquippedLEFT` true)
            (`KismetSystemLibrary.Delay` 0.5)
            (`self.K2_DestroyActor` (`self.Left_weapon`))))))))

(event `EnhancedInput|/Game/Lesson/TTS_PAVEL_M/Blueprints/BP_character/IA_Select_Weapon_FlameT`
  (params (ActionValue :type Boolean) (ElapsedSeconds :type "Float (double-precision)") (TriggeredSeconds :type "Float (double-precision)") (InputAction :type "InputAction Object Reference" :default "/Game/Lesson/TTS_PAVEL_M/Blueprints/BP_character/IA_Select_Weapon_FlameT.IA_Select_Weapon_FlameT"))
  (bind _rigrt_root (`self.Rigrt_root`))
  ; Добавляем и убираем Правое оружие на "3"
  (:`Triggered`
    (if (`self.bWeaponEquippedRIGTH`)
      (`KismetSystemLibrary.RetriggerableDelay` 0.5)
      (`GameplayStatics.PlaySoundAtLocation` "/Game/Lesson/TTS_PAVEL_M/Audio/Лопость.Лопость" (`self.K2_GetActorLocation`) (struct) 1.0 1.0 0.0 null null null null)
      (bind _returnvalue (`|SpawnActorFromClass` "/Game/Lesson/TTS_PAVEL_M/Blueprints/BP_character/BP_Weapon_FlameT.BP_Weapon_FlameT_C" (`KismetMathLibrary.MakeTransform` (`SceneComponent.K2_GetComponentLocation` _rigrt_root) (`SceneComponent.K2_GetComponentRotation` _rigrt_root)) "AlwaysSpawn" "MultiplyWithRoot" null null))
      (bind _output_get (set `self.Rigth_weapon` _returnvalue))
      (`self.K2_AttachToComponent` _output_get (`self.Rigrt_root`) "None" "KeepWorld" "KeepWorld" "KeepWorld" true)
      (bind _output_get_2 (set `self.CorpusRigth` (`SceneComponent.RelativeLocation` (`self.Rigrt_root`))))
      (bind (_direction `_выдвижение`) (`Timeline|Шкала времени_1` :!via `PlayFromStart`)
        (:`Update`
          (`SceneComponent.K2_SetRelativeLocation` (`self.Rigrt_root`) (`KismetMathLibrary.VLerp` (`self.CorpusRigth`) (+ _output_get_2 (`KismetMathLibrary.MakeVector` 0.0 28.0)) `_выдвижение`) false false)
          (set `self.bWeaponEquippedRIGTH` false)))
      (else
        (`KismetSystemLibrary.RetriggerableDelay` 0.5)
        (`GameplayStatics.PlaySoundAtLocation` "/Game/Lesson/TTS_PAVEL_M/Audio/Лопость.Лопость" (`self.K2_GetActorLocation`) (struct) 1.0 1.0 0.0 null null null null)
        (bind _output_get_3 (set `self.CorpusRigth` (`SceneComponent.RelativeLocation` (`self.Rigrt_root`))))
        (bind (_direction_2 `_выдвижение_2`) (`Timeline|Шкала времени_2` :!via `PlayFromStart`)
          (:`Update`
            (`SceneComponent.K2_SetRelativeLocation` (`self.Rigrt_root`) (`KismetMathLibrary.VLerp` (`self.CorpusRigth`) (+ _output_get_3 (`KismetMathLibrary.MakeVector` 0.0 -28.0)) `_выдвижение_2`) false false)
            (set `self.bWeaponEquippedRIGTH` true)
            (`KismetSystemLibrary.Delay` 0.5)
            (`self.K2_DestroyActor` (`self.Rigth_weapon`))))))))

(event `EnhancedInput|/Game/Lesson/TTS_PAVEL_M/Blueprints/BP_character/IA_Select_Linetrace`
  (params (ActionValue :type Boolean) (ElapsedSeconds :type "Float (double-precision)") (TriggeredSeconds :type "Float (double-precision)") (InputAction :type "InputAction Object Reference" :default "/Game/Lesson/TTS_PAVEL_M/Blueprints/BP_character/IA_Select_Linetrace.IA_Select_Linetrace"))
  (bind _liser_root (`self.Liser_root`))
  ; Добавляем и убираем лазерную подсветку "L"
  (:`Triggered`
    (if (`self.bLaserEquip`)
      (bind _returnvalue (`|SpawnActorFromClass` "/Game/Lesson/TTS_PAVEL_M/Blueprints/BP_character/BP_lineLaser.BP_lineLaser_C" (`KismetMathLibrary.MakeTransform` (`SceneComponent.K2_GetComponentLocation` _liser_root) (`SceneComponent.K2_GetComponentRotation` _liser_root)) "AlwaysSpawn" "MultiplyWithRoot" null null))
      (bind _output_get (set `self.LineLaser` _returnvalue))
      (`self.K2_AttachToComponent` _output_get (`self.Liser_root`) "None" "KeepWorld" "KeepWorld" "KeepWorld" true)
      (set `self.bLaserEquip` false)
      (else
        (`self.K2_DestroyActor` (`self.LineLaser`))
        (set `self.bLaserEquip` true)))))

(event `EnhancedInput|/Game/Lesson/TTS_PAVEL_M/Blueprints/BP_character/IA_MedocShooting`
  (params (ActionValue :type Boolean) (ElapsedSeconds :type "Float (double-precision)") (TriggeredSeconds :type "Float (double-precision)") (InputAction :type "InputAction Object Reference" :default "/Game/Lesson/TTS_PAVEL_M/Blueprints/BP_character/IA_MedocShooting.IA_MedocShooting"))
  (bind _rigth_weapon (`self.Rigth_weapon`))
  ; Стрелба "ЛКМ"
  (:`Triggered`
    (`|ExecutionSequence`
      (:`then_0`
        ;; Стрельба фронтального
        (`/Engine/EditorBlueprintResources/StandardMacros.IsValid` (`self.Front_weapon`)
          (:`Is Valid`
            (`/Game/Lesson/TTS_PAVEL_M/Blueprints/BP_character/BP_Weapon_HeavyG.Object_shooting` (`self.Front_weapon`)))))
      (:`then_1`
        ;; Стрельба левого
        (`/Engine/EditorBlueprintResources/StandardMacros.IsValid` (`self.Left_weapon`)
          (:`Is Valid`
            (`/Game/Lesson/TTS_PAVEL_M/Blueprints/BP_character/BP_Weapon_Laser.Linetrace_shoot` (`self.Left_weapon`)))))
      (:`then_2`
        ;; Стрельба левого
        (`/Engine/EditorBlueprintResources/StandardMacros.IsValid` _rigth_weapon
          (:`Is Valid`
            (`/Game/Lesson/TTS_PAVEL_M/Blueprints/BP_character/BP_Weapon_FlameT.flame_shoot` _rigth_weapon)))))))

(event `EnhancedInput|/Game/Lesson/TTS_PAVEL_M/Blueprints/BP_character/IA_Kill_all`
  (params (ActionValue :type Boolean) (ElapsedSeconds :type "Float (double-precision)") (TriggeredSeconds :type "Float (double-precision)") (InputAction :type "InputAction Object Reference" :default "/Game/Lesson/TTS_PAVEL_M/Blueprints/BP_character/IA_Kill_all.IA_Kill_all"))
  ; Удалить ботов "Delete"
  (:`Triggered`
    (bind _outactors (`GameplayStatics.GetAllActorsOfClass` "/Game/Lesson/TTS_PAVEL_M/Blueprints/BP_bot/BP_bot.BP_bot_C"))
    (for _array_element _outactors
      (`/Game/Lesson/TTS_PAVEL_M/Blueprints/BP_bot/BP_bot.DELETEBOT` _array_element))))

(event `self.interact_colision.OnComponentBeginOverlap`
  (params (OverlappedComponent :type "PrimitiveComponent Object Reference") (OtherActor :type "Actor Object Reference") (OtherComp :type "PrimitiveComponent Object Reference") (OtherBodyIndex :type Integer) (bFromSweep :type Boolean) (SweepResult :type "HitResult Structure (by ref)"))
  ;[0 0.3229 0.205 0.1913] Интерактив
  (cast `/Game/Lesson/TTS_PAVEL_M/Blueprints/BP_character/BPI_Medoc_Interface_interact` OtherActor)
  (`/Engine/EditorBlueprintResources/StandardMacros.IncrementInt` (`self.Interact_count`)
    (:`  `
      (`|ExecutionSequence`
        (:`then_1`
          (`SceneComponent.SetHiddenInGame` (`self.Interact  [E]`) (not (> (`self.Interact_count`) 0)) false :!label _label_2))))))

(event `self.interact_colision.OnComponentEndOverlap`
  (params (OverlappedComponent :type "PrimitiveComponent Object Reference") (OtherActor :type "Actor Object Reference") (OtherComp :type "PrimitiveComponent Object Reference") (OtherBodyIndex :type Integer))
  ;[0 0.3229 0.205 0.1913] Интерактив
  (cast `/Game/Lesson/TTS_PAVEL_M/Blueprints/BP_character/BPI_Medoc_Interface_interact` OtherActor)
  (`/Engine/EditorBlueprintResources/StandardMacros.DecrementInt` (`self.Interact_count`)
    (:`  `
      (`|ExecutionSequence`
        (:`then_0`
          (goto _label_2))))))

(event `EnhancedInput|/Game/Lesson/TTS_PAVEL_M/Blueprints/BP_character/IA_Medoc_Interact`
  (params (ActionValue :type Boolean) (ElapsedSeconds :type "Float (double-precision)") (TriggeredSeconds :type "Float (double-precision)") (InputAction :type "InputAction Object Reference" :default "/Game/Lesson/TTS_PAVEL_M/Blueprints/BP_character/IA_Medoc_Interact.IA_Medoc_Interact"))
  ;[0 0.3229 0.205 0.1913] Интерактив
  (:`Triggered`
    (`self.Interact_Objects`)
    (`self.Trigged_object`)))

(fn `Character_Mouse_Rotation`
  (bind (_hitresult _returnvalue) (`PlayerController.GetHitResultUnderCursorByChannel` (`GameplayStatics.GetPlayerController` 0) "TraceTypeQuery1" true))
  (if _returnvalue
    (`self.K2_SetActorRotation` self (`KismetMathLibrary.MakeRotator` 0.0 0.0 (.yaw (`KismetMathLibrary.FindLookAtRotation` (`self.K2_GetActorLocation`) (`.Location` (`GameplayStatics.BreakHitResult` _hitresult))))) false)))

(fn `Interact_Objects`
  (set `self.As BPI Medoc Interface Interact` null)
  (set `self.ClosestInterface` null)
  (set `self.Close distans` 1000.0)
  (for _array_element (`PrimitiveComponent.GetOverlappingActors` (`self.interact_colision`) "/Script/Engine.Actor")
    (bind _asbpi_medoc_interface_interact (cast `/Game/Lesson/TTS_PAVEL_M/Blueprints/BP_character/BPI_Medoc_Interface_interact` _array_element))
    (set `self.As BPI Medoc Interface Interact` _asbpi_medoc_interface_interact)
    (bind _returnvalue (`self.GetDistanceTo` self _array_element))
    (if (< _returnvalue (`self.Close distans`))
      (set `self.Close distans` _returnvalue)
      (set `self.ClosestInterface` _array_element)))
  (bind _asbpi_medoc_interface_interact_2 (cast `/Game/Lesson/TTS_PAVEL_M/Blueprints/BP_character/BPI_Medoc_Interface_interact` (`self.ClosestInterface`)))
  (`/Game/Lesson/TTS_PAVEL_M/Blueprints/BP_character/BPI_Medoc_Interface_interact.Interact` _asbpi_medoc_interface_interact_2)
  (return))

(fn `OpenGates`
  (returns (closestGates :type "/Game/Lesson/TTS_PAVEL_M/Blueprints/BP_actors/Buttons_and_gates/BP_chain_link_gates Object Reference")))

(fn `Trigged_object`
  (locals (NewLocalVar :type "/Game/Lesson/TTS_PAVEL_M/Blueprints/BP_character/BPI_trigged Interface"))
  (set `self.As BPI Trigged` null)
  (set `self.Trigger_object` null)
  (set `self.Trigged_distans` 1000.0)
  (for _array_element (`PrimitiveComponent.GetOverlappingActors` (`self.interact_colision`) "/Script/Engine.Actor")
    (bind _asbpi_trigged (cast `/Game/Lesson/TTS_PAVEL_M/Blueprints/BP_character/BPI_trigged` _array_element))
    (set `self.As BPI Trigged` _asbpi_trigged)
    (bind _returnvalue (`self.GetDistanceTo` self _array_element))
    (if (< _returnvalue (`self.Trigged_distans`))
      (set `self.Trigged_distans` _returnvalue)
      (set `self.Trigger_object` _array_element)))
  (bind _asbpi_trigged_2 (cast `/Game/Lesson/TTS_PAVEL_M/Blueprints/BP_character/BPI_trigged` (`self.Trigger_object`)))
  (`/Game/Lesson/TTS_PAVEL_M/Blueprints/BP_character/BPI_trigged. Trigged_object` _asbpi_trigged_2))

(fn `UserConstructionScript`)
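; BP_Weapon_FlameT is a flamethrower weapon whose flame_shoot event fires a short-range flame attack.
; Each call line-traces forward from its Arrow on the Visibility channel and applies fixed damage to the hit actor.
; A DoOnce with a short delay throttles only the effects: spawning BP_flame attached to the Arrow, calling its DeleteFlame and adding an audio component.
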(event `flame_shoot`
  (bind _arrow (`self.Arrow`))
  (bind _arrow_2 (`self.Arrow`))
  (bind _returnvalue (`SceneComponent.K2_GetComponentLocation` _arrow_2))
  (bind _returnvalue_2 (`SceneComponent.K2_GetComponentLocation` _arrow))
  (bind _outhit (`KismetSystemLibrary.LineTraceSingle` :`Start` _returnvalue :`End` (+ _returnvalue (* (`SceneComponent.GetForwardVector` _arrow_2) 300.0)) :`TraceChannel` "TraceTypeQuery1" :`TraceColor` (struct :`G` 0.153495 :`B` 1.0 :`A` 1.0) :`DrawTime` 2.0))
  (`|ExecutionSequence`
    (:`then_0`
      (`/Engine/EditorBlueprintResources/StandardMacros.DoOnce` false :!label _label
        (:`Completed`
          (bind _returnvalue_3 (`|SpawnActorFromClass` "/Game/Lesson/TTS_PAVEL_M/Blueprints/BP_character/BP_flame.BP_flame_C" (`KismetMathLibrary.MakeTransform` _returnvalue_2 (`KismetMathLibrary.FindLookAtRotation` _returnvalue_2 (+ _returnvalue_2 (`SceneComponent.GetForwardVector` _arrow)))) "AlwaysSpawn" "MultiplyWithRoot" null null))
          (`self.K2_AttachToComponent` _returnvalue_3 (`self.Arrow`) "None" "KeepWorld" "KeepWorld" "KeepWorld" true)
          (bind _asbp_flame (cast `/Game/Lesson/TTS_PAVEL_M/Blueprints/BP_character/BP_flame` _returnvalue_3))
          (`/Game/Lesson/TTS_PAVEL_M/Blueprints/BP_character/BP_flame.delete_flame` _asbp_flame)
          (`AddComponent|NODE_AddAudioComponent-0`)
          (`KismetSystemLibrary.Delay` 0.3)
          (goto _label :!via `Reset`))))
    (:`then_1`
      (`GameplayStatics.ApplyDamage` (`.HitActor` (`GameplayStatics.BreakHitResult` _outhit)) 10.0))))

(fn `UserConstructionScript`)
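; A train wagon actor carrying a destructible barrel, moving along a straight path from the start of play.
; A timeline started on BeginPlay lerps the actor along world Y from its start location while rotating four wheel meshes each update.
; Damage reduces Health, swapping the barrel through three crashed meshes at falling thresholds.
; At zero health the actor is destroyed, and an audio component is added after the destroy call.
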(event `self.ReceiveAnyDamage`
  (params (Damage :type "Float (single-precision)") (DamageType :type "DamageType Object Reference") (InstigatedBy :type "Controller Object Reference") (DamageCauser :type "Actor Object Reference"))
  (bind _health (`self.Health`))
  ; Здоровье
  (`KismetSystemLibrary.PrintString` (`KismetStringLibrary.Conv_DoubleToString` _health))
  (bind _output_get (set `self.Health` (- _health Damage)))
  (if (>= _output_get 80.0)
    _
    (elif (>= _output_get 60.0)
      (`StaticMeshComponent.SetStaticMesh` (`self.Barrel_full`) "/Game/Lesson/TTS_PAVEL_M/Meshes/TrainMeshes/Barrel_crash.Barrel_crash")
      (elif (>= _output_get 40.0)
        (`StaticMeshComponent.SetStaticMesh` (`self.Barrel_full`) "/Game/Lesson/TTS_PAVEL_M/Meshes/TrainMeshes/Barrel_crash1.Barrel_crash1")
        (elif (>= _output_get 20.0)
          (`StaticMeshComponent.SetStaticMesh` (`self.Barrel_full`) "/Game/Lesson/TTS_PAVEL_M/Meshes/TrainMeshes/Barrel_crash2.Barrel_crash2")
          (elif (<= _output_get 0.0)
            (`self.K2_DestroyActor`)
            (`AddComponent|NODE_AddAudioComponent-1`)))))))

(event `self.ReceiveBeginPlay`
  ; Движение вагона и вращение колес
  (bind _output_get (set `self.Start Locarion` (`self.K2_GetActorLocation`)))
  (bind (_direction `_новая_дорожка_0`) (`Timeline|Шкала времени`)
    (:`Update`
      (`SceneComponent.K2_AddLocalRotation` (`self.SM_TrainWeels3`) (struct :`Roll` 3.0) false false)
      (`SceneComponent.K2_AddLocalRotation` (`self.SM_TrainWeels2`) (struct :`Roll` 3.0) false false)
      (`SceneComponent.K2_AddLocalRotation` (`self.SM_TrainWeels1`) (struct :`Roll` 3.0) false false)
      (`SceneComponent.K2_AddLocalRotation` (`self.SM_TrainWeels`) (struct :`Roll` 3.0) false false)
      (`self.K2_SetActorLocation` (`KismetMathLibrary.VLerp` (`self.Start Locarion`) (+ _output_get (`KismetMathLibrary.MakeVector` 0.0 4500.0)) `_новая_дорожка_0`)))))

(fn `UserConstructionScript`)
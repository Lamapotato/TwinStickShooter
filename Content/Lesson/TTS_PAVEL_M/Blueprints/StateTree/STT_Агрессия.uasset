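; StateTree task "Агрессия" (Aggression) that makes an AI actor relentlessly chase the player.
; On state entry it reads the Angry flag from the level's BP_RIchagKorobki and finishes successfully when that is off.
; When angry, it runs AI MoveTo on the player pawn with continuous goal tracking, reissuing it after every success or failure.
; An invalid Actor fails the task, while an active chase never finishes it.
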(event `self.ReceiveLatentEnterState`
  (params (Transition :type "StateTreeTransitionResult Structure (by ref)"))
  (bind _returnvalue (`GameplayStatics.GetActorOfClass` "/Game/Lesson/TTS_PAVEL_M/Blueprints/StateTree/BP_RIchagKorobki.BP_RIchagKorobki_C"))
  (if (`/Game/Lesson/TTS_PAVEL_M/Blueprints/StateTree/BP_RIchagKorobki.Angry` _returnvalue)
    (`/Engine/EditorBlueprintResources/StandardMacros.IsValid` (`self.Actor`)
      (:`Is Valid`
        (`AITask_MoveTo.AIMoveTo` (`AIBlueprintHelperLibrary.GetAIController` (`self.Actor`)) (0.0 0.0 0.0) (`GameplayStatics.GetPlayerPawn` 0) 50.0 "Default" "Default" true true true :!label _label
          (:`OnRequestFailed`
            (goto _label))
          (:`OnMoveFinished`
            (goto _label))))
      (:`Is Not Valid`
        (`self.FinishTask` false)))
    (else
      (`self.FinishTask` true))))
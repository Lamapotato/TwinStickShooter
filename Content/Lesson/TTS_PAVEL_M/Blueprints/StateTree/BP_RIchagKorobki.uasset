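; Lever actor that opens the starting chain-link gates once the BP_case boxes meet its unlock condition.
; Tick copies every box's Open flag into an array and allows interaction only when it matches an all-false array, noted as all boxes opened.
; Interact sets Angry and plays a timeline that rotates the handle, calling OpenStartGates on each update.
; TriggedObject applies a highlight material to the button body, which Tick resets each frame.
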(event `self.Interact`
  (if (`self.bInteract`)
    (set `self.Angry` true)
    (bind (_direction `_новая_дорожка_0`) (`Timeline|Шкала времени`)
      (:`Update`
        (`SceneComponent.K2_SetRelativeRotation` (`self.Cylinder_3F7B4177`) (`KismetMathLibrary.RLerp` (struct :`Pitch` -45.0) (struct :`Pitch` 45.0) `_новая_дорожка_0`) false false)
        (bind _returnvalue (`GameplayStatics.GetActorOfClass` "/Game/Lesson/TTS_PAVEL_M/Blueprints/StateTree/BP_chain_link_gates.BP_chain_link_gates_C"))
        (`/Game/Lesson/TTS_PAVEL_M/Blueprints/StateTree/BP_chain_link_gates.OpenStartGates` _returnvalue)))))

(event `self. Trigged_object`
  (`PrimitiveComponent.SetMaterial` (`self.корпус_кнопки`) 0 "/Engine/EditorResources/FieldNodes/_Resources/M_FieldRadiusPreview.M_FieldRadiusPreview"))

(event `self.ReceiveTick`
  (params (DeltaSeconds :type "Float (single-precision)"))
  (`PrimitiveComponent.SetMaterial` (`self.корпус_кнопки`) 0 "/Engine/Tutorial/SubEditors/TutorialAssets/TutorialMaterial.TutorialMaterial")
  ; Если открыть все коробки то разрешенно дернуть рычаг ( "Как есть" - записывает булевое значение каждой коробоки, "Как надо" - записывает все значение в False. И если два массива равны то разрешен интерактив с рычагом)
  (bind _outactors (`GameplayStatics.GetAllActorsOfClass` "/Game/Lesson/TTS_PAVEL_M/Blueprints/StateTree/BP_case.BP_case_C"))
  (set `self.Out Actors` _outactors)
  (bind _output_get (set `self.Case` (`|GetArrayItem` (`self.Out Actors`) (`self.index`)) :!label _label))
  (bind _asbp_case (cast `/Game/Lesson/TTS_PAVEL_M/Blueprints/StateTree/BP_case` _output_get))
  (`KismetArrayLibrary.Array_Set` (`self.Как Есть`) (`self.index`) (`/Game/Lesson/TTS_PAVEL_M/Blueprints/StateTree/BP_case.bOpen` _asbp_case) true)
  (`KismetArrayLibrary.Array_Set` (`self.Как Надо`) (`self.index`) false true)
  (bind _result (`/Engine/EditorBlueprintResources/StandardMacros.IncrementInt` (`self.index`))
    (:`  `
      (if (< _result (`KismetArrayLibrary.Array_Length` (`self.Out Actors`)))
        (goto _label)
        (else
          (set `self.index` 0)
          (if (`KismetArrayLibrary.Array_Identical` (`self.Как Есть`) (`self.Как Надо`))
            (set `self.bInteract` true)
            (else
              (set `self.bInteract` false))))))))

(fn `UserConstructionScript`)
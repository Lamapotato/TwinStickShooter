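; StateTree task that walks an AI actor through the level's BP_case boxes.
; On entering the state it gathers every box, then steps through them by index, skipping any whose Open flag is set.
; It moves to each remaining box with AIMoveTo and calls BotClose on arrival.
; The task finishes as succeeded after the last box or on a failed move request, and stalls on an invalid box.
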(event `self.ReceiveLatentEnterState`
  (params (Transition :type "StateTreeTransitionResult Structure (by ref)"))
  (bind _outactors (`GameplayStatics.GetAllActorsOfClass` "/Game/Lesson/TTS_PAVEL_M/Blueprints/StateTree/BP_case.BP_case_C"))
  (set `self.All_case` _outactors)
  (bind _output_get (set `self.Case` (`|GetArrayItem` (`self.All_case`) (`self.index`)) :!label _label))
  (`/Engine/EditorBlueprintResources/StandardMacros.IsValid` _output_get
    (:`Is Valid`
      (if (== (`/Game/Lesson/TTS_PAVEL_M/Blueprints/StateTree/BP_case.bOpen` (`self.Case`)) false)
        (`AITask_MoveTo.AIMoveTo` (`AIBlueprintHelperLibrary.GetAIController` (`self.Actor`)) (0.0 0.0 0.0) (`self.Case`) 0.0
          (:`OnRequestFailed`
            (`self.FinishTask` true))
          (:`OnMoveFinished`
            (bind _result (`/Engine/EditorBlueprintResources/StandardMacros.IncrementInt` (`self.index`))
              (:`  `
                (if (< _result (`KismetArrayLibrary.Array_Length` (`self.All_case`)))
                  ; Меняем переменную в коробке
                  (`/Game/Lesson/TTS_PAVEL_M/Blueprints/StateTree/BP_case.Bot_close` (`self.Case`))
                  (goto _label)
                  (else
                    (`/Game/Lesson/TTS_PAVEL_M/Blueprints/StateTree/BP_case.Bot_close` (`self.Case`))
                    (`self.FinishTask` true)))))))
        (else
          (bind _result_2 (`/Engine/EditorBlueprintResources/StandardMacros.IncrementInt` (`self.index`))
            (:`  `
              (if (< _result_2 (`KismetArrayLibrary.Array_Length` (`self.All_case`)))
                (goto _label)
                (else
                  (`self.FinishTask` true))))))))))
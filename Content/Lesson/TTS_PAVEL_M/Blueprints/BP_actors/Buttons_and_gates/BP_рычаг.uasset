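; BP_рычаг is an interactive lever that activates gates through a button panel.
; Interact calls ActivetedGates on the BP_Button_panel found by class lookup, then a FlipFlop alternately plays and reverses a timeline that swings the lever cylinder.
; TriggedObject applies a highlight material to the housing, and Tick restores the default every frame, so the highlight lasts only while the event keeps firing.
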(event `/Game/Lesson/TTS_PAVEL_M/Blueprints/BP_character/BPI_Medoc_Interface_interact.Interact`
  (bind _returnvalue (`GameplayStatics.GetActorOfClass` "/Game/Lesson/TTS_PAVEL_M/Blueprints/BP_actors/Buttons_and_gates/BP_Button_panel.BP_Button_panel_C"))
  (`/Game/Lesson/TTS_PAVEL_M/Blueprints/BP_actors/Buttons_and_gates/BP_Button_panel.Activeted_gates` _returnvalue)
  (`/Engine/EditorBlueprintResources/StandardMacros.FlipFlop`
    (:`A`
      (bind (_direction `_новая_дорожка_0`) (`Timeline|Шкала времени` :!label _label)
        (:`Update`
          (`SceneComponent.K2_SetRelativeRotation` (`self.Cylinder_3F7B4177`) (`KismetMathLibrary.RLerp` (struct :`Pitch` -45.0) (struct :`Pitch` 45.0) `_новая_дорожка_0`) false false))))
    (:`B`
      (goto _label :!via `Reverse`))))

(event `/Game/Lesson/TTS_PAVEL_M/Blueprints/BP_character/BPI_trigged. Trigged_object`
  (`PrimitiveComponent.SetMaterial` (`self.корпус_кнопки`) 0 "/Engine/EditorResources/FieldNodes/_Resources/M_FieldRadiusPreview.M_FieldRadiusPreview"))

(event `self.ReceiveTick`
  (params (DeltaSeconds :type "Float (single-precision)"))
  (`PrimitiveComponent.SetMaterial` (`self.корпус_кнопки`) 0 "/Engine/Tutorial/SubEditors/TutorialAssets/TutorialMaterial.TutorialMaterial"))

(fn `UserConstructionScript`)
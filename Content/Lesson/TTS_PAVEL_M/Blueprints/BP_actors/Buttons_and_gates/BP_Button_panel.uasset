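; Button panel for a sequence puzzle that opens the gates after circle, square and triangle are activated in order.
; Each shape event sets a flag and swaps that shape's material, with square requiring circle and triangle requiring square.
; An out-of-order square or triangle clears the other two flags and restores their material.
; A separate event checks all three flags and calls Open on the BP_Gates2 actor found by class.
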(event `Krug`
  (set `self.круг` true)
  (`PrimitiveComponent.SetMaterial` (`self.круг1`) 0 "/Engine/MapTemplates/Materials/BasicAsset03.BasicAsset03"))

(event `Kvadrad`
  (if (`self.круг`)
    (set `self.квадрат` true)
    (`PrimitiveComponent.SetMaterial` (`self.Квадрат`) 0 "/Engine/MapTemplates/Materials/BasicAsset03.BasicAsset03")
    (else
      (set `self.круг` false)
      (set `self.треуг` false)
      (`PrimitiveComponent.SetMaterial` (`self.треугольник`) 0 "/Engine/MapTemplates/Materials/BasicAsset02.BasicAsset02")
      (`PrimitiveComponent.SetMaterial` (`self.круг1`) 0 "/Engine/MapTemplates/Materials/BasicAsset02.BasicAsset02"))))

(event `Treug`
  (if (`self.квадрат`)
    (set `self.треуг` true)
    (`PrimitiveComponent.SetMaterial` (`self.треугольник`) 0 "/Engine/MapTemplates/Materials/BasicAsset03.BasicAsset03")
    (else
      (set `self.круг` false)
      (set `self.квадрат` false)
      (`PrimitiveComponent.SetMaterial` (`self.круг1`) 0 "/Engine/MapTemplates/Materials/BasicAsset02.BasicAsset02")
      (`PrimitiveComponent.SetMaterial` (`self.Квадрат`) 0 "/Engine/MapTemplates/Materials/BasicAsset02.BasicAsset02"))))

(event `Activeted_gates`
  (if (`self.круг`)
    (if (`self.квадрат`)
      (if (`self.треуг`)
        (bind _returnvalue (`GameplayStatics.GetActorOfClass` "/Game/Lesson/TTS_PAVEL_M/Blueprints/BP_actors/Buttons_and_gates/BP_Gates2.BP_Gates2_C"))
        (`/Game/Lesson/TTS_PAVEL_M/Blueprints/BP_actors/Buttons_and_gates/BP_Gates2.Open` _returnvalue)))))

(fn `UserConstructionScript`)
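; BP_UnoptimizedActor is a lesson actor that bobs vertically while doing expensive per-frame work, as an example of unoptimized Blueprint logic.
; A timeline drives a swept move between 200 units below and above the start location, with a FlipFlop alternating reverse and forward playback endlessly.
; Every Tick, it gets all actors in the level and runs a complex visibility line trace with debug drawing to each one.
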(event `self.ReceiveBeginPlay`
  (set `self.StartLocation` (`self.K2_GetActorLocation`))
  (bind (_direction _newtrack_0) (`Timeline|Timeline` :!via `PlayFromStart` :!label _label)
    (:`Update`
      (`self.K2_SetActorLocation` (+ (`self.StartLocation`) (`KismetMathLibrary.MakeVector` 0.0 0.0 (`KismetMathLibrary.Lerp` -200.0 200.0 _newtrack_0))) true))
    (:`Finished`
      (`/Engine/EditorBlueprintResources/StandardMacros.FlipFlop`
        (:`A`
          (goto _label :!via `ReverseFromEnd`))
        (:`B`
          (goto _label :!via `PlayFromStart`))))))

(event `self.ReceiveTick`
  (params (DeltaSeconds :type "Float (single-precision)"))
  (bind _outactors (`GameplayStatics.GetAllActorsOfClass` "/Script/Engine.Actor"))
  (for _array_element _outactors
    (`KismetSystemLibrary.LineTraceSingle` :`Start` (`self.K2_GetActorLocation`) :`End` (`self.K2_GetActorLocation` _array_element) :`TraceChannel` "TraceTypeQuery1" :`bTraceComplex` true :`DrawDebugType` "ForOneFrame")))

(fn `UserConstructionScript`)
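; BP_Human_Alex_Arkhipov is a lesson human Blueprint representing one named person, with a name label and a list of thoughts.
; The construction script writes the Name variable into the Namealex text.
; PrintInfo prints the third entry of Thoughts, and BeginPlay only calls the parent implementation.
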(event `self.ReceiveBeginPlay`
  (`parent.ReceiveBeginPlay`))

(fn `PrintInfo`
  (`KismetSystemLibrary.PrintString` (`KismetTextLibrary.Conv_TextToString` (`KismetTextLibrary.Conv_StringToText` (`|GetArrayItem` (`self.Thoughts`) 2)))))

(fn `UserConstructionScript`
  (`TextRenderComponent.K2_SetText` (`self.namealex`) (`KismetTextLibrary.Conv_StringToText` (`self.Name`))))
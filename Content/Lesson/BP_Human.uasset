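; BP_Human is a lesson Blueprint for a human that displays its draining health on a text component.
; Tick lowers Health at a constant rate, turning the text from green to red below a threshold; construction previews the first Thought.
; BeginPlay and Space print name and age through PrintInfo.
; Unwired flow-control experiments fill the graph, including a data-table lookup and custom loop macros, with Reverse For Loop left unimplemented.
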(event `self.ReceiveBeginPlay`
  (`|ExecutionSequence`
    (:`then_1`
      (`self.PrintInfo`))))

(event `self.ReceiveTick`
  (params (DeltaSeconds :type "Float (single-precision)"))
  (bind _output_get (set `self.Health` (- (`self.Health`) (* DeltaSeconds 10.0))))
  (`TextRenderComponent.K2_SetText` (`self.TextRender`) (`KismetTextLibrary.Conv_DoubleToText` _output_get "HalfToEven"))
  (if (< _output_get 50.0)
    (`TextRenderComponent.SetTextRenderColor` (`self.TextRender`) (make `Color` 0 0 255 255))
    (else
      (`TextRenderComponent.SetTextRenderColor` (`self.TextRender`) (make `Color` 0 255 0 255)))))

(event `Key|SpaceBar`
  (params (Key :type "Key Structure"))
  (:`Pressed`
    (`self.PrintInfo`)))

(fn `PrintInfo`
  (`KismetSystemLibrary.PrintString` (`self.Name`))
  (`KismetSystemLibrary.PrintString` (`KismetStringLibrary.Conv_IntToString` (`self.Age`))))

(fn `UserConstructionScript`
  (`TextRenderComponent.K2_SetText` (`self.TextRender`) (`KismetTextLibrary.Conv_StringToText` (`|GetArrayItem` (`self.Thoughts`)))))
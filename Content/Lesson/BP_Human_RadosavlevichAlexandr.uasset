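; Lesson Blueprint for a "cube-gentleman" human that greets on meeting and says goodbye on leaving.
; Overlapping CollisionHello prints a hello and sets MeetCube, which gates the farewell printed when overlap with CollisionBye ends.
; The construction script shows Name on a TextRender, and an overridden PrintInfo prints Name with the first and third Thoughts entries, without calling the parent.
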(event `self.CollisionHello.OnComponentBeginOverlap`
  (params (OverlappedComponent :type "PrimitiveComponent Object Reference") (OtherActor :type "Actor Object Reference") (OtherComp :type "PrimitiveComponent Object Reference") (OtherBodyIndex :type Integer) (bFromSweep :type Boolean) (SweepResult :type "HitResult Structure (by ref)"))
  ; CUBE-GENTLEMAN: Say hello when meet and goodbye when leave
  (bind _output_get (set `self.Message` "Hello stranger!"))
  (set `self.MeetCube` true)
  (`KismetSystemLibrary.PrintString` _output_get))

(event `self.CollisionBye.OnComponentEndOverlap`
  (params (OverlappedComponent :type "PrimitiveComponent Object Reference") (OtherActor :type "Actor Object Reference") (OtherComp :type "PrimitiveComponent Object Reference") (OtherBodyIndex :type Integer))
  ; CUBE-GENTLEMAN: Say hello when meet and goodbye when leave
  (if (`self.MeetCube`)
    (bind _output_get (set `self.Message` "Goodbye stranger! Have a nice day!"))
    (`KismetSystemLibrary.PrintString` _output_get)))

(fn `PrintInfo`
  ; Output: Name,  First thoughts, Last thoughts
  (`KismetSystemLibrary.PrintString` (`self.Name`))
  (`KismetSystemLibrary.PrintString` (`|GetArrayItem` (`self.Thoughts`)))
  (`KismetSystemLibrary.PrintString` (`|GetArrayItem` (`self.Thoughts`) 2)))

(fn `UserConstructionScript`
  (`TextRenderComponent.K2_SetText` (`self.TextRender`) (`KismetTextLibrary.Conv_StringToText` (`self.Name`))))
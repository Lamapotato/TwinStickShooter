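; BP_Human_VladBocharov is a lesson Blueprint representing a human with a name and a list of thoughts.
; The construction script shows the Name variable on a TextRender component.
; On BeginPlay it calls Printlnfo, which prints the third entry of the Thoughts array, then prints the Name.
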(event `self.ReceiveBeginPlay`
  (`self.Printlnfo`)
  (`KismetSystemLibrary.PrintString` (`self.Name`)))

(fn `Printlnfo`
  (`KismetSystemLibrary.PrintString` (`|GetArrayItem` (`self.Thoughts`) 2)))

(fn `UserConstructionScript`
  (`TextRenderComponent.K2_SetText` (`self.TextRender`) (`KismetTextLibrary.Conv_StringToText` (`self.Name`))))
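; BP_Sorter is a controlled lesson actor that seeks out BP_ActorToSort actors nearest-first and destroys them.
; Each tick it gathers all of them, and FindClosestActor picks the nearest with a linear minimum-distance scan.
; It shows that target's name on a TextRender, moves toward it with SimpleMoveToActor, and destroys it once within a short range.
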(event `self.ReceiveBeginPlay`)

(event `self.ReceiveTick`
  (params (DeltaSeconds :type "Float (single-precision)"))
  (bind _outactors (`GameplayStatics.GetAllActorsOfClass` "/Game/Lesson/BP_ActorToSort.BP_ActorToSort_C"))
  (bind _closestactor (`self.FindClosestActor` _outactors))
  (bind _asbp_actor_to_sort (cast `/Game/Lesson/BP_ActorToSort` _closestactor))
  (`TextRenderComponent.K2_SetText` (`self.TextRender`) (`/Game/Lesson/BP_ActorToSort.Name` _asbp_actor_to_sort))
  (`AIBlueprintHelperLibrary.SimpleMoveToActor` (`self.GetController`) _asbp_actor_to_sort)
  (if (<= (`self.GetDistanceTo` _asbp_actor_to_sort self) 100.0)
    (`self.K2_DestroyActor` _closestactor)))

(fn `FindClosestActor`
  (params (ActorToSort :type "Array of Actor Object Reference"))
  (returns (ClosestActor :type "Actor Object Reference"))
  (locals (ClosestDistance :type "Float (double-precision)" :default 99999.0) (Actor :type "Actor Object Reference"))
  (for _array_element ActorToSort
    (bind _returnvalue (`self.GetDistanceTo` _array_element self))
    (if (> (`local.ClosestDistance`) _returnvalue)
      (set `local.ClosestDistance` _returnvalue)
      (set `local.Actor` _array_element)))
  (return (`local.Actor`)))

(fn `UserConstructionScript`)
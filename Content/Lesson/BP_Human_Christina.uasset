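; BP_Human_Christina is a lesson Blueprint representing a human, with a name label and a list of thoughts.
; The construction script runs the parent script, then writes the Name variable into a TextRender component.
; PrintInfo prints the name and the first Thoughts entry, but nothing in this Blueprint calls it.
; The event graph holds only disabled placeholder events, so it adds no runtime logic.
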(fn `PrintInfo`
  (`KismetSystemLibrary.PrintString` (`self.Name`))
  (`KismetSystemLibrary.PrintString` (`|GetArrayItem` (`self.Thoughts`))))

(fn `UserConstructionScript`
  (`parent.UserConstructionScript`)
  (`TextRenderComponent.K2_SetText` (`self.TextRender`) (`KismetTextLibrary.Conv_NameToText` (`KismetStringLibrary.Conv_StringToName` (`self.Name`)))))
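; BP_weapon2 is a weapon that fires a burst of BP_PROJETTILE projectiles from its Arrow component, using the player's heavy ammo.
; Fire checks Heavyammo on BP_MainCharecter once, then spawns the whole burst in a single loop.
; Spawn positions are randomly scattered around the arrow, while every projectile faces along its forward vector.
; Each projectile decrements and prints the ammo, so the count can drop below zero.
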(event `self.Fire`
  (bind _arrow (`self.Arrow`))
  (bind _returnvalue (`SceneComponent.K2_GetComponentLocation` _arrow))
  (bind _returnvalue_2 (+ _returnvalue (* (`SceneComponent.GetForwardVector` _arrow) (`KismetSystemLibrary.MakeLiteralDouble` (`KismetMathLibrary.RandomFloat`)))))
  (bind _asbp_main_charecter (cast `/Game/ИванПаскарь/BluePrints/BP_MainCharecter` (`GameplayStatics.GetPlayerPawn` 0)))
  (bind _heavyammo (`/Game/ИванПаскарь/BluePrints/BP_MainCharecter.heavyammo` _asbp_main_charecter))
  (if (> _heavyammo 0)
    (for _ (range 6)
      (`|SpawnActorFromClass` "/Game/ИванПаскарь/BluePrints/BP_PROJETTILE.BP_PROJETTILE_C" (`KismetMathLibrary.MakeTransform` (+ _returnvalue_2 (* (`KismetMathLibrary.RandomUnitVector`) 50.0)) (`KismetMathLibrary.FindLookAtRotation` _returnvalue _returnvalue_2)) "AdjustIfPossibleButAlwaysSpawn" "MultiplyWithRoot" null null)
      (bind _result (`/Engine/EditorBlueprintResources/StandardMacros.DecrementInt` _heavyammo)
        (:`  `
          (`KismetSystemLibrary.PrintString` (`KismetStringLibrary.Conv_IntToString` _result)))))))

(fn `UserConstructionScript`
  (`parent.UserConstructionScript`))
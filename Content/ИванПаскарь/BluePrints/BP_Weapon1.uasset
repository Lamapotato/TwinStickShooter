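; BP_Weapon1 is a weapon Blueprint that fires projectiles using the main character's light ammo.
; Its Fire event casts the player 0 pawn to BP_MainCharecter and checks that LightAmmo is above zero.
; It then spawns BP_PROJETTILE at the Arrow component, oriented along the arrow's forward vector, decrements LightAmmo and prints it to screen.
; BeginPlay, overlap and construction add no logic of their own.
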(event `self.ReceiveBeginPlay`)

(event `self.Fire`
  (bind _arrow (`self.Arrow`))
  (bind _returnvalue (`SceneComponent.K2_GetComponentLocation` _arrow))
  (bind _asbp_main_charecter (cast `/Game/ИванПаскарь/BluePrints/BP_MainCharecter` (`GameplayStatics.GetPlayerPawn` 0)))
  (bind _lightammo (`/Game/ИванПаскарь/BluePrints/BP_MainCharecter.LightAmmo` _asbp_main_charecter))
  (if (> _lightammo 0)
    (`|SpawnActorFromClass` "/Game/ИванПаскарь/BluePrints/BP_PROJETTILE.BP_PROJETTILE_C" (`KismetMathLibrary.MakeTransform` _returnvalue (`KismetMathLibrary.FindLookAtRotation` _returnvalue (+ _returnvalue (`SceneComponent.GetForwardVector` _arrow)))) "AdjustIfPossibleButAlwaysSpawn" "MultiplyWithRoot" null null)
    (bind _result (`/Engine/EditorBlueprintResources/StandardMacros.DecrementInt` _lightammo)
      (:`  `
        (`KismetSystemLibrary.PrintString` (`KismetStringLibrary.Conv_IntToString` _result))))))

(fn `UserConstructionScript`
  (`parent.UserConstructionScript`))
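; BP_Weapon1 is a weapon Blueprint that fires projectiles using the player character's light ammo.
; Its Fire event reads LightAmmo from the player pawn cast to BP_MainCharecter, spawns BP_PROJETTILE along the Arrow component's forward vector, and decrements the count.
; Each shot also plays a sound, prints a debug value, and attaches a Niagara muzzle flash that is destroyed after a short delay.
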(event `self.ReceiveBeginPlay`)

(event `self.Fire`
  (bind _arrow (`self.Arrow`))
  (bind _returnvalue (`SceneComponent.K2_GetComponentLocation` _arrow))
  (bind _asbp_main_charecter (cast `/Game/ИванПаскарь/BluePrints/BP_MainCharecter` (`GameplayStatics.GetPlayerPawn` 0)))
  (bind _lightammo (`/Game/ИванПаскарь/BluePrints/BP_MainCharecter.LightAmmo` _asbp_main_charecter))
  (if (> _lightammo 0)
    (`|SpawnActorFromClass` "/Game/ИванПаскарь/BluePrints/Weapon/BP_PROJETTILE.BP_PROJETTILE_C" (`KismetMathLibrary.MakeTransform` _returnvalue (`KismetMathLibrary.FindLookAtRotation` _returnvalue (+ _returnvalue (`SceneComponent.GetForwardVector` _arrow)))) "AdjustIfPossibleButAlwaysSpawn" "MultiplyWithRoot" null null)
    (bind _result (`/Engine/EditorBlueprintResources/StandardMacros.DecrementInt` _lightammo)
      (:`  `
        (`GameplayStatics.SpawnSoundAtLocation` "/Game/ИванПаскарь/BluePrints/Weapon/16551_1460656891.16551_1460656891" _returnvalue (struct) 0.5 2.0 0.0 null null)
        (`KismetSystemLibrary.PrintString` (`KismetStringLibrary.Conv_IntToString` _result))
        (bind _returnvalue_2 (`NiagaraFunctionLibrary.SpawnSystemAttached` "/Game/ИванПаскарь/MuzzleFlash/MuzzleFlash/Niagara/NS_MuzzleFlash.NS_MuzzleFlash" (`self.Arrow`) "None" (0.0 0.0 0.0) (struct) "KeepRelativeOffset" true))
        (`/Engine/EditorBlueprintResources/StandardMacros.IsValid` _returnvalue_2
          (:`Is Valid`
            (`KismetSystemLibrary.Delay` 0.1)
            (`ActorComponent.K2_DestroyComponent` _returnvalue_2)))))))

(fn `UserConstructionScript`
  (`parent.UserConstructionScript`))
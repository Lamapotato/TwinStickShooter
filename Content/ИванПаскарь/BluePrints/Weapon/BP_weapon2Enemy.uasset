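; BP_weapon2Enemy is an enemy shotgun-style weapon that spawns BP_PROJETTILE actors when FireEnemy2 is called.
; A loop spawns projectiles at randomly scattered points around the Arrow component, each rotated toward a point along its forward vector.
; Each shot also calls ApplyDamage with no target connected and spawns a Shotgun sound at zero volume.
; A Delay wires back into the spawn step, so firing keeps repeating.
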(event `FireEnemy2`
  (bind _arrow (`self.Arrow`))
  (bind _returnvalue (`SceneComponent.K2_GetComponentLocation` _arrow))
  (bind _returnvalue_2 (+ _returnvalue (* (`SceneComponent.GetForwardVector` _arrow) (`KismetSystemLibrary.MakeLiteralDouble` (`KismetMathLibrary.RandomFloat`)))))
  (for _ (range 6)
    (`|SpawnActorFromClass` "/Game/ИванПаскарь/BluePrints/Weapon/BP_PROJETTILE.BP_PROJETTILE_C" (`KismetMathLibrary.MakeTransform` (+ _returnvalue_2 (* (`KismetMathLibrary.RandomUnitVector`) 50.0)) (`KismetMathLibrary.FindLookAtRotation` _returnvalue _returnvalue_2)) "AdjustIfPossibleButAlwaysSpawn" "MultiplyWithRoot" null null :!label _label)
    (`GameplayStatics.ApplyDamage` null 5.0)
    (`GameplayStatics.SpawnSoundAtLocation` "/Game/ИванПаскарь/BluePrints/Weapon/shotgun.shotgun" (0.0 0.0 0.0) (struct) 0.0 1.0 1.0 null null)
    (`KismetSystemLibrary.Delay` 2.0)
    (goto _label)))

(fn `UserConstructionScript`)
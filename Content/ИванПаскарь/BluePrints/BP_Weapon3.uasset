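; BP_Weapon3 is a weapon Blueprint, apparently a sniper, that fires projectiles using ammo stored on the player character.
; Its Fire event reads the Sniper count from BP_MainCharecter on player pawn 0 and does nothing when it is empty.
; Otherwise it spawns an enlarged BP_PROJETTILE_Child at the Arrow component along its forward vector, then decrements the count and prints it for debugging.
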(event `self.Fire`
  (bind _arrow (`self.Arrow`))
  (bind _returnvalue (`SceneComponent.K2_GetComponentLocation` _arrow))
  (bind _asbp_main_charecter (cast `/Game/ИванПаскарь/BluePrints/BP_MainCharecter` (`GameplayStatics.GetPlayerPawn` 0)))
  (bind _sniper (`/Game/ИванПаскарь/BluePrints/BP_MainCharecter.sniper` _asbp_main_charecter))
  (if (> _sniper 0)
    (`|SpawnActorFromClass` "/Game/ИванПаскарь/BluePrints/BP_PROJETTILE_Child.BP_PROJETTILE_Child_C" (`KismetMathLibrary.MakeTransform` _returnvalue (`KismetMathLibrary.FindLookAtRotation` _returnvalue (+ _returnvalue (`SceneComponent.GetForwardVector` _arrow))) (1.5 1.5 1.5)) "AdjustIfPossibleButAlwaysSpawn" "MultiplyWithRoot" null null)
    (bind _result (`/Engine/EditorBlueprintResources/StandardMacros.DecrementInt` _sniper)
      (:`  `
        (`KismetSystemLibrary.PrintString` (`KismetStringLibrary.Conv_IntToString` _result))))))

(fn `UserConstructionScript`
  (`parent.UserConstructionScript`))
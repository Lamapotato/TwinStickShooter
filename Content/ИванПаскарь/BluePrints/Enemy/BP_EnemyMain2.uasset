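; Enemy character that chases the player pawn, turns its mesh toward it and fights with a spawned BP_weapon2Enemy attached at its Weapon component.
; A looping timer line-traces to the player and fires only when BP_MainCharecter is hit, while movement re-issues AIMoveTo after each result.
; Damage updates the health text before subtracting, then destroys the enemy at zero.
; Destruction removes the weapon and randomly drops ammo; a grenade drop branch is unconnected.
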(event `self.ReceiveBeginPlay`
  (bind _returnvalue (`GameplayStatics.GetPlayerPawn` 0))
  (`self.WeaponSelekt_0` "/Game/ИванПаскарь/BluePrints/Weapon/BP_weapon2Enemy.BP_weapon2Enemy_C")
  (`KismetSystemLibrary.K2_SetTimerDelegate` (delegate `FireEnemy2`) 1.0 true false 0.0 1.0)
  (`/Engine/EditorBlueprintResources/StandardMacros.IsValid` _returnvalue :!label _label
    (:`Is Valid`
      (`|AIMoveTo` self (0.0 0.0 0.0) _returnvalue
        (:`OnSuccess`
          _)
        (:`OnFail`
          _))
      (`KismetSystemLibrary.Delay` 1.0)
      (goto _label))))

(event `FireEnemy2`
  (bind _outhit (`KismetSystemLibrary.LineTraceSingle` :`Start` (`SceneComponent.K2_GetComponentLocation` (`self.Arrow1`)) :`End` (`self.K2_GetActorLocation` (`GameplayStatics.GetPlayerPawn` 0)) :`TraceChannel` "TraceTypeQuery2" :`DrawTime` 2.0))
  (cast `/Game/ИванПаскарь/BluePrints/BP_MainCharecter` (`.HitActor` (`GameplayStatics.BreakHitResult` _outhit)))
  (`/Game/ИванПаскарь/BluePrints/Weapon/BP_weapon2Enemy.FireEnemy2` (`self.Weapon!_0`)))

(event `self.ReceiveTick`
  (params (DeltaSeconds :type "Float (single-precision)"))
  (bind _returnvalue (`GameplayStatics.GetPlayerPawn` 0))
  (bind (_returnvalue_roll _returnvalue_pitch _returnvalue_yaw) (`KismetMathLibrary.BreakRotator` (`KismetMathLibrary.FindLookAtRotation` (`self.K2_GetActorLocation`) (`self.K2_GetActorLocation` _returnvalue))))
  (`/Engine/EditorBlueprintResources/StandardMacros.IsValid` _returnvalue
    (:`Is Valid`
      (`SceneComponent.K2_SetWorldRotation` (`self.Mesh`) (`KismetMathLibrary.MakeRotator` 0.0 0.0 (+ _returnvalue_yaw -86.0)) false false))))

(event `self.ReceiveAnyDamage`
  (params (Damage :type "Float (single-precision)") (DamageType :type "DamageType Object Reference") (InstigatedBy :type "Controller Object Reference") (DamageCauser :type "Actor Object Reference"))
  (`self.UpdateHealth`)
  (bind _output_get (set `self.healt` (- (`self.healt`) Damage)))
  (if (<= _output_get 0.0)
    (`self.K2_DestroyActor`)))

(event `self.ReceiveDestroyed`
  (bind _mesh (`self.Mesh`))
  (bind _returnvalue (`SceneComponent.K2_GetComponentLocation` _mesh))
  (`/Engine/EditorBlueprintResources/StandardMacros.IsValid` (`self.Weapon!`)
    (:`Is Valid`
      (`self.K2_DestroyActor` (`self.Weapon!_0`))
      (if true
        (if (> (`KismetMathLibrary.RandomFloatInRange` 0.0 100.0) 50.0)
          (`|SpawnActorFromClass` "/Game/ИванПаскарь/BluePrints/Weapon/BP_AmmoEnemy2.BP_AmmoEnemy2_C" (`KismetMathLibrary.MakeTransform` _returnvalue (`KismetMathLibrary.FindLookAtRotation` _returnvalue (+ _returnvalue (`SceneComponent.GetForwardVector` _mesh))) (3.0 3.0 3.0)) "AdjustIfPossibleButAlwaysSpawn" "MultiplyWithRoot" null null))))))

(fn `UpdateHealth_0`
  (`TextRenderComponent.K2_SetText` (`self.TextRender`) (`KismetTextLibrary.Conv_IntToText` (`KismetMathLibrary.FTrunc` (`self.healt`)))))

(fn `UserConstructionScript`
  (`parent.UserConstructionScript`))

(fn `WeaponSelekt_0`
  (params (Class :type "/Game/ИванПаскарь/BluePrints/Weapon/BP_weapon2Enemy Class Reference"))
  (`/Engine/EditorBlueprintResources/StandardMacros.IsValid` (`self.Weapon!_0`)
    (:`Is Valid`
      (`self.K2_DestroyActor` (`self.Weapon!_0`)))
    (:`Is Not Valid`
      _))
  (bind _returnvalue (`|SpawnActorFromClass` Class (`KismetMathLibrary.MakeTransform` (`SceneComponent.K2_GetComponentLocation` (`self.Weapon!`))) "AlwaysSpawn" "MultiplyWithRoot" null null))
  (bind _output_get (set `self.Weapon!_0` _returnvalue))
  (`self.K2_AttachToComponent` _output_get (`self.Weapon!`) "None" "KeepWorld" "KeepWorld" "KeepWorld" true)
  (`self.K2_SetActorRelativeRotation` :`self` _output_get))
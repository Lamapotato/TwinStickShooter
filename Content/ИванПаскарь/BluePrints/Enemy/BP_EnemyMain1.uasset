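; Enemy that chases the player, shoots on sight, and can drop a grenade or ammo pickup when destroyed.
; BeginPlay spawns its weapon, starts a looping fire timer and repeats AIMoveTo toward the player, while Tick yaws the mesh to face them.
; The timer fires the weapon only when a line trace hits BP_MainCharecter.
; Damage refreshes the health text before subtracting, and destruction removes the weapon and rolls the random drop.
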(event `self.ReceiveBeginPlay`
  (bind _returnvalue (`GameplayStatics.GetPlayerPawn` 0))
  (`self.WeaponSelekt` "/Game/ИванПаскарь/BluePrints/Weapon/BP_Weapon1Enemy.BP_Weapon1Enemy_C")
  (`KismetSystemLibrary.K2_SetTimerDelegate` (delegate `FireEnemy1`) 0.2 true false 0.0 1.0)
  (`/Engine/EditorBlueprintResources/StandardMacros.IsValid` _returnvalue :!label _label
    (:`Is Valid`
      (`|AIMoveTo` self (0.0 0.0 0.0) _returnvalue
        (:`OnSuccess`
          _)
        (:`OnFail`
          _))
      (`KismetSystemLibrary.Delay` 1.0)
      (goto _label))))

(event `FireEnemy1`
  (`/Engine/EditorBlueprintResources/StandardMacros.IsValid` (`GameplayStatics.GetPlayerPawn` 0)
    (:`Is Valid`
      (bind _outhit (`KismetSystemLibrary.LineTraceSingle` :`Start` (`SceneComponent.K2_GetComponentLocation` (`self.Arrow1`)) :`End` (`self.K2_GetActorLocation` (`GameplayStatics.GetPlayerPawn` 0)) :`TraceChannel` "TraceTypeQuery2" :`DrawTime` 2.0))
      (cast `/Game/ИванПаскарь/BluePrints/BP_MainCharecter` (`.HitActor` (`GameplayStatics.BreakHitResult` _outhit)))
      (`/Game/ИванПаскарь/BluePrints/Weapon/BP_Weapon1Enemy.FireEnemy1` (`self.Weapon`)))))

(event `self.ReceiveTick`
  (params (DeltaSeconds :type "Float (single-precision)"))
  (bind _returnvalue (`GameplayStatics.GetPlayerPawn` 0))
  (bind (_returnvalue_roll _returnvalue_pitch _returnvalue_yaw) (`KismetMathLibrary.BreakRotator` (`KismetMathLibrary.FindLookAtRotation` (`self.K2_GetActorLocation`) (`self.K2_GetActorLocation` _returnvalue))))
  (`/Engine/EditorBlueprintResources/StandardMacros.IsValid` _returnvalue
    (:`Is Valid`
      (`SceneComponent.K2_SetWorldRotation` (`self.Mesh`) (`KismetMathLibrary.MakeRotator` 0.0 0.0 (+ _returnvalue_yaw -86.0)) false false))))

(event `self.ReceiveAnyDamage`
  (params (Damage :type "Float (single-precision)") (DamageType :type "DamageType Object Reference") (InstigatedBy :type "Controller Object Reference") (DamageCauser :type "Actor Object Reference"))
  (`self.UpdateHealth`)
  (bind _output_get (set `self.Health` (- (`self.Health`) Damage)))
  (if (<= _output_get 0.0)
    (`self.K2_DestroyActor`)))

(event `self.ReceiveDestroyed`
  (bind _mesh (`self.Mesh`))
  (bind _mesh_2 (`self.Mesh`))
  (bind _returnvalue (`SceneComponent.K2_GetComponentLocation` _mesh))
  (bind _returnvalue_2 (`SceneComponent.K2_GetComponentLocation` _mesh_2))
  (`/Engine/EditorBlueprintResources/StandardMacros.IsValid` (`self.Weapon`)
    (:`Is Valid`
      (`self.K2_DestroyActor` (`self.Weapon`))
      (set `self.Random` (`KismetMathLibrary.RandomFloatInRange` 0.0 100.0))
      (if (> (`self.Random`) 50.0)
        (if (> (`self.Random`) 75.0)
          (`|SpawnActorFromClass` "/Game/ИванПаскарь/BluePrints/Weapon/BP_Granade.BP_Granade_C" (`KismetMathLibrary.MakeTransform` _returnvalue (`KismetMathLibrary.FindLookAtRotation` _returnvalue (+ _returnvalue (`SceneComponent.GetForwardVector` _mesh))) (3.0 3.0 3.0)) "AdjustIfPossibleButAlwaysSpawn" "MultiplyWithRoot" null null)
          (else
            (`|SpawnActorFromClass` "/Game/ИванПаскарь/BluePrints/Weapon/BP_AmmoEnemy1.BP_AmmoEnemy1_C" (`KismetMathLibrary.MakeTransform` _returnvalue_2 (`KismetMathLibrary.FindLookAtRotation` _returnvalue_2 (+ _returnvalue_2 (`SceneComponent.GetForwardVector` _mesh_2))) (3.0 3.0 3.0)) "AdjustIfPossibleButAlwaysSpawn" "MultiplyWithRoot" null null)))))))

(fn `UpdateHealth`
  (`TextRenderComponent.K2_SetText` (`self.TextRender`) (`KismetTextLibrary.Conv_IntToText` (`KismetMathLibrary.FTrunc` (`self.Health`)))))

(fn `UserConstructionScript`)

(fn `WeaponSelekt`
  (params (Class :type "/Game/ИванПаскарь/BluePrints/Weapon/BP_Weapon1Enemy Class Reference"))
  (`/Engine/EditorBlueprintResources/StandardMacros.IsValid` (`self.Weapon`)
    (:`Is Valid`
      (`self.K2_DestroyActor` (`self.Weapon`)))
    (:`Is Not Valid`
      _))
  (bind _returnvalue (`|SpawnActorFromClass` Class (`KismetMathLibrary.MakeTransform` (`SceneComponent.K2_GetComponentLocation` (`self.Weapon!`))) "AlwaysSpawn" "MultiplyWithRoot" null null))
  (bind _output_get (set `self.Weapon` _returnvalue))
  (`self.K2_AttachToComponent` _output_get (`self.Weapon!`) "None" "KeepWorld" "KeepWorld" "KeepWorld" true)
  (`self.K2_SetActorRelativeRotation` :`self` _output_get))
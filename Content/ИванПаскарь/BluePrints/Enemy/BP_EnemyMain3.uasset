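; BP_EnemyMain3 is an enemy that chases player 0, turning its mesh to face them every tick.
; On BeginPlay it spawns BP_Weapon3Enemy onto its Weapon component and fires it on a one-second looping timer.
; Damage lowers health (NewVar0), with the death check subtracting Damage again after the update.
; On destruction it removes the weapon and randomly drops BP_AmmoEnemy3, BP_Granade or nothing.
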(event `self.ReceiveBeginPlay`
  (`self.WeaponSelekt_0` "/Game/ИванПаскарь/BluePrints/Weapon/BP_Weapon3Enemy.BP_Weapon3Enemy_C")
  (`KismetSystemLibrary.K2_SetTimerDelegate` (delegate `CustomEvent_1`) 1.0 true))

(event `CustomEvent_1`
  (`/Game/ИванПаскарь/BluePrints/Weapon/BP_Weapon3Enemy.FireEnemy3` (`self.weapon3`)))

(event `self.ReceiveTick`
  (params (DeltaSeconds :type "Float (single-precision)"))
  (bind _returnvalue (`GameplayStatics.GetPlayerPawn` 0))
  (bind (_returnvalue_roll _returnvalue_pitch _returnvalue_yaw) (`KismetMathLibrary.BreakRotator` (`KismetMathLibrary.FindLookAtRotation` (`self.K2_GetActorLocation`) (`self.K2_GetActorLocation` _returnvalue))))
  (bind (_returnvalue_x _returnvalue_y) (`KismetMathLibrary.BreakVector` (`KismetMathLibrary.Normal` (- (`self.K2_GetActorLocation` (`GameplayStatics.GetPlayerPawn` 0)) (`self.K2_GetActorLocation`)))))
  (`/Engine/EditorBlueprintResources/StandardMacros.IsValid` _returnvalue
    (:`Is Valid`
      (`SceneComponent.K2_SetWorldRotation` (`self.Mesh`) (`KismetMathLibrary.MakeRotator` 0.0 0.0 (+ _returnvalue_yaw -86.0)) false false)
      (`PawnMovementComponent.AddInputVector` (`self.CharacterMovement`) (`KismetMathLibrary.MakeVector` _returnvalue_x _returnvalue_y) false))))

(event `self.ReceiveAnyDamage`
  (params (Damage :type "Float (single-precision)") (DamageType :type "DamageType Object Reference") (InstigatedBy :type "Controller Object Reference") (DamageCauser :type "Actor Object Reference"))
  (bind _returnvalue (- (`self.NewVar_0`) Damage))
  (set `self.NewVar_0` _returnvalue)
  (if (<= _returnvalue 0.0)
    (`self.K2_DestroyActor`)))

(event `self.ReceiveDestroyed`
  (`/Engine/EditorBlueprintResources/StandardMacros.IsValid` (`self.weapon3`)
    (:`Is Valid`
      (`self.K2_DestroyActor` (`self.weapon3`))
      (if (> (`KismetMathLibrary.RandomIntegerInRange` 0 50) 25)
        (`|SpawnActorFromClass` "/Game/ИванПаскарь/BluePrints/Weapon/BP_AmmoEnemy3.BP_AmmoEnemy3_C" (`KismetMathLibrary.MakeTransform` (`SceneComponent.K2_GetComponentLocation` (`self.Mesh`)) (struct) (50.0 50.0 50.0)) "AlwaysSpawn" "MultiplyWithRoot" null null)
        (elif (> (`KismetMathLibrary.RandomIntegerInRange` 0 25) 5)
          (`|SpawnActorFromClass` "/Game/ИванПаскарь/BluePrints/Weapon/BP_Granade.BP_Granade_C" (`KismetMathLibrary.MakeTransform` (`SceneComponent.K2_GetComponentLocation` (`self.Mesh`)) (struct) (5.0 5.0 5.0)) "AlwaysSpawn" "MultiplyWithRoot" null null))))))

(fn `UserConstructionScript`)

(fn `WeaponSelekt_0`
  (params (Class :type "/Game/ИванПаскарь/BluePrints/Weapon/BP_Weapon3Enemy Class Reference"))
  (`/Engine/EditorBlueprintResources/StandardMacros.IsValid` (`self.weapon3`)
    (:`Is Valid`
      (`self.K2_DestroyActor` (`self.weapon3`)))
    (:`Is Not Valid`
      _))
  (bind _returnvalue (`|SpawnActorFromClass` Class (`KismetMathLibrary.MakeTransform` (`SceneComponent.K2_GetComponentLocation` (`self.Weapon!`))) "AlwaysSpawn" "MultiplyWithRoot" null null))
  (bind _output_get (set `self.weapon3` _returnvalue))
  (`self.K2_AttachToComponent` _output_get (`self.Weapon!`) "None" "KeepWorld" "KeepWorld" "KeepWorld" true)
  (`self.K2_SetActorRelativeRotation` :`self` _output_get))
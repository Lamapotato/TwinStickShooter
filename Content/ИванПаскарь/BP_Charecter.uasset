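; Player character for a top-down shooter that moves on world axes, jumps, aims at the mouse cursor and fires a held weapon.
; Enhanced Input drives movement, swapping walk and idle animations directly on the mesh without an Anim Blueprint state machine.
; Each tick, a cursor trace yaws only the mesh toward the hit point.
; ChangeWeapon replaces the current weapon with one attached to the hand socket, used for the rocket launcher slot.
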(event `self.ReceiveBeginPlay`
  (bind _returnvalue (pcsubsystem `EnhancedInputLocalPlayerSubsystem` (`GameplayStatics.GetPlayerController` 0)))
  (`EnhancedInputSubsystemInterface.ClearAllMappings` _returnvalue)
  (`EnhancedInputSubsystemInterface.AddMappingContext` _returnvalue "/Game/TSS/Blueprints/IMC_TSSMovent.IMC_TSSMovent" 0 (struct))
  (set `PlayerController.bShowMouseCursor` true (`GameplayStatics.GetPlayerController` 0)))

(event `EnhancedInput|/Game/TSS/Blueprints/IA_TSSMove`
  (params (ActionValue :type "Vector2D Structure") (ElapsedSeconds :type "Float (double-precision)") (TriggeredSeconds :type "Float (double-precision)") (InputAction :type "InputAction Object Reference" :default "/Game/TSS/Blueprints/IA_TSSMove.IA_TSSMove"))
  (bind (_x _y) (`KismetMathLibrary.BreakVector2D` ActionValue))
  (bind _mesh (`self.Mesh`))
  (:`Triggered`
    (`PawnMovementComponent.AddInputVector` (`self.CharacterMovement`) (`KismetMathLibrary.MakeVector` _x _y) false))
  (:`Started`
    (`SkeletalMeshComponent.SetAnimation` _mesh "/Game/Characters/Mannequins/Anims/Rifle/Walk/MF_Rifle_Walk_Fwd.MF_Rifle_Walk_Fwd"))
  (:`Completed`
    (`SkeletalMeshComponent.SetAnimation` _mesh "/Game/Characters/Mannequins/Anims/Rifle/MF_Rifle_Idle_ADS.MF_Rifle_Idle_ADS")))

(event `EnhancedInput|/Game/TSS/Blueprints/IA_TSSJump`
  (params (ActionValue :type Boolean) (ElapsedSeconds :type "Float (double-precision)") (TriggeredSeconds :type "Float (double-precision)") (InputAction :type "InputAction Object Reference" :default "/Game/TSS/Blueprints/IA_TSSJump.IA_TSSJump"))
  (:`Triggered`
    (`self.Jump`)))

(event `EnhancedInput|/Game/TSS/Blueprints/IA_TSSFire`
  (params (ActionValue :type Boolean) (ElapsedSeconds :type "Float (double-precision)") (TriggeredSeconds :type "Float (double-precision)") (InputAction :type "InputAction Object Reference" :default "/Game/TSS/Blueprints/IA_TSSFire.IA_TSSFire"))
  (:`Triggered`
    (`/Engine/EditorBlueprintResources/StandardMacros.IsValid` (`self.Weapon`)
      (:`Is Valid`
        (`/Game/ИванПаскарь/BP_Ракетница.fire 1` (`self.Weapon`))))))

(event `self.ReceiveTick`
  (params (DeltaSeconds :type "Float (single-precision)"))
  (bind (_hitresult _returnvalue) (`PlayerController.GetHitResultUnderCursorByChannel` (`GameplayStatics.GetPlayerController` 0) "TraceTypeQuery1" true))
  (bind (_returnvalue_roll _returnvalue_pitch _returnvalue_yaw) (`KismetMathLibrary.BreakRotator` (`KismetMathLibrary.FindLookAtRotation` (`self.K2_GetActorLocation`) (`.Location` (`GameplayStatics.BreakHitResult` _hitresult)))))
  (cast `PlayerController` (`self.GetController`))
  (if _returnvalue
    (`SceneComponent.K2_SetRelativeRotation` (`self.Mesh`) (`KismetMathLibrary.MakeRotator` 0.0 0.0 (+ _returnvalue_yaw -90.0)) false false)))

(event `EnhancedInput|/Game/TSS/Blueprints/IA_TSSSelectWeapon1`
  (params (ActionValue :type Boolean) (ElapsedSeconds :type "Float (double-precision)") (TriggeredSeconds :type "Float (double-precision)") (InputAction :type "InputAction Object Reference" :default "/Game/TSS/Blueprints/IA_TSSSelectWeapon1.IA_TSSSelectWeapon1"))
  (:`Triggered`
    (`self.ChangeWeapon` "/Game/ИванПаскарь/BP_Ракетница.BP_Ракетница_C")))

(fn `ChangeWeapon`
  (params (WeaponClass :type "/Game/ИванПаскарь/BP_Ракетница Class Reference"))
  (bind _mesh (`self.Mesh`))
  (`/Engine/EditorBlueprintResources/StandardMacros.IsValid` (`self.Weapon`)
    (:`Is Valid`
      (`self.K2_DestroyActor` (`self.Weapon`)))
    (:`Is Not Valid`
      _))
  (bind _returnvalue (`|SpawnActorFromClass` WeaponClass (`KismetMathLibrary.MakeTransform` (`SceneComponent.K2_GetComponentLocation` _mesh) (`SceneComponent.GetSocketRotation` _mesh "hand_r_weapon")) "AlwaysSpawn" "MultiplyWithRoot" null null))
  (bind _output_get (set `self.Weapon` _returnvalue))
  (`self.K2_AttachToComponent` _output_get (`self.Mesh`) "hand_r_weapon" "SnapToTarget" "SnapToTarget" "SnapToTarget" true)
  (`self.K2_SetActorRelativeRotation` :`self` _output_get))

(fn `UserConstructionScript`)
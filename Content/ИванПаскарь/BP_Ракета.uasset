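; BP_Ракета is a rocket projectile actor that explodes when its ProjectileMovement stops.
; On stop it spawns a bomb explosion emitter, then applies fixed damage to Pawn and WorldStatic actors found by a sphere overlap sized by its Radius variable around the mesh.
; It then plays an explosion sound and destroys itself, with all logic in that one event.
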(event `self.ProjectileMovement.OnProjectileStop`
  (params (ImpactResult :type "HitResult Structure (by ref)"))
  (`GameplayStatics.SpawnEmitterAtLocation` "/Game/ExampleContent/Blueprint_Communication/Effects/P_Explosion_Bomb.P_Explosion_Bomb" (`self.K2_GetActorLocation`))
  (bind _outactors (`KismetSystemLibrary.SphereOverlapActors` (`SceneComponent.K2_GetComponentLocation` (`self.StaticMesh`)) (`self.Radius`) (`|MakeArray` "ObjectTypeQuery3" "ObjectTypeQuery1" :!type "EObjectTypeQuery Enum")))
  (for _array_element _outactors
    (`GameplayStatics.ApplyDamage` _array_element 5.0 null self))
  (`GameplayStatics.PlaySoundAtLocation` "/Game/TSS/Sounds/big-bang.big-bang" (`SceneComponent.K2_GetComponentLocation` (`self.StaticMesh`)) (struct) 1.0 1.0 0.0 null null null null)
  (`self.K2_DestroyActor`))

(fn `UserConstructionScript`)
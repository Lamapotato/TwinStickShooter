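; Scatter actor that places instanced banner and statue meshes on surfaces around its location, judging by its naming.
; CreateBannersStatue runs two loops sized by HowManyBanners, tracing downward from random offsets scaled by ScatterDistance, with debug drawing.
; Each hit adds a randomly yawed instance to that loop's InstancedStaticMesh component, the first at double scale.
; DeleteMeshes clears both instance sets; the construction script is empty.
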(event `CreateBannersStatue`
  (bind _returnvalue (+ (* (`KismetMathLibrary.RandomUnitVector`) (`self.ScatterDistance`)) (`self.K2_GetActorLocation`)))
  (bind _returnvalue_2 (+ (* (`KismetMathLibrary.RandomUnitVector`) (`self.ScatterDistance`)) (`self.K2_GetActorLocation`)))
  (`|ExecutionSequence`
    (:`then_0`
      (for _ (range (+ (`self.HowManyBanners`) 1))
        (bind (_outhit _returnvalue_3) (`KismetSystemLibrary.LineTraceSingle` :`Start` _returnvalue_2 :`End` (- _returnvalue_2 (0.0 0.0 500.0)) :`TraceChannel` "TraceTypeQuery1" :`DrawDebugType` "ForDuration"))
        (if _returnvalue_3
          (`InstancedStaticMeshComponent.AddInstance` (`self.InstancedStaticMesh`) (`KismetMathLibrary.MakeTransform` (`.Location` (`GameplayStatics.BreakHitResult` _outhit)) (`KismetMathLibrary.MakeRotator` 0.0 0.0 (`KismetMathLibrary.RandomFloatInRange` 0.0 360.0)) (2.0 2.0 2.0)) true))))
    (:`then_1`
      (for _ (range (+ (`self.HowManyBanners`) 1))
        (bind (_outhit_2 _returnvalue_4) (`KismetSystemLibrary.LineTraceSingle` :`Start` _returnvalue :`End` (- _returnvalue (0.0 0.0 500.0)) :`TraceChannel` "TraceTypeQuery1" :`DrawDebugType` "ForDuration"))
        (if _returnvalue_4
          (`InstancedStaticMeshComponent.AddInstance` (`self.InstancedStaticMesh1`) (`KismetMathLibrary.MakeTransform` (`.Location` (`GameplayStatics.BreakHitResult` _outhit_2)) (`KismetMathLibrary.MakeRotator` 0.0 0.0 (`KismetMathLibrary.RandomFloatInRange` 0.0 360.0))) true))))))

(event `DeleteMeshes`
  (`InstancedStaticMeshComponent.ClearInstances` (`self.InstancedStaticMesh`))
  (`InstancedStaticMeshComponent.ClearInstances` (`self.InstancedStaticMesh1`)))

(fn `UserConstructionScript`)
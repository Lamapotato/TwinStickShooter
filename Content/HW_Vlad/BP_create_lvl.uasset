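; Room generator actor that, on its CreateRoom event, spawns static mesh actors in an X by Y grid from its location.
; Nested loops lay Block meshes as floor and raised Column meshes along the four edges, rotating those on the X edges.
; The edge loops nest inside earlier loops, so columns spawn repeatedly in the same spots.
; NewMacro, a loop with a randomized bound check, is not used by the event.
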(event `CreateRoom`
  (bind _y (`self.y`))
  (bind _x (`self.x`))
  (for _index (range (+ (`self.x`) 1))
    (for _index_2 (range (+ (`self.y`) 1))
      (bind _returnvalue (`|SpawnActorFromClass` "/Script/Engine.StaticMeshActor" (`KismetMathLibrary.MakeTransform` (+ (`self.K2_GetActorLocation`) (`KismetMathLibrary.MakeVector` (* _index (`self.offset`)) (* _index_2 (`self.offset`)))) (struct) (3.0 3.0 3.0)) "Undefined" "MultiplyWithRoot" null null))
      (`StaticMeshComponent.SetStaticMesh` (`StaticMeshActor.StaticMeshComponent` _returnvalue) "/Game/HW_Vlad/Assets/Block/block/StaticMeshes/block.block"))
    (for _index_3 (range (+ (`self.x`) 1))
      (for _index_4 (range (+ _y 1))
        (if (or (== _index_4 0) (== _y _index_4) false false)
          (bind _returnvalue_2 (`|SpawnActorFromClass` "/Script/Engine.StaticMeshActor" (`KismetMathLibrary.MakeTransform` (+ (`self.K2_GetActorLocation`) (`KismetMathLibrary.MakeVector` (* _index_3 (`self.offset`)) (* _index_4 (`self.offset`)) 100.0)) (struct) (4.0 4.0 4.0)) "Undefined" "MultiplyWithRoot" null null))
          (`StaticMeshComponent.SetStaticMesh` (`StaticMeshActor.StaticMeshComponent` _returnvalue_2) "/Game/HW_Vlad/Assets/Colomn/column/StaticMeshes/column.column")
          (for _index_5 (range (+ _x 1))
            (for _index_6 (range (+ (`self.y`) 1))
              (if (or false false (== _index_5 _x) (== _index_5 0))
                (bind _returnvalue_3 (`|SpawnActorFromClass` "/Script/Engine.StaticMeshActor" (`KismetMathLibrary.MakeTransform` (+ (`self.K2_GetActorLocation`) (`KismetMathLibrary.MakeVector` (* _index_5 (`self.offset`)) (* _index_6 (`self.offset`)) 100.0)) (`KismetMathLibrary.MakeRotator` 0.0 0.0 90.0) (4.0 4.0 4.0)) "Undefined" "MultiplyWithRoot" null null))
                (`StaticMeshComponent.SetStaticMesh` (`StaticMeshActor.StaticMeshComponent` _returnvalue_3) "/Game/HW_Vlad/Assets/Colomn/column/StaticMeshes/column.column")))))))))

(fn `UserConstructionScript`)
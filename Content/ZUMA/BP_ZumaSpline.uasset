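; BP_ZumaSpline is the track of a Zuma-style game, driving a chain of colored balls along a spline.
; A speed-based timer spawns balls from a color list, while Tick advances each by distance, reversing those ahead of gaps and destroying those reaching the end.
; InsertBall shifts the chain to fit a new ball and triggers its neighbor check.
; CheckForMatchingBalls scans adjacent balls and removes same-color runs of three or more.
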(event `self.ReceiveBeginPlay`
  (bind _returnvalue (`KismetSystemLibrary.K2_SetTimerDelegate` (`|CreateDelegate` :!event `SpawnBall`) (* (/ 1.0 (`self.BallsSpeed`)) 100.0) true))
  (set `self.SpawnTimer` _returnvalue))

(event `self.ReceiveTick`
  (params (DeltaSeconds :type "Float (single-precision)"))
  (for _array_element (`self.Balls`)
    (`self.UpdateBallLocation` _array_element)))

(event `AddBallToStart`
  (params (NewBall :type "/Game/ZUMA/BP_ZumaBall Object Reference"))
  (`KismetArrayLibrary.Array_AddUnique` (`self.Balls`) NewBall))

(event `SpawnBall`
  (bind _returnvalue (`|SpawnActorFromClass` "/Game/ZUMA/BP_ZumaBall.BP_ZumaBall_C" (`KismetMathLibrary.MakeTransform` (0.0 0.0 -1000.0)) "Undefined" "MultiplyWithRoot" null (`|GetArrayItem` (`self.ColorsToSpawn`) (`self.ColorsIndex`)) true null))
  (`self.AddBallToStart` _returnvalue)
  (`/Engine/EditorBlueprintResources/StandardMacros.IncrementInt` (`self.ColorsIndex`)
    (:`  `
      (if (not (`KismetArrayLibrary.Array_IsValidIndex` (`self.ColorsToSpawn`) (`self.ColorsIndex`)))
        (`KismetSystemLibrary.K2_PauseTimerHandle` (`self.SpawnTimer`))))))

(event `InsertBall`
  (params (Ball :type "/Game/ZUMA/BP_ZumaBall Object Reference") (Color :type "/Game/ZUMA/E_ZumaColors Enum" :default "NewEnumerator0"))
  (bind _balls (`self.Balls`))
  (bind _distanceonspline (`/Game/ZUMA/BP_ZumaBall.DistanceOnSpline` Ball))
  (bind _returnvalue (`KismetArrayLibrary.Array_Find` _balls Ball))
  (for (_array_element _array_index) _balls
    (set `/Game/ZUMA/BP_ZumaBall.DistanceOnSpline` (+ (`/Game/ZUMA/BP_ZumaBall.DistanceOnSpline` _array_element) (select `bool` (> _array_index _returnvalue) :`false` 100.0)) _array_element))
  (bind _returnvalue_2 (`|SpawnActorFromClass` "/Game/ZUMA/BP_ZumaBall.BP_ZumaBall_C" (`KismetMathLibrary.MakeTransform` (0.0 0.0 0.0)) "Undefined" "MultiplyWithRoot" null Color true null))
  (set `self.NewBall` _returnvalue_2)
  (set `/Game/ZUMA/BP_ZumaBall.DistanceOnSpline` _distanceonspline _returnvalue_2)
  (`KismetArrayLibrary.Array_Insert` (`self.Balls`) _returnvalue_2 _returnvalue)
  (set `/Game/ZUMA/BP_ZumaBall.DistanceOnSpline` (- _distanceonspline 100.0) Ball)
  (for _array_element_2 (`self.Balls`)
    (`self.UpdateBallLocation` _array_element_2))
  (`/Game/ZUMA/BP_ZumaBall.CheckClosestBalls` (`self.NewBall`)))

(fn `CheckForMatchingBalls`
  (params (Index :type Integer))
  (locals (LastRightIndex :type Integer :default 0) (AmountOfSameColor :type Integer :default 0))
  (bind _lastrightindex (`local.LastRightIndex`))
  (bind _output (`|GetArrayItem` (`self.Balls`) (`local.Index`)))
  (bind _output_2 (`|GetArrayItem` (`self.Balls`) (`local.Index`)))
  (bind _output_3 (`|GetArrayItem` (`self.Balls`) (- (`local.Index`) 1)))
  (bind _output_4 (`|GetArrayItem` (`self.Balls`) (+ (`local.Index`) 1)))
  (if (`KismetArrayLibrary.Array_IsValidIndex` (`self.Balls`) (+ (`local.Index`) 1)) :!label _label
    (if (and (<= (`self.GetDistanceTo` _output_2 _output_4) 110.0) (`|EnumEquality` (`/Game/ZUMA/BP_ZumaBall.Color` _output_2) (`/Game/ZUMA/BP_ZumaBall.Color` _output_4)))
      (`/Engine/EditorBlueprintResources/StandardMacros.IncrementInt` (`local.Index`)
        (:`  `
          (goto _label)))
      (else
        _)))
  (set `local.LastRightIndex` (`local.Index`))
  (if (`KismetArrayLibrary.Array_IsValidIndex` (`self.Balls`) (- (`local.Index`) 1)) :!label _label_2
    (if (and (<= (`self.GetDistanceTo` _output _output_3) 110.0) (`|EnumEquality` (`/Game/ZUMA/BP_ZumaBall.Color` _output) (`/Game/ZUMA/BP_ZumaBall.Color` _output_3)))
      (`/Engine/EditorBlueprintResources/StandardMacros.IncrementInt` (`local.AmountOfSameColor`)
        (:`  `
          (`/Engine/EditorBlueprintResources/StandardMacros.DecrementInt` (`local.Index`)
            (:`  `
              (goto _label_2)))))
      (else
        _)))
  (if (>= (`local.AmountOfSameColor`) 2)
    (for _index (range (- _lastrightindex (`local.AmountOfSameColor`)) (+ _lastrightindex 1))
      (`self.SetLifeSpan` (`|GetArrayItem` (`self.Balls`) _index) 0.1))))

(fn `UpdateBallLocation`
  (params (Ball :type "/Game/ZUMA/BP_ZumaBall Object Reference"))
  (locals (PrevBallLaggingBehind :type Boolean))
  (bind _balls (`self.Balls`))
  (bind _returnvalue (+ (`KismetArrayLibrary.Array_Find` (`self.Balls`) (`local.Ball`)) 1))
  (`/Engine/EditorBlueprintResources/StandardMacros.IsValid` Ball
    (:`Is Valid`
      (if (`KismetArrayLibrary.Array_IsValidIndex` _balls _returnvalue)
        (set `local.PrevBallLaggingBehind` (<= (+ (`/Game/ZUMA/BP_ZumaBall.DistanceOnSpline` (`|GetArrayItem` _balls _returnvalue)) 100.0) (`/Game/ZUMA/BP_ZumaBall.DistanceOnSpline` (`local.Ball`)))))
      (bind _output_get (set `/Game/ZUMA/BP_ZumaBall.DistanceOnSpline` (+ (`/Game/ZUMA/BP_ZumaBall.DistanceOnSpline` (`local.Ball`)) (* (`self.BallsSpeed`) (`GameplayStatics.GetWorldDeltaSeconds`) (select `bool` (`local.PrevBallLaggingBehind`) :`false` 1.0 :`true` -1.0))) (`local.Ball`)))
      (`self.K2_SetActorLocation` (`local.Ball`) (`SplineComponent.GetLocationAtDistanceAlongSpline` (`self.Spline`) _output_get "World") false false)
      (if (>= (`/Game/ZUMA/BP_ZumaBall.DistanceOnSpline` (`local.Ball`)) (`SplineComponent.GetSplineLength` (`self.Spline`)))
        (`KismetArrayLibrary.Array_RemoveItem` (`self.Balls`) (`local.Ball`))
        (`self.K2_DestroyActor` (`local.Ball`))))
    (:`Is Not Valid`
      (`KismetArrayLibrary.Array_RemoveItem` (`self.Balls`) Ball))))

(fn `UserConstructionScript`)
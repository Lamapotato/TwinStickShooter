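; Procedural room generator actor that builds a rectangular room from a configurable X/Y grid of floor tiles and perimeter wall pieces.
; The construction script clears and rebuilds two instanced static mesh components, rotating edge walls and adding extra pieces at corners.
; SpawnRoom copies each instance into an individual StaticMeshActor.
; ScatterHealthPacks line-traces downward from random points around the actor and spawns floating healthkit items at the hits.
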(event `SpawnRoom`
  (`self.SpawnActorsFromInstances` (`self.InstancedStaticMesh`))
  (`self.SpawnActorsFromInstances` (`self.InstancedStaticMesh1`)))

(event `ScatterHealthPacks`
  (bind _returnvalue (+ (* (`KismetMathLibrary.RandomUnitVector`) (`self.ScatterDistance`)) (`self.K2_GetActorLocation`)))
  (for _ (range (+ (`self.NumberOfHealthkits`) 1))
    (bind (_outhit _returnvalue_2) (`KismetSystemLibrary.LineTraceSingle` :`Start` _returnvalue :`End` (- _returnvalue (0.0 0.0 500.0)) :`TraceChannel` "TraceTypeQuery1" :`DrawDebugType` "ForDuration"))
    (if _returnvalue_2
      (`|SpawnActorFromClass` "/Game/TSS/Blueprints/Items/BP_FloatingItem_Healthkit.BP_FloatingItem_Healthkit_C" (`KismetMathLibrary.MakeTransform` (`.Location` (`GameplayStatics.BreakHitResult` _outhit))) "Undefined" "MultiplyWithRoot" null null))))

(fn `GenerateRoom`
  (locals (FirstXRow :type Boolean) (LastXRow :type Boolean) (FirstYRow :type Boolean) (LastYRow :type Boolean) (z :type "Float (single-precision)") (Offset :type "Vector Structure"))
  (`|ExecutionSequence`
    (:`then_0`
      (for _index (range (+ (`self.X`) 1))
        (for _index_2 (range (+ (`self.Y`) 1))
          (`InstancedStaticMeshComponent.AddInstance` (`self.InstancedStaticMesh`) (`KismetMathLibrary.MakeTransform` (+ (`self.K2_GetActorLocation`) (`KismetMathLibrary.MakeVector` (* _index (`self.Offset`)) (* _index_2 (`self.Offset`)))) (struct) (0.5 0.5 0.5)) true))))
    (:`then_1`
      (for _index_3 (range (+ (`self.X`) 1))
        (set `local.FirstXRow` (== _index_3 0))
        (set `local.LastXRow` (== _index_3 (`self.X`)))
        (for _index_4 (range (+ (`self.Y`) 1))
          (set `local.FirstYRow` (== _index_4 0))
          (set `local.LastYRow` (== _index_4 (`self.Y`)))
          (if (or (`local.FirstXRow`) (`local.LastXRow`) (`local.FirstYRow`) (`local.LastYRow`))
            (`|ExecutionSequence`
              (:`then_0`
                (if (`local.FirstXRow`)
                  (set `local.z` 90.0)
                  (set `local.Offset` (-100.0 0.0 0.0))
                  (elif (`local.LastXRow`)
                    (set `local.z` -90.0)
                    (set `local.Offset` (100.0 0.0 0.0))
                    (elif (`local.FirstYRow`)
                      (set `local.z` 180.0)
                      (set `local.Offset` (0.0 -100.0 0.0))
                      (elif (`local.LastYRow`)
                        (set `local.z` 0.0)
                        (set `local.Offset` (0.0 100.0 0.0)))))))
              (:`then_1`
                (bind _returnvalue (+ (+ (`self.K2_GetActorLocation`) (`KismetMathLibrary.MakeVector` (* _index_3 (`self.Offset`)) (* _index_4 (`self.Offset`)))) (`local.Offset`)))
                (`InstancedStaticMeshComponent.AddInstance` (`self.InstancedStaticMesh1`) (`KismetMathLibrary.MakeTransform` _returnvalue (`KismetMathLibrary.MakeRotator` 0.0 0.0 (`local.z`)) (0.5 0.5 0.5)) true)
                (if (and (`local.FirstYRow`) (`local.LastXRow`))
                  (`InstancedStaticMeshComponent.AddInstance` (`self.InstancedStaticMesh1`) (`KismetMathLibrary.MakeTransform` (+ _returnvalue (-100.0 -100.0 0.0)) (`KismetMathLibrary.MakeRotator` 0.0 0.0 180.0) (0.5 0.5 0.5)) true)
                  (elif (and (`local.FirstXRow`) (`local.LastYRow`))
                    (`InstancedStaticMeshComponent.AddInstance` (`self.InstancedStaticMesh1`) (`KismetMathLibrary.MakeTransform` (+ _returnvalue (100.0 100.0 0.0)) (`KismetMathLibrary.MakeRotator` 0.0) (0.5 0.5 0.5)) true)
                    (elif (and (`local.FirstXRow`) (`local.FirstYRow`))
                      (`InstancedStaticMeshComponent.AddInstance` (`self.InstancedStaticMesh1`) (`KismetMathLibrary.MakeTransform` (+ _returnvalue (100.0 -100.0 0.0)) (`KismetMathLibrary.MakeRotator` 0.0 0.0 180.0) (0.5 0.5 0.5)) true)
                      (elif (and (`local.LastYRow`) (`local.LastXRow`))
                        (`InstancedStaticMeshComponent.AddInstance` (`self.InstancedStaticMesh1`) (`KismetMathLibrary.MakeTransform` (+ _returnvalue (-100.0 100.0 0.0)) (`KismetMathLibrary.MakeRotator` 0.0) (0.5 0.5 0.5)) true)))))))))))))

(fn `SpawnActorsFromInstances`
  (params (InputPin :type "InstancedStaticMeshComponent Object Reference"))
  (for _index (range (+ (`InstancedStaticMeshComponent.GetInstanceCount` InputPin) 1))
    (bind _returnvalue (`|SpawnActorFromClass` "/Script/Engine.StaticMeshActor" (`InstancedStaticMeshComponent.GetInstanceTransform` InputPin _index true) "AlwaysSpawn" "MultiplyWithRoot" null null))
    (`StaticMeshComponent.SetStaticMesh` (`StaticMeshActor.StaticMeshComponent` _returnvalue) (`StaticMeshComponent.StaticMesh` InputPin)))
  (return))

(fn `UserConstructionScript`
  (`InstancedStaticMeshComponent.ClearInstances` (`self.InstancedStaticMesh`))
  (`InstancedStaticMeshComponent.ClearInstances` (`self.InstancedStaticMesh1`))
  (`self.GenerateRoom`))
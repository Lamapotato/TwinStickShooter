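; Blueprint actor that scatters random trash meshes around its location.
; The construction script clamps the mesh count, then adds physics-simulating static mesh components at random X/Y offsets within a square set by Radius.
; Each gets a random rotation and a random mesh from MeshsToSpawn.
; An identical copy in the event graph is disconnected, and the SpawnTrash event is empty.
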(event `SpawnTrash`)

(fn `UserConstructionScript`
  (bind _returnvalue (`KismetMathLibrary.RandomFloatInRange` 0.0 360.0))
  (bind _meshstospawn (`self.MeshsToSpawn`))
  (bind _radius (`self.Radius`))
  (bind _returnvalue_2 (* _radius -1.0))
  (set `self.NumberOfMeshs` (`KismetMathLibrary.Clamp` (`self.NumberOfMeshs`) 0 100))
  (for _ (range 1 (+ (`self.NumberOfMeshs`) 1))
    (bind _returnvalue_3 (`AddComponent|NODE_AddStaticMeshComponent-1` :`RelativeTransform` (`KismetMathLibrary.MakeTransform` (`KismetMathLibrary.MakeVector` (`KismetMathLibrary.RandomFloatInRange` _returnvalue_2 _radius) (`KismetMathLibrary.RandomFloatInRange` _returnvalue_2 _radius)) (`KismetMathLibrary.SelectRotator` (`KismetMathLibrary.MakeRotator` _returnvalue _returnvalue _returnvalue) (struct) true))))
    (`PrimitiveComponent.SetSimulatePhysics` _returnvalue_3 true)
    (`StaticMeshComponent.SetStaticMesh` _returnvalue_3 (`|GetArrayItem` _meshstospawn (`KismetMathLibrary.RandomIntegerInRange` 0 (`KismetArrayLibrary.Array_LastIndex` _meshstospawn))))))
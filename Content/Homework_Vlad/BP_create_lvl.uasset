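; BP_create_lvl is a level-building Blueprint that generates a rectangular room from static meshes when its CreateRoom event runs.
; Nested loops over X and Y spawn StaticMeshActors at Offset spacing from the actor's location, first laying a Block floor grid.
; Two further passes place raised Column meshes along the perimeter, rotating one pair of sides 90 degrees.
; NewMacro, a loop variant with a randomized condition, is unused here.
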(event `CreateRoom`
  (bind _offset (`self.offset`))
  (bind _y (`self.y`))
  (bind _x (`self.x`))
  (`|ExecutionSequence`
    (:`then_0`
      ; Спавн пола
      (for _index (range (+ (`self.x`) 1))
        (for _index_2 (range (+ (`self.y`) 1))
          (bind _returnvalue (`|SpawnActorFromClass` "/Script/Engine.StaticMeshActor" (`KismetMathLibrary.MakeTransform` (+ (`self.K2_GetActorLocation`) (`KismetMathLibrary.MakeVector` (* _index (`self.offset`)) (* _index_2 (`self.offset`)))) (struct) (3.0 3.0 3.0)) "Undefined" "MultiplyWithRoot" null null))
          (`StaticMeshComponent.SetStaticMesh` (`StaticMeshActor.StaticMeshComponent` _returnvalue) "/Game/Homework_Vlad/Assets/Block/block/StaticMeshes/block.block"))))
    (:`then_1`
      ; Спавн колонн по оси Х
      (for _index_3 (range (+ (`self.x`) 1))
        (for _index_4 (range (+ _y 1))
          (if (or (== _index_4 0) (== _y _index_4) false false)
            (bind _returnvalue_2 (`|SpawnActorFromClass` "/Script/Engine.StaticMeshActor" (`KismetMathLibrary.MakeTransform` (+ (`self.K2_GetActorLocation`) (`KismetMathLibrary.MakeVector` (* _index_3 _offset) (* _index_4 _offset) 100.0)) (struct) (4.0 4.0 4.0)) "Undefined" "MultiplyWithRoot" null null))
            (`StaticMeshComponent.SetStaticMesh` (`StaticMeshActor.StaticMeshComponent` _returnvalue_2) "/Game/Homework_Vlad/Assets/Colomn/column/StaticMeshes/column.column")))))
    (:`then_2`
      ; Спавн колонн по оси У
      (for _index_5 (range (+ _x 1))
        (for _index_6 (range (+ (`self.y`) 1))
          (if (or (== _index_5 0) (== _index_5 _x) false false)
            (bind _returnvalue_3 (`|SpawnActorFromClass` "/Script/Engine.StaticMeshActor" (`KismetMathLibrary.MakeTransform` (+ (`self.K2_GetActorLocation`) (`KismetMathLibrary.MakeVector` (* _index_5 (`self.offset`)) (* _index_6 (`self.offset`)) 100.0)) (`KismetMathLibrary.MakeRotator` 0.0 0.0 90.0) (4.0 4.0 4.0)) "Undefined" "MultiplyWithRoot" null null))
            (`StaticMeshComponent.SetStaticMesh` (`StaticMeshActor.StaticMeshComponent` _returnvalue_3) "/Game/Homework_Vlad/Assets/Colomn/column/StaticMeshes/column.column")))))))

(fn `UserConstructionScript`)
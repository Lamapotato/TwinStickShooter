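; Projectile actor for a Zuma game that carries a color and inserts a ball of that color where it hits the ball chain.
; On BeginPlay the sphere takes a dynamic material instance chosen by its Red, Green or Blue color.
; Tick sweeps it forward at its speed.
; The first overlap with a BP_ZumaBall passes the color to that ball's InsertBall and destroys the projectile, with a DoOnce preventing repeat insertions.
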(event `self.ReceiveBeginPlay`
  (`PrimitiveComponent.CreateDynamicMaterialInstance` (`self.Sphere`) 0 (select `/Game/ZUMA/E_ZumaColors` (`self.Color`) :`NewEnumerator0` "/Game/ZUMA/M_ZumaColor_Red.M_ZumaColor_Red" :`NewEnumerator1` "/Game/ZUMA/M_ZumaColor_Green.M_ZumaColor_Green" :`NewEnumerator2` "/Game/ZUMA/M_ZumaColor_Blue.M_ZumaColor_Blue" :!type "MaterialInterface Object Reference") "None"))

(event `self.ReceiveActorBeginOverlap`
  (params (OtherActor :type "Actor Object Reference"))
  (bind _asbp_zuma_ball (cast `/Game/ZUMA/BP_ZumaBall` OtherActor))
  (`/Engine/EditorBlueprintResources/StandardMacros.DoOnce` false
    (:`Completed`
      (`/Game/ZUMA/BP_ZumaBall.InsertBall` _asbp_zuma_ball (`self.Color`))
      (`self.K2_DestroyActor`))))

(event `self.ReceiveTick`
  (params (DeltaSeconds :type "Float (single-precision)"))
  (`self.K2_AddActorWorldOffset` (* (* DeltaSeconds (`self.Speed`)) (`self.GetActorForwardVector`)) true))

(fn `UserConstructionScript`)
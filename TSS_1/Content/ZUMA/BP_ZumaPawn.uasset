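; BP_ZumaPawn is the shooter pawn for a Zuma-style game, aiming at the mouse cursor and firing colored projectiles.
; Each tick it yaws its mesh toward the cursor's visibility-trace hit, with a 90-degree offset.
; A left-click debug key event spawns a BP_ZumaProjectile at the Sphere's transform with NextColor, then randomly picks red, green or blue.
; UpdateColor previews the next color through the Sphere's material.
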(event EventBeginPlay
  (Variables|/Script/Engine.PlayerController|SetbShowMouseCursor (Game|GetPlayerController 0) true)
  (CallFunction|UpdateColor))

(event Collision|EventActorBeginOverlap
  (params (OtherActor :type Actor%20Object%20Reference)))

(event EventTick
  (params (DeltaSeconds :type Float%20%28single-precision%29))
  (bind _returnvalue (Game|GetPlayerController 0))
  (bind (_hitresult _returnvalue_2) (Game|Player|GetHitResultUnderCursorbyChannel _returnvalue "TraceTypeQuery1" true))
  (if _returnvalue_2
    (Transformation|SetRelativeRotation (Variables|Default|GetMesh) (Math|Rotator|MakeRotator 0.0 0.0 (+ (.yaw (Math|Rotator|FindLookatRotation (Transformation|GetActorLocation) (.Location (Collision|BreakHitResult _hitresult)))) 9e+01)) false false)))

(event Input|MouseEvents|DebugKeyLeftMouseButton
  (params (Key :type Key%20Structure :default "None") (ActionValue :type Input%20Action%20Value%20Structure))
  (:Pressed
    (Game|SpawnActorfromClass "/Game/ZUMA/BP_ZumaProjectile.BP_ZumaProjectile_C" (Transformation|GetWorldTransform (Variables|Default|GetSphere)) "AlwaysSpawn" "MultiplyWithRoot" 0 (Variables|Default|GetNextColor) 0)
    (switch int (Math|Random|RandomIntegerinRange 0 2)
      (:0
        (Variables|Default|SetNextColor "NewEnumerator0"))
      (:1
        (Variables|Default|SetNextColor "NewEnumerator1"))
      (:2
        (Variables|Default|SetNextColor "NewEnumerator2")))
    (CallFunction|UpdateColor)))

(fn ConstructionScript)

(fn UpdateColor
  (Rendering|Material|CreateDynamicMaterialInstance (Variables|Default|GetSphere) 0 (Utilities|Select :Index (Variables|Default|GetNextColor) :NewEnumerator0 "/Game/ZUMA/M_ZumaColor_Red.M_ZumaColor_Red" :NewEnumerator1 "/Game/ZUMA/M_ZumaColor_Green.M_ZumaColor_Green" :NewEnumerator2 "/Game/ZUMA/M_ZumaColor_Blue.M_ZumaColor_Blue") "None" :!class /Script/Engine.PrimitiveComponent))
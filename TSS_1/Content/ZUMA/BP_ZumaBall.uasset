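; BP_ZumaBall is a colored ball in a Zuma-style game, taking a preset or random red, green or blue material on BeginPlay.
; It delegates insertion and match checks to BP_ZumaSpline, passing itself or its index in the Balls array, and removes itself from that array when destroyed.
; A helper sphere-overlaps for nearby same-colored balls, while InsertRandomBall always passes Red despite its name.
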(event `self.ReceiveBeginPlay`
  (if (`self.bSpawnWithCertaintColor`)
    (`self.UpdateColor`)
    (else
      (switch `int` (`KismetMathLibrary.RandomIntegerInRange` 0 2)
        (:`0`
          (set `self.Color` "NewEnumerator0"))
        (:`1`
          (set `self.Color` "NewEnumerator1"))
        (:`2`
          (set `self.Color` "NewEnumerator2")))
      (`self.UpdateColor`))))

(event `CheckBallsNearby`
  (`self.CheckClosestBalls`))

(event `InsertBall`
  (params (Color :type "/Game/ZUMA/E_ZumaColors Enum" :default "NewEnumerator0"))
  (bind _returnvalue (`GameplayStatics.GetActorOfClass` "/Game/ZUMA/BP_ZumaSpline.BP_ZumaSpline_C"))
  (`/Game/ZUMA/BP_ZumaSpline.InsertBall` _returnvalue self Color))

(event `InsertRandomBall`
  (bind _returnvalue (`GameplayStatics.GetActorOfClass` "/Game/ZUMA/BP_ZumaSpline.BP_ZumaSpline_C"))
  (`/Game/ZUMA/BP_ZumaSpline.InsertBall` _returnvalue self "NewEnumerator0"))

(event `DeleteBall`
  (`self.K2_DestroyActor`))

(event `self.ReceiveDestroyed`
  (bind _returnvalue (`GameplayStatics.GetActorOfClass` "/Game/ZUMA/BP_ZumaSpline.BP_ZumaSpline_C"))
  (`KismetArrayLibrary.Array_RemoveItem` (`/Game/ZUMA/BP_ZumaSpline.Balls` _returnvalue) self))

(fn `CheckClosestBalls`
  (locals (bAllMatch :type Boolean :default true) (OvelappedBalls :type "Array of Actor Object Reference") (NewOvelaps :type "Array of Actor Object Reference"))
  (bind _returnvalue (`GameplayStatics.GetActorOfClass` "/Game/ZUMA/BP_ZumaSpline.BP_ZumaSpline_C"))
  (`/Game/ZUMA/BP_ZumaSpline.CheckForMatchingBalls` _returnvalue (`KismetArrayLibrary.Array_Find` (`/Game/ZUMA/BP_ZumaSpline.Balls` _returnvalue) self)))

(fn `GetOverlappingBalls`
  (returns (OutActors :type "Array of Actor Object Reference"))
  (locals (NewLocalVar :type "Array of Actor Object Reference"))
  (bind _outactors (`KismetSystemLibrary.SphereOverlapActors` (`self.K2_GetActorLocation`) 120.0 (`|MakeArray` "ObjectTypeQuery2" :!type "EObjectTypeQuery Enum") "BP_ZumaBall_C"))
  (for _array_element _outactors
    (bind _asbp_zuma_ball (cast `/Game/ZUMA/BP_ZumaBall` _array_element))
    (if (`|EnumEquality` (`/Game/ZUMA/BP_ZumaBall.Color` _asbp_zuma_ball) (`self.Color`))
      (`KismetArrayLibrary.Array_AddUnique` (`local.NewLocalVar`) _asbp_zuma_ball)))
  (return (`local.NewLocalVar`)))

(fn `UpdateColor`
  (`PrimitiveComponent.CreateDynamicMaterialInstance` (`self.Sphere`) 0 (select `/Game/ZUMA/E_ZumaColors` (`self.Color`) :`NewEnumerator0` "/Game/ZUMA/M_ZumaColor_Red.M_ZumaColor_Red" :`NewEnumerator1` "/Game/ZUMA/M_ZumaColor_Green.M_ZumaColor_Green" :`NewEnumerator2` "/Game/ZUMA/M_ZumaColor_Blue.M_ZumaColor_Blue" :!type "MaterialInterface Object Reference") "None"))

(fn `UserConstructionScript`)
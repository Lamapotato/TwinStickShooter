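; Player character for a top-down-style shooter, with Enhanced Input movement, jumping, cursor-facing mesh rotation and punch/sword montages.
; Weapon keys replace the spawned weapon on the hand socket, and fire delegates to it.
; A sphere counts overlapping BPI_Interactable actors to show a text prompt, while interact targets the closest one.
; Damage lowers health, refreshing its text before the subtraction, and reloads the level at zero.
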(event `self.ReceiveBeginPlay`
  (bind _returnvalue (pcsubsystem `EnhancedInputLocalPlayerSubsystem` (`GameplayStatics.GetPlayerController` 0)))
  (`EnhancedInputSubsystemInterface.ClearAllMappings` _returnvalue)
  (`EnhancedInputSubsystemInterface.AddMappingContext` _returnvalue "/Game/TSS/Blueprints/IMC_TSSMovent.IMC_TSSMovent" 0 (struct))
  (set `PlayerController.bShowMouseCursor` true (`GameplayStatics.GetPlayerController` 0)))

(event `EnhancedInput|/Game/TSS/Blueprints/IA_TSSMove`
  (params (ActionValue :type "Vector2D Structure") (ElapsedSeconds :type "Float (double-precision)") (TriggeredSeconds :type "Float (double-precision)") (InputAction :type "InputAction Object Reference" :default "/Game/TSS/Blueprints/IA_TSSMove.IA_TSSMove"))
  (bind (_x _y) (`KismetMathLibrary.BreakVector2D` ActionValue))
  (bind _mesh (`self.Mesh`))
  (:`Triggered`
    (`PawnMovementComponent.AddInputVector` (`self.CharacterMovement`) (`KismetMathLibrary.MakeVector` _x _y) false))
  (:`Started`
    (`SkeletalMeshComponent.SetAnimation` _mesh "/Game/Characters/Mannequins/Anims/Rifle/Walk/MF_Rifle_Walk_Fwd.MF_Rifle_Walk_Fwd"))
  (:`Completed`
    (`SkeletalMeshComponent.SetAnimation` _mesh "/Game/Characters/Mannequins/Anims/Rifle/MF_Rifle_Idle_ADS.MF_Rifle_Idle_ADS")))

(event `EnhancedInput|/Game/TSS/Blueprints/IA_TSSJump`
  (params (ActionValue :type Boolean) (ElapsedSeconds :type "Float (double-precision)") (TriggeredSeconds :type "Float (double-precision)") (InputAction :type "InputAction Object Reference" :default "/Game/TSS/Blueprints/IA_TSSJump.IA_TSSJump"))
  (:`Triggered`
    (`self.Jump`)))

(event `EnhancedInput|/Game/TSS/Blueprints/IA_TSSSelectWeapon1`
  (params (ActionValue :type Boolean) (ElapsedSeconds :type "Float (double-precision)") (TriggeredSeconds :type "Float (double-precision)") (InputAction :type "InputAction Object Reference" :default "/Game/TSS/Blueprints/IA_TSSSelectWeapon1.IA_TSSSelectWeapon1"))
  (:`Triggered`
    (`self.ChangeWeapon` "/Game/TSS/Blueprints/Weapons/BP_TSSWeapon_1.BP_TSSWeapon_1_C")))

(event `EnhancedInput|/Game/TSS/Blueprints/IA_TSSSelectWeapon2`
  (params (ActionValue :type Boolean) (ElapsedSeconds :type "Float (double-precision)") (TriggeredSeconds :type "Float (double-precision)") (InputAction :type "InputAction Object Reference" :default "/Game/TSS/Blueprints/IA_TSSSelectWeapon2.IA_TSSSelectWeapon2"))
  (:`Triggered`
    (`self.ChangeWeapon` "/Game/TSS/Blueprints/Weapons/BP_TSSWeapon_2.BP_TSSWeapon_2_C")))

(event `EnhancedInput|/Game/TSS/Blueprints/IA_TSSFire`
  (params (ActionValue :type Boolean) (ElapsedSeconds :type "Float (double-precision)") (TriggeredSeconds :type "Float (double-precision)") (InputAction :type "InputAction Object Reference" :default "/Game/TSS/Blueprints/IA_TSSFire.IA_TSSFire"))
  (:`Triggered`
    (`/Engine/EditorBlueprintResources/StandardMacros.IsValid` (`self.Weapon`)
      (:`Is Valid`
        (`/Game/TSS/Blueprints/Weapons/BP_TSSWeapon.Fire` (`self.Weapon`))))))

(event `self.ReceiveTick`
  (params (DeltaSeconds :type "Float (single-precision)"))
  (bind (_hitresult _returnvalue) (`PlayerController.GetHitResultUnderCursorByChannel` (`GameplayStatics.GetPlayerController` 0) "TraceTypeQuery1" true))
  (bind (_returnvalue_roll _returnvalue_pitch _returnvalue_yaw) (`KismetMathLibrary.BreakRotator` (`KismetMathLibrary.FindLookAtRotation` (`self.K2_GetActorLocation`) (`.Location` (`GameplayStatics.BreakHitResult` _hitresult)))))
  (cast `PlayerController` (`self.GetController`))
  (if _returnvalue
    (`SceneComponent.K2_SetRelativeRotation` (`self.Mesh`) (`KismetMathLibrary.MakeRotator` 0.0 0.0 (+ _returnvalue_yaw -90.0)) false false)))

(event `self.ReceiveAnyDamage`
  (params (Damage :type "Float (single-precision)") (DamageType :type "DamageType Object Reference") (InstigatedBy :type "Controller Object Reference") (DamageCauser :type "Actor Object Reference"))
  (`self.UpdateHealth`)
  (bind _output_get (set `self.Health` (- (`self.Health`) Damage)))
  (if (<= _output_get 0.0)
    (bind _returnvalue (`GameplayStatics.GetCurrentLevelName` true))
    (`GameplayStatics.OpenLevel` (`KismetStringLibrary.Conv_StringToName` _returnvalue))))

(event `self.Sphere.OnComponentBeginOverlap`
  (params (OverlappedComponent :type "PrimitiveComponent Object Reference") (OtherActor :type "Actor Object Reference") (OtherComp :type "PrimitiveComponent Object Reference") (OtherBodyIndex :type Integer) (bFromSweep :type Boolean) (SweepResult :type "HitResult Structure (by ref)"))
  (cast `/Game/TSS/Blueprints/BPI_Interactable` OtherActor)
  (`/Engine/EditorBlueprintResources/StandardMacros.IncrementInt` (`self.InteractableCount`)
    (:`  `
      (`SceneComponent.SetHiddenInGame` (`self.TextRender`) (not (> (`self.InteractableCount`) 0)) false :!label _label))))

(event `self.Sphere.OnComponentEndOverlap`
  (params (OverlappedComponent :type "PrimitiveComponent Object Reference") (OtherActor :type "Actor Object Reference") (OtherComp :type "PrimitiveComponent Object Reference") (OtherBodyIndex :type Integer))
  (cast `/Game/TSS/Blueprints/BPI_Interactable` OtherActor)
  (`/Engine/EditorBlueprintResources/StandardMacros.DecrementInt` (`self.InteractableCount`)
    (:`  `
      (goto _label))))

(event `EnhancedInput|/Game/TSS/Blueprints/IA_TSSInteract`
  (params (ActionValue :type Boolean) (ElapsedSeconds :type "Float (double-precision)") (TriggeredSeconds :type "Float (double-precision)") (InputAction :type "InputAction Object Reference" :default "/Game/TSS/Blueprints/IA_TSSInteract.IA_TSSInteract"))
  (:`Triggered`
    (bind _closestactor (`self.OpenClosestDoor`))
    (bind _asbpi_interactable (cast `/Game/TSS/Blueprints/BPI_Interactable` _closestactor))
    (`/Game/TSS/Blueprints/BPI_Interactable.Interact` _asbpi_interactable)))

(event `EnhancedInput|/Game/TSS/Blueprints/IA_TSSPunch`
  (params (ActionValue :type Boolean) (ElapsedSeconds :type "Float (double-precision)") (TriggeredSeconds :type "Float (double-precision)") (InputAction :type "InputAction Object Reference" :default "/Game/TSS/Blueprints/IA_TSSPunch.IA_TSSPunch"))
  (:`Triggered`
    (`self.PlayAnimMontage` "/Game/TSS/Animations/AM_cross_punch_Montage.AM_cross_punch_Montage")))

(event `EnhancedInput|/Game/TSS/Blueprints/IA_TSSSwordIdle`
  (params (ActionValue :type Boolean) (ElapsedSeconds :type "Float (double-precision)") (TriggeredSeconds :type "Float (double-precision)") (InputAction :type "InputAction Object Reference" :default "/Game/TSS/Blueprints/IA_TSSSwordIdle.IA_TSSSwordIdle"))
  (:`Triggered`
    (`self.PlayAnimMontage` "/Game/TSS/Animations/AM_TSSSwordIdl.AM_TSSSwordIdl")))

(event `EnhancedInput|/Game/TSS/Blueprints/IA_TSSSwordPunch`
  (params (ActionValue :type Boolean) (ElapsedSeconds :type "Float (double-precision)") (TriggeredSeconds :type "Float (double-precision)") (InputAction :type "InputAction Object Reference" :default "/Game/TSS/Blueprints/IA_TSSSwordPunch.IA_TSSSwordPunch"))
  (:`Triggered`
    (`self.PlayAnimMontage` "/Game/TSS/Animations/AM_TSSSwordPunch.AM_TSSSwordPunch")))

(fn `ChangeWeapon`
  (params (WeaponClass :type "/Game/TSS/Blueprints/Weapons/BP_TSSWeapon Class Reference"))
  (bind _mesh (`self.Mesh`))
  (`/Engine/EditorBlueprintResources/StandardMacros.IsValid` (`self.Weapon`)
    (:`Is Valid`
      (`self.K2_DestroyActor` (`self.Weapon`)))
    (:`Is Not Valid`
      _))
  (bind _returnvalue (`|SpawnActorFromClass` WeaponClass (`KismetMathLibrary.MakeTransform` (`SceneComponent.K2_GetComponentLocation` _mesh) (`SceneComponent.GetSocketRotation` _mesh "hand_r_weapon")) "AlwaysSpawn" "MultiplyWithRoot" null null))
  (bind _output_get (set `self.Weapon` _returnvalue))
  (`self.K2_AttachToComponent` _output_get (`self.Mesh`) "hand_r_weapon" "SnapToTarget" "SnapToTarget" "SnapToTarget" true)
  (`self.K2_SetActorRelativeRotation` :`self` _output_get))

(fn `OpenClosestDoor`
  (returns (ClosestActor :type "/Game/TSS/Blueprints/BPI_Interactable Interface"))
  (locals (ClosestDistance :type "Float (single-precision)" :default 9999.0) (ClosestInteractible :type "Actor Object Reference"))
  (for _array_element (`PrimitiveComponent.GetOverlappingActors` (`self.Sphere`) "/Script/Engine.Actor")
    (cast `/Game/TSS/Blueprints/BPI_Interactable` _array_element)
    (bind _returnvalue (`self.GetDistanceTo` self _array_element))
    (if (< _returnvalue (`local.ClosestDistance`))
      (set `local.ClosestDistance` _returnvalue)
      (set `local.ClosestInteractible` _array_element)))
  (bind _asbpi_interactable (cast `/Game/TSS/Blueprints/BPI_Interactable` (`local.ClosestInteractible`)))
  (return _asbpi_interactable))

(fn `UpdateHealth`
  (`TextRenderComponent.K2_SetText` (`self.HealthTextRender`) (`KismetTextLibrary.Conv_IntToText` (`KismetMathLibrary.FTrunc` (`self.Health`)))))

(fn `UserConstructionScript`
  (`self.UpdateHealth`))
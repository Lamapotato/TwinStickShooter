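; BP_TSSPhysicalPawn is a physics-driven pawn that chases the first player's pawn.
; Each tick it applies an impulse to its capsule straight toward the player, scaled by MovementForce and delta time.
; BeginPlay computes and debug-draws a navigation path to the player once, but the steering ignores it, as the path-point validity check is disconnected.
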(event `self.ReceiveBeginPlay`
  (`/Engine/EditorBlueprintResources/StandardMacros.IsValid` (`GameplayStatics.GetPlayerPawn` 0)
    (:`Is Valid`
      (bind _returnvalue (`NavigationSystemV1.FindPathToActorSynchronously` (`self.K2_GetActorLocation`) (`GameplayStatics.GetPlayerPawn` 0) 50.0 null null))
      (`NavigationPath.EnableDebugDrawing` _returnvalue true (struct :`R` 1.0 :`B` 0.889183 :`A` 1.0))
      (set `self.Path` _returnvalue))))

(event `self.ReceiveTick`
  (params (DeltaSeconds :type "Float (single-precision)"))
  (`PrimitiveComponent.AddImpulse` (`self.Capsule`) (* (`KismetMathLibrary.Normal` (- (`self.K2_GetActorLocation` (`GameplayStatics.GetPlayerPawn` 0)) (`self.K2_GetActorLocation`))) (`self.MovementForce`) (`GameplayStatics.GetWorldDeltaSeconds`)) "None" false))

(fn `UserConstructionScript`)